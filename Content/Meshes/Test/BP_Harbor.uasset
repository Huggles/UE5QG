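; Harbor Blueprint that shows team ownership, Axis or Allies, through the flag material on its mesh.
; SetTeam stores the team and calls HandleMaterials, which applies the Mesh variable to HarborMesh and swaps the first material slot to that team's flag material.
; The construction script always calls SetTeam with Allies, so every harbor is constructed as Allied.
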(event Custom|Set%20Team
  (params (Team :type TeamEnum%20Enum :default "NewEnumerator0"))
  (Variables|Default|SetTeam Team)
  (CallFunction|HandleMaterials))

(event Custom|Handle%20Materials
  (bind _harbormesh (Variables|Default|GetHarborMesh))
  ;[1 1 1] Set Materials
  (Components|StaticMesh|SetStaticMesh (Variables|Default|GetHarborMesh) (Variables|Default|GetMesh))
  (switch Utilities|FlowControl|Switch|SwitchonTeamEnum (Variables|Default|GetTeam)
    (:NewEnumerator2
      (Rendering|Material|SetMaterial _harbormesh 0 (Variables|Default|GetFlag%20Material%20Axis)))
    (:NewEnumerator1
      (Rendering|Material|SetMaterial _harbormesh 0 (Variables|Default|GetFlag%20Material%20Allies)))))

(fn ConstructionScript
  (CallFunction|SetTeam "NewEnumerator1"))