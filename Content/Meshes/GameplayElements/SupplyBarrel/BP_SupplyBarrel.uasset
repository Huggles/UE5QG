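; Supply barrel actor that can be shown or hidden in a faction's color.
; BeginPlay puts a dynamic material instance on the mesh's second material slot.
; Toggle tints that material using the race color from the game state, blacks out emissive, and sets visibility on the whole component tree.
; While shown, a timeline animates the actor's pitch, restarting on each show and stopping on hide.
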(event Custom|Toggle
  (params (Faction :type PlayableRaceEnum%20Enum :default "NewEnumerator0") (Show :type Boolean))
  (CallFunction|SetFactionColor Faction)
  (Rendering|SetVisibility (Variables|Default|GetDefaultSceneRoot self) Show true)
  (if Show
    (bind _rotation (Timeline|Timeline PlayFromStart)
      (:Update
        (Transformation|SetActorRelativeRotation (Math|Rotator|MakeRotator 0.0 _rotation 0.0))))
    (else
      (Timeline|Timeline Stop))))

(event Custom|Handle%20Materials
  (Development|PrintString "Handle Materials")
  (bind _returnvalue (Rendering|Material|CreateDynamicMaterialInstance (Variables|Default|GetStaticMesh) 1 "/Game/Meshes/GameplayElements/SupplyBarrel/M_Simple_Color_Black.M_Simple_Color_Black" "FactionColor_Inst_Dynamic" :!class /Script/Engine.PrimitiveComponent))
  (Variables|Default|SetFaction%20Color%20Material _returnvalue)
  (Rendering|Material|SetMaterial (Variables|Default|GetStaticMesh) 1 (Variables|Default|GetFaction%20Color%20Material)))

(event Custom|Set%20Faction%20Color
  (params (Set%20Faction :type PlayableRaceEnum%20Enum :default "NewEnumerator0"))
  (Variables|Default|SetFaction Set%20Faction)
  (bind _faction_color (CallFunction|SetPlayerColor))
  (Development|PrintString (Utilities|String|ToString(Integer) _faction_color)))

(event EventBeginPlay
  (CallFunction|HandleMaterials))

(fn ConstructionScript)

(fn SetPlayerColor
  (bind _tb_game_state (CallFunction|TBGameState))
  (bind _faction (Variables|Default|GetFaction))
  (bind _race_struct (Default|GetRaceStructStructforRace _tb_game_state _faction))
  (bind _returnvalue (Math|Conversions|ToLinearColor(Color) (.color _race_struct)))
  (Rendering|Material|SetVectorParameterValue (Variables|Default|GetFaction%20Color%20Material) "color" _returnvalue :!class /Script/Engine.MaterialInstanceDynamic)
  (Rendering|Material|SetVectorParameterValue (Variables|Default|GetFaction%20Color%20Material) "emissive" "(R=0.000000,G=0.000000,B=0.000000,A=1.000000)" :!class /Script/Engine.MaterialInstanceDynamic)
  (return _returnvalue))