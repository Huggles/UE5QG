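; BP_SelectionRing is a selection ring Blueprint that changes color as the mouse cursor hovers over its static mesh.
; On BeginPlay it creates a dynamic instance of the unit selection plane material on the mesh's second material slot.
; Cursor-over events pass green on enter and red on exit to SetSelectionColor, which sets the material's color vector parameter.
; Both cursor events also print debug test strings.
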(event OnBeginCursorOver(StaticMesh)
  (params (TouchedComponent :type Primitive%20Component%20Object%20Reference))
  (Development|PrintString "Test 1")
  (CallFunction|SetSelectionColor "(R=0.038414,G=1.000000,B=0.000000,A=1.000000)"))

(event OnEndCursorOver(StaticMesh)
  (params (TouchedComponent :type Primitive%20Component%20Object%20Reference))
  (Development|PrintString "Test 2")
  (CallFunction|SetSelectionColor "(R=1.000000,G=0.000000,B=0.004558,A=1.000000)"))

(event EventBeginPlay
  (bind _returnvalue (Rendering|Material|CreateDynamicMaterialInstance (Variables|Default|GetStaticMesh) 1 "/Game/Material/Units/M_UnitSelectionPlane_Inst.M_UnitSelectionPlane_Inst" "Unit_Selected_Inst_Dynamic" :!class /Script/Engine.PrimitiveComponent))
  (Variables|Default|SetDynamic%20Selection%20Circle%20Material _returnvalue)
  (Rendering|Material|SetMaterial (Variables|Default|GetStaticMesh) 1 (Variables|Default|GetDynamic%20Selection%20Circle%20Material)))

(fn ConstructionScript)

(fn SetSelectionColor
  (params (Color :type Linear%20Color%20Structure))
  (Rendering|Material|SetVectorParameterValue (Variables|Default|GetDynamic%20Selection%20Circle%20Material) "c" Color :!class /Script/Engine.MaterialInstanceDynamic))