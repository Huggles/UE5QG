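; Base Blueprint actor for a turn-based gameplay ability, with empty hooks for pre/post processing and animation lists.
; On BeginPlay the server binds to every client animation manager, runs PreprocessAbility, then has the game state execute the ability's animations.
; Each manager unbinds when it reports all animations finished.
; A DoOnce lets only the first report trigger PostprocessAbility and notify the IGameplayAbilityCallback that execution finished.
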(event Custom|Postprocess%20Ability)

(event Custom|Preprocess%20Ability)

(event Custom|Register%20Animations%20Finished%20Callback
  (for _array_element (CallFunction|GetAllClientAnimationManagers)
    (EventDispatchers|AssignAllAnimationsFinished _array_element (delegate Custom|AllAnimationsFinished_Event))))

(event Custom|AllAnimationsFinished_Event
  (params (TB%20Player%20Controller :type BP%20Turn%20Based%20Player%20Controller%20Object%20Reference) (Client%20Animation%20Manager :type BP%20Client%20Animation%20Manager%20Object%20Reference))
  (EventDispatchers|UnbindEventfromAllAnimationsFinished Client%20Animation%20Manager (delegate Custom|AllAnimationsFinished_Event))
  (Utilities|FlowControl|DoOnce false
    (:Completed
      (CallFunction|PostprocessAbility)
      (Utilities|Casting|CastToIGameplayAbilityCallback (Variables|Default|GetCallback))
      (Default|AbilityExecutionFinished (Variables|Default|GetCallback) self))))

(event EventBeginPlay
  (Networking|SwitchHasAuthority
    (:Authority
      (CallFunction|RegisterAnimationsFinishedCallback)
      (CallFunction|PreprocessAbility)
      (Default|ExecuteAnimations (CallFunction|TBGameState) (CallFunction|AbilityAnimations)))))

(fn ConstructionScript)

(fn TBPawn
  (return (.AsBP%20Turn%20Based%20Pawn (Utilities|Casting|CastToBP_TurnBasedPawn (Pawn|GetControlledPawn (CallFunction|GetFirstLocalTBPlayerController))))))

(fn ConstructAnimations
  (return))

(fn AbilityAnimations
  (return 0))