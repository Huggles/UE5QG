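; Gameplay ability for attacking a unit, which results in that unit being destroyed and removed from its country.
; It returns a client animation sequence that moves the camera to the unit's spawn point, plays the destroy-unit animation, then returns the camera.
; The post-process step removes the unit from its country.
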(event Custom|Process%20Ability%20Animations_1)

(event EventPostprocessAbility
  (Default|RemoveUnitfromCountry (Variables|Default|GetUnit)))

(fn ConstructionScript
  (|CallParentFunction))

(fn AbilityAnimations
  (return (Utilities|Array|MakeArray (Utilities|Struct|MakeAnimation_Payload "/Game/Blueprints/Actions/ClientAnimations/BP_Client_Animation_MoveCamera.BP_Client_Animation_MoveCamera_C" 0 true 0 1.0 0 0 "0.000000,0.000000,0.000000" (Transformation|GetWorldLocation (Variables|/Game/Blueprints/Units/BP_Unit.BP_Unit_C|GetSpawn%20Point (Variables|Default|GetUnit))) "1.000000,1.000000,1.000000" "/Game/StarterContent/Particles/P_Explosion.P_Explosion" 0.0 0) (Utilities|Struct|MakeAnimation_Payload "/Game/Blueprints/Actions/ClientAnimations/BP_Client_Animation_DestroyUnit.BP_Client_Animation_DestroyUnit_C" 0 true 0 1.0 (Utilities|Array|MakeArray (Variables|Default|GetUnit)) 0 "0.000000,0.000000,0.000000" "0.000000,0.000000,0.000000" "1.000000,1.000000,1.000000" "/Game/StarterContent/Particles/P_Explosion.P_Explosion" 0.0 0) (Utilities|Struct|MakeAnimation_Payload "/Game/Blueprints/Actions/ClientAnimations/BP_Client_Animation_ReturnCamera.BP_Client_Animation_ReturnCamera_C" 0 true 0 1.0 0 0 "0.000000,0.000000,0.000000" "0.000000,0.000000,0.000000" "1.000000,1.000000,1.000000" "/Game/StarterContent/Particles/P_Explosion.P_Explosion" 0.0 0))))