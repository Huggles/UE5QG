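; Client-side animation action that plays when a unit is eliminated, tipping the target unit over.
; It tweens the unit's rotation to a combined 90-degree yaw and roll offset from its current rotation.
; On completion it hides the unit and its children, resets its rotation to zero and notifies that the animation has finished.
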(event EventExecuteAnimation
  (bind _target_unit (Utilities|TargetUnit))
  (bind _returnvalue (Transformation|GetActorRotation _target_unit))
  (bind _value (|TweenRotator _returnvalue (Math|Rotator|CombineRotators _returnvalue "90.000000,90.000000,0.000000") 1.0 "InOutQuad")
    (:ApplyEasing
      (Transformation|SetActorRelativeRotation (Utilities|TargetUnit) _value))
    (:OnComplete
      (Rendering|SetVisibility (Variables|/Script/Engine.Actor|GetRootComponent (Utilities|TargetUnit)) false true)
      (Transformation|SetActorRelativeRotation (Utilities|TargetUnit))
      (CallFunction|NotifyAnimationFinished))))

(fn ConstructionScript)