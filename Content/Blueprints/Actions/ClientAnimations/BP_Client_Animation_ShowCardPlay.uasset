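; Client animation action that shows a played card as a zoomed UI overlay on the local player's screen.
; It passes the first payload card to the local controller's UI widget for a timed zoom, with a subtitle built from the card's race.
; It binds to the end of the widget's hide animation and only then reports the animation as finished.
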(event Custom|On%20Played%20Card%20Shown
  (CallFunction|NotifyAnimationFinished))

(event EventExecuteAnimation
  (bind _local_tb_player_controller (CallFunction|GetFirstLocalTBPlayerController))
  (bind _payload (Variables|Default|GetPayload))
  (bind _output (Utilities|Array|Get(acopy) (.cards _payload)))
  (bind _userinterfacewidget (Variables|/Game/Blueprints/Game/BP_TurnBasedPlayerController.BP_TurnBasedPlayerController_C|GetUserInterfaceWidget _local_tb_player_controller))
  (Default|ShowPlayedCardZoom _userinterfacewidget _output (Utilities|Text|ToText(String) (Utilities|String|Append (Utilities|String|EnumtoString (Default|CardRace _output)) " plays card:")) 3.0)
  (Class|UserWidget|BindtoAnimationFinished _userinterfacewidget (Variables|/Game/Blueprints/UI/UIB_GameInterface_Base.UIB_GameInterface_Base_C|GetHidePlayedCardZoomAnimation _userinterfacewidget) (delegate Custom|On%20Played%20Card%20Shown)))

(fn ConstructionScript)