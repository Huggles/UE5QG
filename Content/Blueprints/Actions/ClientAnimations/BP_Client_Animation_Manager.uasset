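; Client animation manager actor that queues and plays payload-driven animation actors, then reports to the server when finished.
; AddAnimation spawns and attaches an animation actor, appends it to the pending list and tries to start the first pending one.
; New animations can overlap running ones unless any of those is blocking.
; Finished animations are destroyed, advancing the queue or, once empty, relaying client-to-server to signal all animations finished for that player controller.
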(event Custom|Add%20Animation
  (params (Payload :type Animation%20Payload%20Structure%20%28by%20ref%29))
  (bind _returnvalue (Game|SpawnActorfromClass (.AnimationClass (Utilities|Struct|BreakAnimation_Payload Payload)) (Math|Transform|MakeTransform "0, 0, 0") "Undefined" "MultiplyWithRoot" (CallFunction|GetFirstLocalTBPlayerController) Payload self 0 0))
  (Transformation|AttachActorToActor _returnvalue self "None" "KeepRelative" "KeepRelative" "KeepRelative" true)
  (Utilities|Array|Add (Variables|Default|GetPendingAnimations) _returnvalue)
  (CallFunction|RunNextAnimation))

(event Custom|On%20Animation%20Queue%20Empty%20%28Server%29
  (params (TB%20Player%20Controller :type BP%20Turn%20Based%20Player%20Controller%20Object%20Reference))
  (Default|CallAllAnimationsFinished TB%20Player%20Controller self))

(event Custom|Init%20Owner
  (Networking|SwitchHasAuthority
    (:Authority
      (Development|PrintString (Utilities|String|Append "Set Owner" (Utilities|GetDisplayName 0)))
      (Actor|SetOwner (Actor|GetParentActor self)))))

(event Custom|On%20Animation%20Queue%20Empty%20%28Client%29
  (CallFunction|OnAnimationQueueEmpty(Server) (CallFunction|GetFirstLocalTBPlayerController)))

(event Custom|Run%20Next%20Animation
  (bind _next_animation (CallFunction|NextAnimation))
  (if (CallFunction|CanPlayNextAnimation)
    (Utilities|Array|Add (Variables|Default|GetCurrentAnimations) _next_animation)
    (Default|ExecuteAnimation _next_animation)
    (Utilities|Array|RemoveItem (Variables|Default|GetPendingAnimations) _next_animation)))

(event Custom|Handle%20Animation%20Finished
  (params (Animation :type BP%20Client%20Animation%20Object%20Reference))
  (Utilities|Array|RemoveItem (Variables|Default|GetCurrentAnimations) Animation)
  (Actor|DestroyActor Animation)
  (if (CallFunction|IsWorking)
    (CallFunction|RunNextAnimation)
    (else
      (CallFunction|OnAnimationQueueEmpty(Client)))))

(event EventBeginPlay)

(fn ConstructionScript)

(fn NextAnimation
  (return (Utilities|Array|Get(acopy) (Variables|Default|GetPendingAnimations))))

(fn IsPlayingAnimation
  (return (> (Utilities|Array|Length (Variables|Default|GetCurrentAnimations)) 0)))

(fn HasPendingAnimation
  (return (> (Utilities|Array|Length (Variables|Default|GetPendingAnimations)) 0)))

(fn OnRepPendingAnimations)

(fn IsWorking
  (return (or (CallFunction|IsPlayingAnimation) (CallFunction|HasPendingAnimation))))

(fn IsPlayingBlockingAnimation
  (for _array_element (Variables|Default|GetCurrentAnimations)
    (if (.blocking (Variables|/Game/Blueprints/Actions/ClientAnimations/BP_Client_Animation.BP_Client_Animation_C|GetPayload _array_element))
      (return true)))
  (return false))

(fn CanPlayNextAnimation
  (return (and (CallFunction|HasPendingAnimation) (or (not (CallFunction|IsPlayingAnimation)) (and (CallFunction|IsPlayingAnimation) (not (CallFunction|IsPlayingBlockingAnimation)))))))