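; BP_World is the map manager that registers every country actor in the level and links them together.
; On BeginPlay it builds a country list and class-to-instance map, has each country connect through that map, then notifies the local player controller.
; Getters build this data lazily if empty.
; A helper finds harbors linking two given countries in either order.
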(event EventBeginPlay
  (CallFunction|BuildCountryData)
  (Default|WorldSpawned (CallFunction|GetFirstLocalTBPlayerController) self))

(fn ConstructionScript)

(fn AreCountriesPartOfHarbor
  (params (Country%201 :type BP%20Country%20Object%20Reference%20%28by%20ref%29) (Country%202 :type BP%20Country%20Object%20Reference))
  (bind _harbors_local (LocalVariables|GetHarbors%20Local))
  (for _array_element 0
    (if (or (and (== (Variables|/Game/Blueprints/Countries/BP_Country.BP_Country_C|GetHarbor%20For%201 _array_element) Country%201) (== (Variables|/Game/Blueprints/Countries/BP_Country.BP_Country_C|GetHarbor%20For%202 _array_element) Country%202)) (and (== (Variables|/Game/Blueprints/Countries/BP_Country.BP_Country_C|GetHarbor%20For%202 _array_element) Country%201) (== (Variables|/Game/Blueprints/Countries/BP_Country.BP_Country_C|GetHarbor%20For%201 _array_element) Country%202)))
      (Utilities|Array|Add (LocalVariables|GetHarbors%20Local) _array_element)))
  (return (> (Utilities|Array|Length _harbors_local) 0) _harbors_local))

(fn BuildCountryData
  (bind _country_map (Variables|Default|GetCountry%20Map))
  (bind _outactors (Actor|GetAllActorsOfClass "/Game/Blueprints/Countries/BP_Country.BP_Country_C"))
  (for _array_element _outactors
    (Utilities|Array|Add (Variables|Default|GetCountries) _array_element)
    (Utilities|Map|Add (Variables|Default|GetCountry%20Map) (Utilities|GetClass _array_element) _array_element))
  (Utilities|FlowControl|Sequence
    (:then_0
      (for _array_element_2 (Variables|Default|GetCountries)
        (Default|ConnectCountries _array_element_2 _country_map)))
    (:then_1
      (return (Variables|Default|GetCountries) _country_map))))

(fn GetCountries
  (bind _countries (Variables|Default|GetCountries))
  (if (Utilities|Array|IsEmpty _countries)
    (bind _countries_2 (CallFunction|BuildCountryData))
    (return _countries_2)
    (else
      (return _countries))))

(fn GetCountryMap
  (bind _country_map (Variables|Default|GetCountry%20Map))
  (if (Utilities|Map|IsEmpty _country_map)
    (bind _country_map_2 (CallFunction|BuildCountryData))
    (return _country_map_2)
    (else
      (return _country_map))))