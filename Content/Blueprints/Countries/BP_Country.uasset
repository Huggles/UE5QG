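; BP_Country is a land or water territory on a turn-based strategy board, holding units of races grouped into teams.
; Construction applies terrain material, supply star, harbor and label; BeginPlay resolves neighbors from class references and forwards clicks to the player controller.
; Queries derive ownership from units present, then decide build eligibility and supply.
; Supply groups recurse through neighbors holding the race's units, water requiring an adjacent land unit.
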(event Custom|On%20Unit%20Removed%20From%20Country
  (params (Unit :type BP%20Unit%20Object%20Reference))
  (Utilities|Array|RemoveItem (Variables|Default|GetUnits) Unit))

(event Custom|EvOnComponentClicked_Event
  (params (Clicked%20Actor :type Actor%20Object%20Reference) (TB%20Player%20State :type BP%20Turn%20Based%20Player%20State%20Object%20Reference) (TB%20Player%20Controller :type BP%20Turn%20Based%20Player%20Controller%20Object%20Reference))
  (bind _asbp_country (Utilities|Casting|CastToBP_Country Clicked%20Actor))
  (Default|OnClickedCountry(Client) TB%20Player%20Controller _asbp_country)
  (Development|PrintString (Utilities|String|Append "On Country Clicked: " (Utilities|GetDisplayName _asbp_country))))

(event Custom|On%20Unit%20Added%20To%20Country
  (params (Unit :type BP%20Unit%20Object%20Reference))
  (Utilities|Array|Add (Variables|Default|GetUnits) Unit))

(event Custom|Construct%20Country)

(event Custom|Set%20Home%20Space%20For%20Player
  (params (Race :type PlayableRaceEnum%20Enum :default "NewEnumerator6"))
  (bind _watchtower (Variables|Default|GetWatchTower))
  (bind _asbp_watch_tower (Utilities|Casting|CastToBP_WatchTower (Variables|/Script/Engine.ChildActorComponent|GetChildActor _watchtower)))
  (Default|SetPlayerRace _asbp_watch_tower Race)
  (Rendering|SetVisibility _watchtower true true))

(event EventBeginPlay
  (Utilities|FlowControl|Sequence
    (:then_0
      (Utilities|Array|Clear (Variables|Default|GetConnectedCountries))
      (for _array_element (Variables|CountryProperties|GetConnectedCountryClasses)
        (bind _outactors (Actor|GetAllActorsOfClass _array_element))
        (for _array_element_2 _outactors
          (Utilities|Array|Add (Variables|Default|GetConnectedCountries) _array_element_2))))
    (:then_1
      (EventDispatchers|AssignEvonComponentClicked (Variables|Default|GetClickableMesh) (delegate Custom|EvOnComponentClicked_Event)))))

(event EventIBuildUnit
  (params (Owning%20Player :type BP%20Turn%20Based%20Player%20State%20Object%20Reference) (Unit%20Type :type UnitTypeEnum%20Enum :default "NewEnumerator0")))

(fn ConstructionScript
  (Init|InitMaterial)
  (Init|InitGameplayElements))

(fn EmphasizeCountry
  (bind _countrymeshcomponent (Variables|Components|GetCountryMeshComponent))
  (if true
    (Transformation|SetRelativeScale3D _countrymeshcomponent (LocalVariables|Get_onHoverScale))
    (else
      (Transformation|SetRelativeScale3D _countrymeshcomponent (LocalVariables|Get_onNormalScale)))))

(fn GetAvailableUnitPos
  (if (Utilities|IsValid (Components|GetChildComponent (Variables|Default|GetUnitPos1) 0))
    (if (Utilities|IsValid (Components|GetChildComponent (Variables|Default|GetUnitPos2) 0))
      (if (Utilities|IsValid (Components|GetChildComponent (Variables|Default|GetUnitPos3) 0))
        (return 0)
        (else
          (return (Variables|Default|GetUnitPos3))))
      (else
        (return (Variables|Default|GetUnitPos2))))
    (else
      (return (Variables|Default|GetUnitPos1)))))

(fn EliminateUnit
  (params (Defender :type BP%20Unit%20Object%20Reference))
  (Actor|DestroyActor Defender)
  (return))

(fn GetUnitsinCountry
  (bind __units (LocalVariables|Get_units))
  (bind _outactors (Actor|GetAllActorsOfClass "/Game/Blueprints/Units/BP_Unit.BP_Unit_C"))
  (for _array_element _outactors
    (if (== (Variables|/Game/Blueprints/Units/BP_Unit.BP_Unit_C|GetCountry _array_element) self)
      (Utilities|Array|Add __units _array_element)))
  (return __units))

(fn GetCountryTeamOwner
  (bind _units_in_country (Units|GetUnitsinCountry))
  (if (== (Utilities|Array|Length _units_in_country) 0)
    (return "NewEnumerator0")
    (else
      (return (CallFunction|GetTeamforRace (Variables|/Game/Blueprints/Units/BP_Unit.BP_Unit_C|GetRace (Utilities|Array|Get(acopy) _units_in_country)))))))

(fn HasPlayerUnit
  (params (Race :type PlayableRaceEnum%20Enum :default "NewEnumerator6"))
  (bind _unit (Game|GetPlayerUnit Race))
  (return (Utilities|IsValid _unit) _unit))

(fn CanPlayerAttack
  (params (TB%20Player%20State :type BP%20Turn%20Based%20Player%20State%20Object%20Reference))
  (Game|GetCountryTeamOwner)
  (return false))

(fn CanRaceBuild
  (params (Playable%20Race :type PlayableRaceEnum%20Enum :default "NewEnumerator6"))
  (return (and (or (Game|IsAdjacentforRace Playable%20Race) (Game|IsHomeSpace Playable%20Race)) (and (not (Game|IsEnemyOwned (CallFunction|GetTeamforRace Playable%20Race))) (not (.Player%20Has%20Unit (Game|HasPlayerUnit Playable%20Race)))))))

(fn GetPlayerUnit
  (params (Race :type PlayableRaceEnum%20Enum :default "NewEnumerator6"))
  (for _array_element (Units|GetUnitsinCountry)
    (if (Utilities|Enum|Equal(Enum) (Variables|/Game/Blueprints/Units/BP_Unit.BP_Unit_C|GetRace _array_element) Race)
      (return _array_element)))
  (return 0))

(fn IsHomeSpace
  (params (Playable%20Race :type PlayableRaceEnum%20Enum :default "NewEnumerator6"))
  (return (== (Utilities|GetClass self) (.homespace (Default|GetRaceStructStructforRace (CallFunction|TBGameState) Playable%20Race)))))

(fn IsEnemyOwned
  (params (team :type TeamEnum%20Enum :default "NewEnumerator0"))
  (bind _team (Game|GetCountryTeamOwner))
  (return (or (and (Utilities|Enum|Equal(Enum) _team "NewEnumerator2") (Utilities|Enum|Equal(Enum) team "NewEnumerator1")) (and (Utilities|Enum|Equal(Enum) _team "NewEnumerator1") (Utilities|Enum|Equal(Enum) team "NewEnumerator2")))))

(fn IsTeamOwned
  (params (Team :type TeamEnum%20Enum :default "NewEnumerator0"))
  (bind _team (Game|GetCountryTeamOwner))
  (return (Utilities|Enum|Equal(Enum) _team Team)))

(fn IsCountryEmpty
  (return (== (Utilities|Array|Length (Units|GetUnitsinCountry)) 0)))

(fn IsAdjacentforRace
  (params (Playable%20Race :type PlayableRaceEnum%20Enum :default "NewEnumerator6"))
  (for _array_element (Variables|Default|GetConnectedCountries)
    (LocalVariables|SetPlayer%20Is%20Adjacent%20Local (or (LocalVariables|GetPlayer%20Is%20Adjacent%20Local) (.Player%20Has%20Unit (Game|HasPlayerUnit _array_element Playable%20Race)))))
  (return (LocalVariables|GetPlayer%20Is%20Adjacent%20Local)))

(fn InitMaterial
  (bind __landmaterial (LocalVariables|Get_landMaterial))
  (bind __watermaterial (LocalVariables|Get_waterMaterial))
  (switch Utilities|FlowControl|Switch|SwitchonCountryTypeEnum (Variables|CountryProperties|GetCountry%20Type)
    (:NewEnumerator0
      (if (!= (Variables|Default|GetOriginal%20Material) (LocalVariables|Get_landMaterial))
        (Rendering|Material|SetMaterial (Variables|Components|GetCountryMeshComponent) 0 __landmaterial)
        (Variables|Default|SetOriginal%20Material __landmaterial)))
    (:NewEnumerator1
      (if (!= (Variables|Default|GetOriginal%20Material) (LocalVariables|Get_waterMaterial))
        (Rendering|Material|SetMaterial (Variables|Components|GetCountryMeshComponent) 0 __watermaterial)
        (Variables|Default|SetOriginal%20Material __watermaterial)))))

(fn InitGameplayElements
  (Utilities|FlowControl|Sequence
    (:then_0
      (Rendering|SetVisibility (Variables|Default|GetSupplyStar) (Variables|CountryProperties|GetIsSupply) true))
    (:then_1
      (Rendering|SetVisibility (Variables|Default|GetBP_Harbor) (Variables|CountryProperties|GetIsHarbor) true))
    (:then_3
      (Variables|/Script/Text3D.Text3DComponent|SetText (Variables|Default|GetText3D) (Utilities|Text|ToText(String) (Variables|CountryProperties|GetLabel))))))

(fn GetAdjacentCountires
  (return (Variables|Default|GetConnectedCountries)))

(fn IsWater
  (return (Utilities|Enum|Equal(Enum) (Variables|CountryProperties|GetCountry%20Type) "NewEnumerator1")))

(fn IsLand
  (return (Utilities|Enum|Equal(Enum) (Variables|CountryProperties|GetCountry%20Type) "NewEnumerator0")))

(fn CalculateIsCountryClickable
  (Default|SetClickable (Variables|Default|GetClickableMesh) (Utilities|Array|ContainsItem (Variables|/Game/Blueprints/Game/BP_TurnBasedPlayerState.BP_TurnBasedPlayerState_C|GetClickableActors (Default|TBPlayerState (CallFunction|GetFirstLocalTBPlayerController))) self)))

(fn SupplyGroupforRace
  (params (Race :type PlayableRaceEnum%20Enum :default "NewEnumerator0") (Processed%20Countries :type Array%20of%20BP%20Country%20Object%20References))
  (LocalVariables|SetProcessed%20Countries%20Local Processed%20Countries)
  (Utilities|Array|AddUnique (LocalVariables|GetProcessed%20Countries%20Local) self)
  (if (and (.Player%20Has%20Unit (Game|HasPlayerUnit Race)) (select (Utilities|IsWater) (Game|HasHarbor Race) true))
    (Utilities|Array|AddUnique (LocalVariables|GetCountries%20Local) self)
    (for _array_element (Game|GetAdjacentCountires)
      (if (not (Utilities|Array|ContainsItem (LocalVariables|GetProcessed%20Countries%20Local) _array_element))
        (Development|PrintString (Utilities|GetDisplayName _array_element))
        (Utilities|FlowControl|Sequence
          (:then_0
            (for _array_element_2 (.Supply%20Group%20Countries (Game|SupplyGroupforRace _array_element Race (LocalVariables|GetProcessed%20Countries%20Local)))
              (Utilities|Array|AddUnique (LocalVariables|GetCountries%20Local) _array_element_2)))
          (:then_1
            (for _array_element_3 (.Processed%20Countrie (Game|SupplyGroupforRace _array_element Race (LocalVariables|GetProcessed%20Countries%20Local)))
              (Utilities|Array|AddUnique (LocalVariables|GetProcessed%20Countries%20Local) _array_element_3)))))))
  (return (LocalVariables|GetCountries%20Local) (LocalVariables|GetProcessed%20Countries%20Local)))

(fn HasHarbor
  (params (Race :type PlayableRaceEnum%20Enum :default "NewEnumerator0"))
  (for _array_element (Game|GetAdjacentCountires)
    (if (and (Utilities|IsLand _array_element) (.Player%20Has%20Unit (Game|HasPlayerUnit _array_element Race)))
      (return true)))
  (return false))

(fn ProvidesSupplyforRace
  (params (Race :type PlayableRaceEnum%20Enum :default "NewEnumerator0"))
  (return (and (or (Game|IsHomeSpace Race) (.Player%20Has%20Unit (Game|HasPlayerUnit Race))) (Variables|CountryProperties|GetIsSupply))))

(fn FnHighlightConnected
  (params (Highlight :type Boolean))
  (for _array_element (Variables|Default|GetConnectedCountries)
    (Default|FnHighlightSelf _array_element Highlight)))

(fn FnHighlightSelf
  (params (Highlight :type Boolean) (Trigger :type Actor%20Object%20Reference))
  (bind _countrymeshcomponent (Variables|Components|GetCountryMeshComponent))
  (if true
    (if (== Trigger (Components|GetOwner))
      (Rendering|Material|SetMaterial _countrymeshcomponent 0 "/Game/Material/World/M_Highlighted_Self.M_Highlighted_Self")
      (else
        (Rendering|Material|SetMaterial _countrymeshcomponent 0 "/Game/Material/World/M_Highlighted_Connected.M_Highlighted_Connected")))
    (else
      (Rendering|Material|SetMaterial _countrymeshcomponent 0 (Variables|Default|GetOriginal%20Material)))))

(fn FnonClick
  (bind _self self)
  (bind _countrymeshcomponent (Variables|Components|GetCountryMeshComponent))
  (Development|PrintString (Utilities|String|Append (Utilities|GetDisplayName _self) (Utilities|GetDisplayName _countrymeshcomponent)))
  (return _self _countrymeshcomponent))