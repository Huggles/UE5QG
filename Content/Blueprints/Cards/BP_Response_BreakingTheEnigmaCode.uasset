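; Response card Blueprint for Breaking the Enigma Code, a card keyed to enemy control of Western Europe.
; RelevantUnits returns the units in Western Europe when that country is enemy-owned relative to the card's team, and Playable requires exactly one.
; The server activation event calls the parent, then checks Activatable, which always returns true.
; No card-specific effect is implemented, as that branch and ExecuteCard are empty.
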(event EventExecuteCard)

(event EventBeginPlay
  (|CallParentFunction))

(event EventActivateCardEffect(Server)
  (params (Callback :type I%20Effective%20Card%20Callback%20Interface))
  (|CallParentFunction Callback)
  (if (CallFunction|Activatable)
    _))

(fn ConstructionScript
  (|CallParentFunction))

(fn Playable
  (return (== (Utilities|Array|Length (CallFunction|RelevantUnits)) 1)))

(fn RelevantUnits
  (bind _bp_world (CallFunction|BPWorld))
  (bind _countrymap (Variables|/Game/Blueprints/Countries/BP_World.BP_World_C|GetCountryMap _bp_world))
  (bind _value (Utilities|Map|Find _countrymap "/Game/Blueprints/Countries/BP_WesternEurope.BP_WesternEurope_C"))
  (if (Default|IsEnemyOwned _value (CallFunction|GetTeamforRace (Variables|/Game/DataAssets/PDA_Card.PDA_Card_C|GetRace (Variables|Default|GetCardAsset))))
    (return (Default|GetUnitsinCountry _value))))

(fn Activatable
  (return true))