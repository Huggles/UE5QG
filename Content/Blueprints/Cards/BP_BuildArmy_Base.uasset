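; BP_BuildArmy_Base is a base card that lets a race build a unit on a land country.
; On execution, a server-side select command offers the valid countries, and its finish callback passes the chosen one to the ability factory's build-unit ability.
; Valid targets are land neighbours of the race's occupied countries, supplied or not, plus its home space, excluding enemy-owned or already occupied-by-that-race spaces.
; The card is playable only when a target exists.
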(event Custom|CommandFinished_Event_0
  (params (Command :type BP%20Command%20Object%20Reference))
  (Default|BuildUnit(Ability) (CallFunction|AbilityFactory) self (Default|GetSelectedCountry (stale EventExecuteCard(Protected) _select_actor_client_command)) (CallFunction|CardRace) "NewEnumerator0" true true true))

(event EventExecuteCard(Protected)
  (bind _select_actor_client_command (CallFunction|SelectActor(Command) (CallFunction|Controller(ServerOnly)) (CallFunction|RelevantCountriesonPlay)))
  (EventDispatchers|AssignCommandFinished _select_actor_client_command (delegate Custom|CommandFinished_Event_0)))

(event EventBeginPlay
  (|CallParentFunction))

(fn ConstructionScript
  (|CallParentFunction))

(fn RelevantCountriesonPlay
  (bind _race (CallFunction|CardRace))
  (bind _race_2 (CallFunction|CardRace))
  (bind _home_space_country (CallFunction|GetHomeSpaceforRace _race))
  (Utilities|FlowControl|Sequence
    (:then_0
      (for _array_element (Default|GetAllOccupiedCountriesforRace (CallFunction|BPWorld) (CallFunction|CardRace) false)
        (for _array_element_2 (Default|GetAdjacentCountires _array_element)
          (if (Math|Boolean|ANDBoolean (Default|IsLand _array_element_2) (not (Default|IsEnemyOwned _array_element_2 (CallFunction|GetTeamforRace _race_2))) (not (.Player%20Has%20Unit (Default|HasPlayerUnit _array_element_2 _race_2))))
            (Utilities|Array|AddUnique (LocalVariables|GetRelevant%20Countries) _array_element_2)))))
    (:then_1
      (if (and (not (.Player%20Has%20Unit (Default|HasPlayerUnit _home_space_country _race))) (not (Default|IsEnemyOwned _home_space_country (CallFunction|CardTeam))))
        (Utilities|Array|AddUnique (LocalVariables|GetRelevant%20Countries) _home_space_country)))
    (:then_2
      (return (LocalVariables|GetRelevant%20Countries)))))

(fn Playable
  (return (> (Utilities|Array|Length (CallFunction|RelevantCountriesonPlay)) 0)))