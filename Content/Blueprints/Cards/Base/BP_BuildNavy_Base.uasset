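; Base Blueprint for navy-building cards, which place a naval unit for the card's faction in a chosen country.
; Eligible countries are adjacent, supplied water spaces that are not enemy-owned, hold no unit of that faction and allow navy building.
; The card is playable when any such country exists.
; Playing it issues a mandatory actor-selection command, whose completion event triggers the build-unit ability on the selected country.
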(event Custom|CommandFinished_Event_0
  (params (Command :type BP%20Command%20Object%20Reference) (Result :type Command%20Result%20Structure))
  (Default|BuildUnit(Ability) (CallFunction|AbilityFactory) self (.country Result) (CallFunction|CardFaction) "NewEnumerator1" true true true))

(event EventBeginPlay
  (|CallParentFunction))

(event EventPlayCardImplementation
  (bind _select_actor_client_command (CallFunction|SelectActor(Command) (CallFunction|Controller(ServerOnly)) (.Relevant%20Actors (CallFunction|RelevantActorsonPlay (CallFunction|CardFaction))) false))
  (EventDispatchers|AssignCommandFinished _select_actor_client_command (delegate Custom|CommandFinished_Event_0)))

(fn ConstructionScript
  (|CallParentFunction))

(fn RelevantCountriesonPlay
  (params (Placed%20Units :type Array%20of%20BP%20Unit%20Object%20References) (Occupied%20Countries :type Array%20of%20BP%20Country%20Object%20References) (Adjacent%20Countries :type Array%20of%20BP%20Country%20Object%20References) (Adjacent%20Supplied%20Countries :type Array%20of%20BP%20Country%20Object%20References))
  (bind _faction (CallFunction|CardFaction))
  (for _array_element Adjacent%20Supplied%20Countries
    (if (Default|IsWater _array_element)
      (if (Math|Boolean|ANDBoolean (Default|IsWater _array_element) (not (Default|IsEnemyOwned _array_element (CallFunction|GetTeamforRace (CallFunction|CardFaction)))) (not (.Player%20Has%20Unit (Default|HasPlayerUnit _array_element _faction))) (Default|CanBuildNavy _array_element _faction))
        (Utilities|Array|AddUnique (LocalVariables|GetRelevant%20Countries%20Local) _array_element))))
  (return (LocalVariables|GetRelevant%20Countries%20Local)))

(fn Playable
  (return (> (Utilities|Array|Length (.Relevant%20Countries (CallFunction|RelevantActorsonPlay (CallFunction|CardFaction)))) 0)))