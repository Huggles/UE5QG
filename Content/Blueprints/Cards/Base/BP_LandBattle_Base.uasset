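; Base Blueprint for Land Battle cards, which let the card's faction attack an enemy unit or an empty country on adjacent land.
; Overrides gather units in adjacent enemy-owned land countries and empty adjacent land countries as targets; the card is playable only when relevant targets exist.
; Playing it issues a non-skippable selection command to the server-only controller, then hands the result to the ability factory as a unit or country attack.
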(event Custom|CommandFinished_Event_0
  (params (Command :type BP%20Command%20Object%20Reference) (Result :type Command%20Result%20Structure))
  (if (Utilities|IsValid (.unit Result))
    (Default|AttackUnit(Ability) (CallFunction|AbilityFactory) self (.unit Result) true true)
    (elif (Utilities|IsValid (.country Result))
      (Default|AttackCountry(Ability) (CallFunction|AbilityFactory) self (.country Result) true true)
      (else
        (Development|PrintString "Nothing Was Selected?")))))

(event EventPlayCardImplementation
  (bind _select_actor_client_command (CallFunction|SelectActor(Command) (CallFunction|Controller(ServerOnly)) (.Relevant%20Actors (CallFunction|RelevantActorsonPlay (CallFunction|CardFaction))) false))
  (EventDispatchers|AssignCommandFinished _select_actor_client_command (delegate Custom|CommandFinished_Event_0)))

(event EventBeginPlay
  (|CallParentFunction))

(fn ConstructionScript
  (|CallParentFunction))

(fn RelevantUnitsonPlay
  (params (Placed%20Units :type Array%20of%20BP%20Unit%20Object%20References) (Occupied%20Countries :type Array%20of%20BP%20Country%20Object%20References) (Adjacent%20Countries :type Array%20of%20BP%20Country%20Object%20References) (Adjacent%20Supplied%20Countries :type Array%20of%20BP%20Country%20Object%20References))
  (for _array_element Adjacent%20Countries
    (if (and (Default|IsLand _array_element) (Default|IsEnemyOwned _array_element (CallFunction|GetTeamforRace (CallFunction|CardFaction))))
      (for _array_element_2 (Variables|/Game/Blueprints/Countries/BP_Country.BP_Country_C|GetUnits _array_element)
        (Utilities|Array|AddUnique (LocalVariables|GetRelevant%20Units%20Local) _array_element_2))))
  (return (LocalVariables|GetRelevant%20Units%20Local)))

(fn Playable
  (return (> (Utilities|Array|Length (.Relevant%20Actors (CallFunction|RelevantActorsonPlay (CallFunction|CardFaction)))) 0)))

(fn RelevantCountriesonPlay
  (params (Placed%20Units :type Array%20of%20BP%20Unit%20Object%20References) (Occupied%20Countries :type Array%20of%20BP%20Country%20Object%20References) (Adjacent%20Countries :type Array%20of%20BP%20Country%20Object%20References) (Adjacent%20Supplied%20Countries :type Array%20of%20BP%20Country%20Object%20References))
  (for _array_element Adjacent%20Countries
    (if (and (Default|IsCountryEmpty _array_element) (Default|IsLand _array_element))
      (Utilities|Array|AddUnique (LocalVariables|GetEmpty%20Countries) _array_element)))
  (return (LocalVariables|GetEmpty%20Countries)))