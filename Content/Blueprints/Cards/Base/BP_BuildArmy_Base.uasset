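; Base Blueprint for a Build Army card, which lets the card's faction build a unit in a chosen country.
; Valid targets are adjacent land countries without enemy ownership or the faction's own unit, plus the home space if likewise free.
; Playing it issues a mandatory server-controller selection command, whose finished callback hands the chosen country to the build-unit ability.
; The card is playable only when at least one valid target exists.
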(event Custom|CommandFinished_Event_0
  (params (Command :type BP%20Command%20Object%20Reference) (Result :type Command%20Result%20Structure))
  (Default|BuildUnit(Ability) (CallFunction|AbilityFactory) self (.country Result) (CallFunction|CardFaction) "NewEnumerator0" true true true))

(event EventPlayCardImplementation
  (bind _select_actor_client_command (CallFunction|SelectActor(Command) (CallFunction|Controller(ServerOnly)) (.Relevant%20Actors (CallFunction|RelevantActorsonPlay (CallFunction|CardFaction))) false))
  (EventDispatchers|AssignCommandFinished _select_actor_client_command (delegate Custom|CommandFinished_Event_0)))

(event EventBeginPlay
  (|CallParentFunction))

(fn ConstructionScript
  (|CallParentFunction))

(fn RelevantCountriesonPlay
  (params (Occupied%20Countries :type Array%20of%20BP%20Country%20Object%20References) (Adjacent%20Countries :type Array%20of%20BP%20Country%20Object%20References) (Placed%20Units :type Array%20of%20BP%20Unit%20Object%20References))
  (bind _faction (CallFunction|CardFaction))
  (bind _faction_2 (CallFunction|CardFaction))
  (bind _home_space_country (CallFunction|GetHomeSpaceforRace _faction))
  (Utilities|FlowControl|Sequence
    (:then_0
      (for _array_element Adjacent%20Countries
        (if (Math|Boolean|ANDBoolean (Default|IsLand _array_element) (not (Default|IsEnemyOwned _array_element (CallFunction|GetTeamforRace _faction_2))) (not (.Player%20Has%20Unit (Default|HasPlayerUnit _array_element _faction_2))))
          (Utilities|Array|AddUnique (LocalVariables|GetRelevant%20Countries) _array_element))))
    (:then_1
      (if (and (not (.Player%20Has%20Unit (Default|HasPlayerUnit _home_space_country _faction))) (not (Default|IsEnemyOwned _home_space_country (CallFunction|CardTeam))))
        (Utilities|Array|AddUnique (LocalVariables|GetRelevant%20Countries) _home_space_country)))
    (:then_2
      (return (LocalVariables|GetRelevant%20Countries)))))

(fn Playable
  (return (> (Utilities|Array|Length (.Relevant%20Actors (CallFunction|RelevantActorsonPlay (CallFunction|CardFaction)))) 0)))