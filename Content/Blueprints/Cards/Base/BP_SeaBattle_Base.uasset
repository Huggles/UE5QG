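; Base Blueprint for sea battle cards, which let a player attack a unit or country in adjacent water.
; Valid targets are units in adjacent enemy-owned water countries plus any empty adjacent water country, and the card is playable only if one exists.
; Playing it runs a non-skippable select-actor command on the controller, then triggers the ability factory's attack-country or attack-unit ability based on the selection.
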(event Custom|CommandFinished_Event_0
  (params (Command :type BP%20Command%20Object%20Reference) (Result :type Command%20Result%20Structure))
  (bind _ability_factory (CallFunction|AbilityFactory))
  (bind _self self)
  (if (Utilities|IsValid (.country Result))
    (Default|AttackCountry(Ability) _ability_factory _self (.country Result) true true)
    (elif (Utilities|IsValid (.unit Result))
      (Default|AttackUnit(Ability) _ability_factory _self (.unit Result) true true))))

(event EventPlayCardImplementation
  (bind _select_actor_client_command (CallFunction|SelectActor(Command) (CallFunction|Controller(ServerOnly)) (.Relevant%20Actors (CallFunction|RelevantActorsonPlay)) false))
  (EventDispatchers|AssignCommandFinished _select_actor_client_command (delegate Custom|CommandFinished_Event_0)))

(event EventBeginPlay
  (|CallParentFunction))

(fn ConstructionScript
  (|CallParentFunction))

(fn RelevantUnitsonPlay
  (params (Occupied%20Countries :type Array%20of%20BP%20Country%20Object%20References) (Adjacent%20Countries :type Array%20of%20BP%20Country%20Object%20References) (Placed%20Units :type Array%20of%20BP%20Unit%20Object%20References))
  (for _array_element Adjacent%20Countries
    (if (and (Default|IsWater _array_element) (Default|IsEnemyOwned _array_element (CallFunction|GetTeamforRace (CallFunction|CardRace))))
      (for _array_element_2 (Variables|/Game/Blueprints/Countries/BP_Country.BP_Country_C|GetUnits _array_element)
        (Utilities|Array|AddUnique (LocalVariables|GetRelevant%20Units%20Local) _array_element_2))))
  (return (LocalVariables|GetRelevant%20Units%20Local)))

(fn RelevantCountriesonPlay
  (params (Occupied%20Countries :type Array%20of%20BP%20Country%20Object%20References) (Adjacent%20Countries :type Array%20of%20BP%20Country%20Object%20References) (Placed%20Units :type Array%20of%20BP%20Unit%20Object%20References))
  (for _array_element Adjacent%20Countries
    (if (and (Default|IsCountryEmpty _array_element) (Default|IsWater _array_element))
      (Utilities|Array|AddUnique (LocalVariables|GetEmpty%20Countries) _array_element)))
  (return (LocalVariables|GetEmpty%20Countries)))

(fn Playable
  (return (> (Utilities|Array|Length (.Relevant%20Actors (CallFunction|RelevantActorsonPlay))) 0)))