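; Sturmfuhrer event card: replaces an enemy unit in Western Europe with one from the card race's unit pool.
; It is playable only when Western Europe is enemy-owned and holds exactly one unit, which becomes clickable on execution.
; The click adds the pool unit, then queues blocking camera, destroy and build animations on the server animation manager.
; When they finish, it removes the old unit from the country and completes the card's actions.
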(event Custom|AllAnimationsFinished_Event_0
  (EventDispatchers|UnbindEventfromAllAnimationsFinished (CallFunction|ServerAnimationManager) (delegate Custom|AllAnimationsFinished_Event_0))
  (Default|RemoveUnitfromCountry (Variables|Default|GetSelected%20Unit))
  (Default|CallCardActionsFinished))

(event Custom|On%20Unit%20Clicked
  (params (Unit :type BP%20Unit%20Object%20Reference) (TB%20Player%20State :type BP%20Turn%20Based%20Player%20State%20Object%20Reference) (TB%20Player%20Controller :type BP%20Turn%20Based%20Player%20Controller%20Object%20Reference))
  (if (== TB%20Player%20Controller (Variables|Default|GetPlayer%20Controller))
    (EventDispatchers|UnbindEventfromUnitClicked (CallFunction|BPWorld) (delegate Custom|On%20Unit%20Clicked))
    (Variables|Default|SetSelected%20Unit Unit)
    (Variables|/Game/Blueprints/Game/BP_TurnBasedPlayerState.BP_TurnBasedPlayerState_C|SetClickableActors (Variables|Default|GetPlayer%20State) (Utilities|Array|MakeArray))
    (bind _unit_pool (CallFunction|GetUnitPool (Variables|/Game/DataAssets/PDA_Card.PDA_Card_C|GetRace (Variables|Default|GetCardAsset))))
    (bind _unit (Default|GetAvailableUnit _unit_pool "NewEnumerator0"))
    (Default|AddUnittoCountry _unit (.Value (Utilities|Map|Find (Variables|/Game/Blueprints/Countries/BP_World.BP_World_C|GetCountryMap (CallFunction|BPWorld)) "/Game/Blueprints/Countries/BP_WesternEurope.BP_WesternEurope_C")))
    (Default|AddAnimations (CallFunction|ServerAnimationManager) (Utilities|Array|MakeArray (Utilities|Struct|MakeCA_Payload "/Game/ClientAnimations/BP_Animation_MoveCamera.BP_Animation_MoveCamera_C" true 1.0 0 0 true 0 "0.000000,0.000000,0.000000" (+ (Transformation|GetActorLocation (Variables|Default|GetSelected%20Unit)) "0.000000,600.000000,1000.000000") "1.000000,1.000000,1.000000" 0) (Utilities|Struct|MakeCA_Payload "/Game/ClientAnimations/BP_Animation_DestroyUnit.BP_Animation_DestroyUnit_C" true 2.0 (Utilities|Array|MakeArray (Variables|Default|GetSelected%20Unit)) 0 true 0 "0.000000,0.000000,0.000000" "0.000000,0.000000,0.000000" "5.000000,5.000000,5.000000" "/Game/StarterContent/Particles/P_Explosion.P_Explosion") (Utilities|Struct|MakeCA_Payload "/Game/ClientAnimations/BP_Animation_BuildUnit.BP_Animation_BuildUnit_C" true 1.0 (Utilities|Array|MakeArray _unit) 0 true 0 "0.000000,0.000000,0.000000" "0.000000,0.000000,0.000000" "1.000000,1.000000,1.000000" 0) (Utilities|Struct|MakeCA_Payload "/Game/ClientAnimations/BP_Animation_ReturnCamera.BP_Animation_ReturnCamera_C" true 1.0 0 0 true 0 "0.000000,0.000000,0.000000" "0.000000,0.000000,0.000000" "1.000000,1.000000,1.000000" 0)))
    (EventDispatchers|AssignAllAnimationsFinished (CallFunction|ServerAnimationManager) (delegate Custom|AllAnimationsFinished_Event_0))))

(event EventExecuteCard
  (Default|ChangeUIState (Variables|Default|GetPlayer%20Controller) "NewEnumerator6")
  (EventDispatchers|AssignUnitClicked (CallFunction|BPWorld) (delegate Custom|On%20Unit%20Clicked))
  (Variables|/Game/Blueprints/Game/BP_TurnBasedPlayerState.BP_TurnBasedPlayerState_C|SetClickableActors (Variables|Default|GetPlayer%20State) (CallFunction|RelevantUnits)))

(event EventBeginPlay
  (|CallParentFunction))

(fn ConstructionScript
  (Rendering|Components|Sprite|SetSprite (Variables|Default|GetPaperSprite_0) (Variables|/Game/DataAssets/PDA_Card.PDA_Card_C|GetSprite (Variables|Default|GetCardAsset))))

(fn Playable
  (return (== (Utilities|Array|Length (CallFunction|RelevantUnits)) 1)))

(fn RelevantUnits
  (bind _bp_world (CallFunction|BPWorld))
  (bind _countrymap (Variables|/Game/Blueprints/Countries/BP_World.BP_World_C|GetCountryMap _bp_world))
  (bind _value (Utilities|Map|Find _countrymap "/Game/Blueprints/Countries/BP_WesternEurope.BP_WesternEurope_C"))
  (if (Default|IsEnemyOwned _value (CallFunction|GetTeamforRace (Variables|/Game/DataAssets/PDA_Card.PDA_Card_C|GetRace (Variables|Default|GetCardAsset))))
    (return (Default|GetUnitsinCountry _value))))