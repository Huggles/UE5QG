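; Italy response card "German Reinforcements Counterattack" for the card game.
; It is always playable and defers its play and activation logic to the parent class.
; It can be activated as a response when the triggering ability's origin card is of a specific type and the card faction check matches a specific faction.
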(event EventActivateCardImplementation
  (params (Ability%20Trigger :type BP%20Ability%20Object%20Reference))
  (|CallParentFunction Ability%20Trigger))

(event EventPlayCardImplementation
  (|CallParentFunction))

(fn ConstructionScript
  (|CallParentFunction))

(fn Playable
  (return true))

(fn CanbeActivatedasResponse
  (params (Ability :type BP%20Ability%20Object%20Reference))
  (return (and (Utilities|Enum|Equal(Enum) (Default|CardType (Variables|/Game/Blueprints/Abilities/BP_Ability.BP_Ability_C|GetOrigin%20Card Ability)) "NewEnumerator3") (Utilities|Enum|Equal(Enum) (CallFunction|CardFaction) "NewEnumerator0"))))