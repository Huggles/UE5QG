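; United Kingdom event card "King Peter Enthroned in Yugoslavia": attacks an enemy unit in the Balkans, then recruits an army there.
; Playable when the Balkans are enemy-owned or hold no units of the card's faction.
; AbilityFactory commands drive target selection and attack; RecruitArmy follows the finished attack, or runs directly if no target exists.
; An impossible deployment ends the card; other finished abilities pass to the parent.
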(event Custom|Recruit%20Army
  (bind _deployment_possible (Default|DeployUnitifPossible(Ability) (CallFunction|AbilityFactory) self (.Value (Utilities|Map|Find (Default|GetCountryMap (CallFunction|BPWorld)) "/Game/Blueprints/Countries/BP_Balkans.BP_Balkans_C")) (CallFunction|CardFaction) "NewEnumerator0" "NewEnumerator1"))
  (if (not _deployment_possible)
    (CallFunction|CardExecutionFinished)))

(event Custom|CommandFinished_Event_0
  (params (Command :type BP%20Command%20Object%20Reference) (Result :type Command%20Result%20Structure))
  (if (not (.skipped Result))
    (bind _attack_unit_ability (Default|AttackUnit(Ability) (CallFunction|AbilityFactory) self (.unit Result)))
    (Variables|Default|SetAttack%20Unit%20Ability _attack_unit_ability)))

(event EventPlayCardImplementation
  (bind (_enemy_units_found _select_actor_client_command) (Default|SelectEnemyUnitifPossible(Command) (CallFunction|AbilityFactory) (Variables|Default|GetPlayer%20Controller) (CallFunction|CardFaction) (.Value (Utilities|Map|Find (Default|GetCountryMap (CallFunction|BPWorld)) "/Game/Blueprints/Countries/BP_Balkans.BP_Balkans_C"))))
  (if _enemy_units_found
    (EventDispatchers|AssignCommandFinished _select_actor_client_command (delegate Custom|CommandFinished_Event_0))
    (else
      (CallFunction|RecruitArmy))))

(event EventAbilityFinished
  (params (Ability :type BP%20Ability%20Object%20Reference))
  (if (== Ability (Variables|Default|GetAttack%20Unit%20Ability))
    (CallFunction|RecruitArmy)
    (else
      (|CallParentFunction Ability))))

(fn ConstructionScript
  (|CallParentFunction))

(fn Playable
  (bind _bp_world (CallFunction|BPWorld))
  (bind _country_map (Default|GetCountryMap _bp_world))
  (bind _value (Utilities|Map|Find _country_map "/Game/Blueprints/Countries/BP_Balkans.BP_Balkans_C"))
  (return (or (Default|IsEnemyOwned _value (CallFunction|CardTeam)) (not (.Has%20Units (Default|FactionHasUnits _value (CallFunction|CardFaction)))))))