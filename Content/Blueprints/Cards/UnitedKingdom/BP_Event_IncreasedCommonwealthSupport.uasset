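; United Kingdom event card "Increased Commonwealth Support" that builds a unit in Canada, India or Australia.
; Relevant countries are those three, filtered by whether the card's faction can recruit an army there; the card is playable only if any remain.
; Playing it issues a non-skippable select-actor command, whose completion calls the ability factory to build the unit in the chosen country.
; The filter removes entries from the array while looping over it.
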(event Custom|CommandFinished_Event_0
  (params (Command :type BP%20Command%20Object%20Reference) (Result :type Command%20Result%20Structure))
  (Default|BuildUnit(Ability) (CallFunction|AbilityFactory) self (.country Result) "NewEnumerator3" "NewEnumerator0" true true true))

(event EventPlayCardImplementation
  (bind _select_actor_client_command (CallFunction|SelectActor(Command) (CallFunction|Controller(ServerOnly)) (.Relevant%20Countries (CallFunction|RelevantActorsonPlay (CallFunction|CardFaction))) false))
  (EventDispatchers|AssignCommandFinished _select_actor_client_command (delegate Custom|CommandFinished_Event_0)))

(fn ConstructionScript
  (|CallParentFunction))

(fn RelevantCountriesonPlay
  (params (Occupied%20Countries :type Array%20of%20BP%20Country%20Object%20References) (Adjacent%20Countries :type Array%20of%20BP%20Country%20Object%20References) (Adjacent%20Countries%20In%20Supply :type Array%20of%20BP%20Country%20Object%20References) (Placed%20Units :type Array%20of%20BP%20Unit%20Object%20References))
  (bind _bp_world (CallFunction|BPWorld))
  (bind _countrymap (Variables|/Game/Blueprints/Countries/BP_World.BP_World_C|GetCountryMap _bp_world))
  (bind _output_get (LocalVariables|SetRCountriesLocal (Utilities|Array|MakeArray (.Value (Utilities|Map|Find _countrymap "/Game/Blueprints/Countries/BP_Canada.BP_Canada_C")) (.Value (Utilities|Map|Find _countrymap "/Game/Blueprints/Countries/BP_India.BP_India_C")) (.Value (Utilities|Map|Find _countrymap "/Game/Blueprints/Countries/BP_Australia.BP_Australia_C")))))
  (for _array_element _output_get
    (if (not (Default|CanRecruitArmy _array_element (CallFunction|CardFaction)))
      (Utilities|Array|RemoveItem (LocalVariables|GetRCountriesLocal) _array_element)))
  (return (LocalVariables|GetRCountriesLocal)))

(fn Playable
  (return (> (Utilities|Array|Length (.Relevant%20Countries (CallFunction|RelevantActorsonPlay (CallFunction|CardFaction)))) 0)))