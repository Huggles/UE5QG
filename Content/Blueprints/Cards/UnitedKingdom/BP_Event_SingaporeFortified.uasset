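; UK event card Singapore Fortified, which deploys a unit in South East Asia, then a navy in the South China Sea.
; It is playable if the card's faction can recruit an army or navy in the respective region.
; AbilityFinished chains the navy step after the first deployment, finishing the card if that step is impossible.
; An impossible first deployment triggers neither the navy step nor card completion in this graph.
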(event Custom|Recruit%20Navy
  (bind (_deployment_possible _deploy_unit_ability) (Default|DeployUnitifPossible(Ability) (CallFunction|AbilityFactory) self (.Value (Utilities|Map|Find (Default|GetCountryMap (CallFunction|BPWorld)) "/Game/Blueprints/Countries/BP_SouthChinaSea.BP_SouthChinaSea_C")) (CallFunction|CardFaction) "NewEnumerator1" "NewEnumerator1"))
  (if _deployment_possible
    (Variables|Default|SetDeploy%20Unit%20Ability _deploy_unit_ability)
    (else
      (CallFunction|CardExecutionFinished))))

(event EventPlayCardImplementation
  (bind (_deployment_possible _deploy_unit_ability) (Default|DeployUnitifPossible(Ability) (CallFunction|AbilityFactory) self (.Value (Utilities|Map|Find (Default|GetCountryMap (CallFunction|BPWorld)) "/Game/Blueprints/Countries/BP_SouthEastAsia.BP_SouthEastAsia_C")) (CallFunction|CardFaction) "NewEnumerator0" "NewEnumerator1"))
  (if _deployment_possible
    (Variables|Default|SetBuild%20Unit%20Ability _deploy_unit_ability)))

(event EventAbilityFinished
  (params (Ability :type BP%20Ability%20Object%20Reference))
  (if (== Ability (Variables|Default|GetBuild%20Unit%20Ability))
    (CallFunction|RecruitNavy)
    (else
      (|CallParentFunction Ability))))

(fn ConstructionScript
  (|CallParentFunction))

(fn Playable
  (bind _faction (CallFunction|CardFaction))
  (bind _bp_world (CallFunction|BPWorld))
  (bind _country_map (Default|GetCountryMap _bp_world))
  (return (or (Default|CanRecruitArmy (.Value (Utilities|Map|Find _country_map "/Game/Blueprints/Countries/BP_SouthEastAsia.BP_SouthEastAsia_C")) _faction) (Default|CanRecruitNavy (.Value (Utilities|Map|Find _country_map "/Game/Blueprints/Countries/BP_SouthChinaSea.BP_SouthChinaSea_C")) _faction))))