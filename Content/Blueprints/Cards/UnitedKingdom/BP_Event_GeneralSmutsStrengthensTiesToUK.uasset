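; United Kingdom event card "General Smuts Strengthens Ties to UK" that deploys an army in Africa, then a navy in Bay of Bengal or Southern Ocean.
; The army step runs through the ability factory, and its completion, or ineligibility, triggers the navy check.
; A non-skippable select command offers seas filtered by removal during iteration, feeding the navy deployment.
; Playable checks only Africa and Southern Ocean, leaving Bay of Bengal unused.
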(event Custom|Check%20Navy%20Recruitment
  (bind _bp_world (CallFunction|BPWorld))
  (bind _recruitnavytargets (Variables|Default|GetRecruitNavyTargets))
  (bind _recruitnavytargets_2 (Variables|Default|GetRecruitNavyTargets))
  (bind _country_map (Default|GetCountryMap _bp_world))
  (Utilities|Array|Add _recruitnavytargets_2 (.Value (Utilities|Map|Find _country_map "/Game/Blueprints/Countries/BP_BayOfBengal.BP_BayOfBengal_C")))
  (Utilities|Array|Add _recruitnavytargets_2 (.Value (Utilities|Map|Find _country_map "/Game/Blueprints/Countries/BP_SouthernOcean.BP_SouthernOcean_C")))
  (for _array_element (Variables|Default|GetRecruitNavyTargets)
    (if (not (Default|CanRecruitNavy _array_element (CallFunction|CardFaction)))
      (Utilities|Array|RemoveItem (Variables|Default|GetRecruitNavyTargets) _array_element)))
  (if (Utilities|Array|IsNotEmpty _recruitnavytargets)
    (bind _select_actor_client_command (Default|SelectActor(Command) (CallFunction|AbilityFactory) (Variables|Default|GetPlayer%20Controller) _recruitnavytargets false))
    (bind _output_get (Variables|Default|SetSelect%20Actor%20Client%20Command _select_actor_client_command))
    (EventDispatchers|AssignCommandFinished _output_get (delegate Custom|CommandFinished_Event_1))
    (else
      (CallFunction|CardExecutionFinished))))

(event Custom|CommandFinished_Event_1
  (params (Command :type BP%20Command%20Object%20Reference) (Result :type Command%20Result%20Structure))
  (bind (_skipped _country) (Utilities|Struct|BreakCommandResult Result))
  (bind _select_actor_client_command (Variables|Default|GetSelect%20Actor%20Client%20Command))
  (if (== Command _select_actor_client_command)
    (EventDispatchers|UnbindEventfromCommandFinished _select_actor_client_command (delegate Custom|CommandFinished_Event_1))
    (if _skipped
      (CallFunction|CardExecutionFinished)
      (else
        (Default|DeployUnit(Ability) (CallFunction|AbilityFactory) self _country (CallFunction|CardFaction) "NewEnumerator1" "NewEnumerator1")))))

(event EventPlayCardImplementation
  (bind _bp_world (CallFunction|BPWorld))
  (bind _country_map (Default|GetCountryMap _bp_world))
  (bind _value (Utilities|Map|Find _country_map "/Game/Blueprints/Countries/BP_Africa.BP_Africa_C"))
  (if (Default|CanRecruitArmy _value (CallFunction|CardFaction))
    (bind _build_unit_ability (Default|DeployUnit(Ability) (CallFunction|AbilityFactory) self _value (CallFunction|CardFaction) "NewEnumerator0" "NewEnumerator1"))
    (Variables|Default|SetBuild%20Unit%20Ability _build_unit_ability)
    (else
      (CallFunction|CheckNavyRecruitment))))

(event EventAbilityFinished
  (params (Ability :type BP%20Ability%20Object%20Reference))
  (if (== Ability (Variables|Default|GetBuild%20Unit%20Ability))
    (CallFunction|CheckNavyRecruitment)
    (else
      (|CallParentFunction Ability))))

(fn ConstructionScript
  (|CallParentFunction))

(fn Playable
  (bind _faction (CallFunction|CardFaction))
  (bind _bp_world (CallFunction|BPWorld))
  (bind _country_map (Default|GetCountryMap _bp_world))
  (return (or (Default|CanRecruitArmy (.Value (Utilities|Map|Find _country_map "/Game/Blueprints/Countries/BP_Africa.BP_Africa_C")) _faction) (Default|CanRecruitNavy (.Value (Utilities|Map|Find _country_map "/Game/Blueprints/Countries/BP_SouthernOcean.BP_SouthernOcean_C")) _faction))))