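; Base sea battle card that lets its race attack enemy units or empty countries in adjacent water.
; Relevant targets come from water bordering the race's occupied countries, supplied or not, though the unit search returns after the first occupied country.
; The card is playable when targets exist; executing it sends a selection command to the server-only controller.
; The selected unit or country feeds the matching AbilityFactory attack ability.
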(event EventOnCountrySelected(Protected)
  (params (Country :type BP%20Country%20Object%20Reference%20%28by%20ref%29))
  (Default|AttackCountry(Ability) (CallFunction|AbilityFactory) self Country true true))

(event EventExecuteCard
  (|CallParentFunction)
  (CallFunction|SelectActor(Command) (CallFunction|Controller(ServerOnly)) (CallFunction|RelevantActorsonPlay)))

(event EventBeginPlay
  (|CallParentFunction))

(event EventOnUnitSelected(Protected)
  (params (Unit :type BP%20Unit%20Object%20Reference%20%28by%20ref%29))
  (Default|AttackUnit(Ability) (CallFunction|AbilityFactory) self Unit true true))

(fn ConstructionScript
  (|CallParentFunction))

(fn RelevantUnitsonPlay
  (for _array_element (Default|GetAllOccupiedCountriesforRace (CallFunction|BPWorld) (CallFunction|CardRace) false)
    (for _array_element_2 (Default|GetAdjacentCountires _array_element)
      (if (and (Default|IsWater _array_element_2) (Default|IsEnemyOwned _array_element_2 (CallFunction|GetTeamforRace (CallFunction|CardRace))))
        (for _array_element_3 (Variables|/Game/Blueprints/Countries/BP_Country.BP_Country_C|GetUnits _array_element_2)
          (Utilities|Array|AddUnique (LocalVariables|GetRelevant%20Units%20Local) _array_element_3))))
    (return (LocalVariables|GetRelevant%20Units%20Local)))
  (return 0))

(fn RelevantCountriesonPlay
  (for _array_element (Default|GetAllOccupiedCountriesforRace (CallFunction|BPWorld) (CallFunction|CardRace) false)
    (for _array_element_2 (Default|GetAdjacentCountires _array_element)
      (if (and (Default|IsCountryEmpty _array_element_2) (Default|IsWater _array_element_2))
        (Utilities|Array|AddUnique (LocalVariables|GetEmpty%20Countries) _array_element_2))))
  (return (LocalVariables|GetEmpty%20Countries)))

(fn Playable
  (return (> (Utilities|Array|Length (CallFunction|RelevantActorsonPlay)) 0)))