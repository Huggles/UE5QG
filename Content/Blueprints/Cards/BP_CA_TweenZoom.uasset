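; BP_CA_TweenZoom is a card action that glides the turn-based pawn, acting as the camera, to a target location.
; It saves the pawn's current location as OriginalPosition, then tweens the actor there with InOutSine easing.
; KeepDistance offsets the destination along Y and Z to hold the view back from the target.
; When the tween completes, it signals that the action has finished.
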(event Custom|Ev%20Tween%20Camera%20To%20Location
  (params (Target%20Location :type Vector) (Keep%20Distance :type Boolean))
  (bind _asbp_turn_based_pawn (Utilities|TBPawn))
  (Variables|/Game/Blueprints/Game/BP_TurnBasedPawn.BP_TurnBasedPawn_C|SetOriginalPosition _asbp_turn_based_pawn (Transformation|GetActorLocation _asbp_turn_based_pawn))
  (bind _value (|TweenVector (Transformation|GetActorLocation _asbp_turn_based_pawn) (Math|Vector|MakeVector (.x Target%20Location) (Math|Float|SelectFloat (+ (.y Target%20Location) 4e+02) (.y Target%20Location) Keep%20Distance) (Math|Float|SelectFloat (+ (.z Target%20Location) 7.5e+02) (.z Target%20Location) Keep%20Distance)) 1.5 "InOutSine")
    (:ApplyEasing
      (Transformation|SetActorLocation _asbp_turn_based_pawn _value false false))
    (:OnComplete
      (Default|CallActionFinished self))))

(event EventExecuteAction
  (CallFunction|EvTweenCameratoLocation (Variables|Default|GetTarget) (Variables|Default|GetKeep%20Distance)))

(fn ConstructionScript)