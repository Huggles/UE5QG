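; Per-race deck manager for a turn-based card game, owned on the server by that race's player controller.
; It spawns attached card actors from the race's initial deck and handles shuffling and drawing into the hand.
; Card plays execute locally predicted, then go to the server through the card execution manager.
; Client RPCs show status and response card lists, and activated effective cards route through the game state, which then requests responses.
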(event Custom|Draw%20Cards%20%28Server%29
  (params (Number :type Integer))
  (if (> (Utilities|Array|Length (Variables|Default|GetDeck)) 0)
    (for _index (range 0 (Math|Integer|Min(Integer) Number (Utilities|Array|Length (Variables|Default|GetDeck))))
      (if (Utilities|IsValid (Utilities|Array|Get(acopy) (Variables|Default|GetDeck) _index))
        (CallFunction|DrawCard (Utilities|Array|Get(acopy) (Variables|Default|GetDeck) _index))))
    (Utilities|Array|Add (Variables|Default|GetDeckHistory) "NewEnumerator0")
    (Variables|Default|SetDeckHistory (Variables|Default|GetDeckHistory))))

(event Custom|Shuffle%20Deck%20%28Server%29
  (Utilities|Array|Shuffle (Variables|Default|GetDeck))
  (Utilities|Array|Add (Variables|Default|GetDeckHistory) "NewEnumerator3"))

(event Custom|Request%20Status%20Card%20%28Client%29
  (Default|ShowCardList (Variables|/Game/Blueprints/Game/BP_TurnBasedPlayerController.BP_TurnBasedPlayerController_C|GetUserInterfaceWidget (CallFunction|GetFirstLocalTBPlayerController)) (Variables|Default|GetPlayable%20Race) "NewEnumerator3" "NewEnumerator2" self))

(event Custom|Cancel%20Request%20Effective%20Card%20%28Client%29
  (Default|HideCardList (Variables|/Game/Blueprints/Game/BP_TurnBasedPlayerController.BP_TurnBasedPlayerController_C|GetUserInterfaceWidget (CallFunction|GetFirstLocalTBPlayerController))))

(event Custom|Request%20Response%20Card%20%28Client%29
  (params (Triggered%20By%20Card :type BP%20Card%20Object%20Reference))
  (Default|ShowCardList (Variables|/Game/Blueprints/Game/BP_TurnBasedPlayerController.BP_TurnBasedPlayerController_C|GetUserInterfaceWidget (CallFunction|GetFirstLocalTBPlayerController)) (Variables|Default|GetPlayable%20Race) "NewEnumerator4" "NewEnumerator1" self))

(event Custom|Init%20Owner
  (bind _tb_game_state (CallFunction|TBGameState))
  (bind _playable_race (Variables|Default|GetPlayable%20Race))
  (bind _tb_player_controller (Default|GetPlayerControllerforRace(Server) _tb_game_state _playable_race))
  (Networking|SwitchHasAuthority
    (:Authority
      (Actor|SetOwner _tb_player_controller)
      (Development|PrintString (Utilities|String|Append "Changed Deck Manager Owner: " (Utilities|String|EnumtoString (Variables|Default|GetPlayable%20Race)) " to " (Default|GetDebugString _tb_player_controller))))))

(event Custom|Play%20Card%20%28Client%29
  (params (Card :type BP%20Card%20Object%20Reference))
  (bind _output_get (Variables|/Game/Blueprints/Cards/CardExecutionManager.CardExecutionManager_C|SetActive%20Card (CallFunction|CardExecutionManager) Card))
  (Default|ExecuteCard(LocalPredicted) _output_get)
  (CallFunction|PlayCard(Server) _output_get))

(event Custom|Draw%20Card
  (params (BP%20Card :type BP%20Card%20Object%20Reference))
  (Utilities|Array|Add (Variables|Default|GetHand) BP%20Card)
  (Default|CallAfterCardDraw BP%20Card self))

(event Custom|Play%20Card%20%28Server%29
  (params (Card :type BP%20Card%20Object%20Reference))
  (Default|PlayCard (CallFunction|CardExecutionManager) Card))

(event Custom|Request%20Effective%20Card%20Usage%20%28Server%29
  (Development|PrintString (Utilities|GetDisplayName (Utilities|OwningTBController))))

(event Custom|Effective%20Card%20Execution%20Finished_1
  (params (Effective%20Card :type BP%20Card%20Object%20Reference))
  (Default|RequestResponseCard(Server) (CallFunction|TBGameState) Effective%20Card))

(event EventBeginPlay)

(event EventActivateEffectiveCard
  (params (BP%20Card :type BP%20Card%20Object%20Reference) (Player%20Controller :type BP%20Turn%20Based%20Player%20Controller%20Object%20Reference))
  (Default|ActivateEffectiveCard(Server) (CallFunction|TBGameState) BP%20Card 0 self))

(event EventDoNotActivateEffectiveCard
  (params (Player%20Controller :type BP%20Turn%20Based%20Player%20Controller%20Object%20Reference) (Player%20State :type BP%20Turn%20Based%20Player%20State%20Object%20Reference))
  (Development|PrintString "Do Not Play Effective Card"))

(fn ConstructionScript)

(fn OnRepDeckHistory)

(fn InstantiateDeck
  (params (TB%20Player%20Controller :type BP%20Turn%20Based%20Player%20Controller%20Object%20Reference) (TB%20Player%20State :type BP%20Turn%20Based%20Player%20State%20Object%20Reference))
  (Variables|META|SetPlayer%20Controller TB%20Player%20Controller)
  (Variables|META|SetPlayer%20State TB%20Player%20State)
  (bind _playable_race (Default|RaceStructforRace (CallFunction|TBGameState) (Variables|Default|GetPlayable%20Race)))
  (for _array_element (.initialdeck _playable_race)
    (bind _returnvalue (Game|SpawnActorfromClass (Variables|/Game/DataAssets/PDA_Card.PDA_Card_C|GetActorClass _array_element) (Math|Transform|MakeTransform "0, 0, 0") "Undefined" "MultiplyWithRoot" 0 (Variables|META|GetPlayer%20Controller) (Variables|META|GetPlayer%20State) _array_element 0))
    (Transformation|AttachActorToActor _returnvalue self "None" "KeepRelative" "KeepRelative" "KeepRelative" false)
    (Utilities|Array|Add (Variables|Default|GetDeck) _returnvalue)))

(fn HasStatusCardEffective
  (return (> (Utilities|Array|Length (Variables|Default|GetStatusCards)) 0)))

(fn HasResponseCardEffective
  (return (> (Utilities|Array|Length (Variables|Default|GetStatusCards)) 0)))

(fn GetCardbyClass
  (params (Card%20Class :type BP%20Card%20Class%20Reference))
  (for _array_element (Variables|Default|GetDeck)
    (if (== (Utilities|GetClass _array_element) Card%20Class)
      (return _array_element)))
  (return 0))