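; Base Blueprint for faction cards in a turn-based game with countries and units, played or activated by an ability trigger.
; Play and activation record the turn, update visibility and batch blocking show-card client commands; only play waits for them before its implementation hook.
; Subclasses override those hooks, playability checks and relevant country/unit queries, using helpers that spawn server-queued selection commands.
; Finishing clears the active card and ends the play step unless ability-triggered.
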(event Custom|Play%20Card
  ;[0 1 0.04137] Card Execution
  (Utilities|Array|Add (Variables|History|GetPlayed%20In%20Turns) (Variables|/Game/Blueprints/Game/BP_TurnBasedGameState.BP_TurnBasedGameState_C|GetTurnCounter (.TB%20Game%20State (CallFunction|TBGameState))))
  (Variables|Default|SetCard%20Effect "NewEnumerator2")
  (Variables|/Game/Blueprints/Game/BP_TurnBasedGameState.BP_TurnBasedGameState_C|SetActive%20Card (.TB%20Game%20State (CallFunction|TBGameState)) self)
  (Variables|Deck|SetIs%20Played true)
  (CallFunction|SetCardPublicVisibility (Play|VisibleAfterPlay))
  (bind _client_command_batch (CommandHelpers|ShowCardPlaytoAllControllers(Command)))
  (EventDispatchers|AssignCommandFinished _client_command_batch (delegate Custom|CommandFinished_Event)))

(event Custom|Command%20Finished
  (params (Finished%20Command :type BP%20Command%20Object%20Reference))
  ;[0 1 0.04137] Card Execution
  ;;[1 1 1] Virtuals
)

(event Custom|Activate%20Card%20Implementation
  (params (Ability%20Trigger :type BP%20Ability%20Object%20Reference))
  ;[0 1 0.04137] Card Execution
  ;;[1 1 1] Virtuals
)

(event Custom|Activate%20Card
  (params (Ability%20Trigger :type BP%20Ability%20Object%20Reference))
  ;[0 1 0.04137] Card Execution
  (Utilities|Array|Add (Variables|History|GetActivated%20In%20Turns) (Variables|/Game/Blueprints/Game/BP_TurnBasedGameState.BP_TurnBasedGameState_C|GetTurnCounter (.TB%20Game%20State (CallFunction|TBGameState))))
  (Variables|Deck|SetIs%20Played true)
  (Variables|Deck|SetIs%20Activated%20As%20Response true)
  (CallFunction|SetCardPublicVisibility true)
  (CommandHelpers|ShowCardPlaytoAllControllers(Command))
  (CallFunction|ActivateCardImplementation Ability%20Trigger))

(event Custom|Card%20Execution%20Finished
  ;[0 1 0.04137] Card Execution
  (Variables|/Game/Blueprints/Game/BP_TurnBasedGameState.BP_TurnBasedGameState_C|SetActive%20Card (.TB%20Game%20State (CallFunction|TBGameState)) 0)
  (if (not (Getters|TriggeredbyAbility))
    (Default|CallPlayStepFinished (CallFunction|GameEventManager))))

(event Custom|Play%20Card%20Implementation
  ;[0 1 0.04137] Card Execution
  ;;[1 1 1] Virtuals
)

(event Custom|CommandFinished_Event
  (params (Command :type BP%20Command%20Object%20Reference) (Result :type Command%20Result%20Structure))
  ;[0 1 0.04137] Card Execution
  (CallFunction|PlayCardImplementation))

(event Custom|Ability%20Finished
  (params (Ability :type BP%20Ability%20Object%20Reference))
  ;[0 1 0.04137] Card Execution
  ;;[1 1 1] Virtuals
  (Utilities|FlowControl|Delay 1.0)
  (CallFunction|CardExecutionFinished))

(fn ConstructionScript
  (|CallParentFunction))

(fn DebugCardPlay
  (Development|PrintString (Utilities|String|Append "Card Owner:" (Variables|/Game/Blueprints/Game/BP_TurnBasedPlayerState.BP_TurnBasedPlayerState_C|GetPlayer%20Name (Variables|Default|GetPlayer%20State)) "" (Utilities|GetDisplayName self)) true true "(R=0.974547,G=0.529491,B=1.000000,A=1.000000)" 5.0))

(fn IsCardPlayed
  (return (Default|IsCardPlayed (Getters|CardDeckManager) self)))

(fn CardTeam
  (return (.team (Default|GetRaceStructStructforRace (.TB%20Game%20State (CallFunction|TBGameState)) (CardProperties|CardFaction)))))

(fn CardDeckManager
  (return (CallFunction|GetDeckManager (CardProperties|CardFaction))))

(fn Playable
  (return false))

(fn RelevantActorsonPlay
  (params (Faction :type FactionEnum%20Enum :default "NewEnumerator0"))
  (bind _bp_world (CallFunction|BPWorld))
  (bind _adjacent_countries_for_card_faction_local (LocalVariables|GetAdjacent%20Countries%20For%20Card%20Faction%20Local))
  (bind (_placed_units _occupied_countries) (Default|GetAllPlacedUnits&OccupiedCountriesforFaction _bp_world Faction))
  (Utilities|FlowControl|Sequence
    (:then_0
      (LocalVariables|SetPlaced%20Units _placed_units)
      (bind _output_get (LocalVariables|SetOccupied%20Countries%20For%20Card%20Faction%20Local _occupied_countries))
      (for _array_element _output_get
        (for _array_element_2 (Variables|/Game/Blueprints/Countries/BP_Country.BP_Country_C|GetAdjacent%20Countries _array_element)
          (Utilities|Array|AppendArray (LocalVariables|GetAdjacent%20Countries%20For%20Card%20Faction%20Local) (.adjacentcountries _array_element_2)))))
    (:then_1
      (bind _output_get_2 (LocalVariables|SetRel%20Actors (Utilities|Array|MakeArray 0)))
      (Utilities|Array|Clear _output_get_2)
      (Utilities|FlowControl|Sequence
        (:then_0
          (bind _output_get_3 (LocalVariables|SetRelevant%20Countries%20On%20Play%20Local (Play|RelevantCountriesonPlay (LocalVariables|GetOccupied%20Countries%20For%20Card%20Faction%20Local) _adjacent_countries_for_card_faction_local (LocalVariables|GetPlaced%20Units))))
          (Utilities|Array|AppendArray (LocalVariables|GetRel%20Actors) _output_get_3))
        (:then_1
          (LocalVariables|SetRelevant%20Units%20On%20Play%20Local (Play|RelevantUnitsonPlay (LocalVariables|GetOccupied%20Countries%20For%20Card%20Faction%20Local) _adjacent_countries_for_card_faction_local (LocalVariables|GetPlaced%20Units)))
          (Utilities|Array|AppendArray (LocalVariables|GetRel%20Actors) (Play|RelevantUnitsonPlay (LocalVariables|GetOccupied%20Countries%20For%20Card%20Faction%20Local) _adjacent_countries_for_card_faction_local (LocalVariables|GetPlaced%20Units))))
        (:then_2
          (return (LocalVariables|GetRel%20Actors) (LocalVariables|GetRelevant%20Countries%20On%20Play%20Local) (LocalVariables|GetRelevant%20Units%20On%20Play%20Local) (Utilities|Array|Length (LocalVariables|GetRel%20Actors)) (Utilities|Array|Length (LocalVariables|GetRelevant%20Countries%20On%20Play%20Local)) (Utilities|Array|Length (LocalVariables|GetRelevant%20Units%20On%20Play%20Local))))))))

(fn RelevantUnitsonPlay
  (params (Occupied%20Countries :type Array%20of%20BP%20Country%20Object%20References) (Adjacent%20Countries :type Array%20of%20BP%20Country%20Object%20References) (Placed%20Units :type Array%20of%20BP%20Unit%20Object%20References))
  (return 0))

(fn TriggeredbyAbility
  (return (Utilities|IsValid (Variables|Default|GetAbility%20Trigger))))

(fn SelectActor(Command)
  (params (Target%20Controller :type BP%20Turn%20Based%20Player%20Controller%20Object%20Reference) (Actors :type Array%20of%20Actor%20Object%20References) (Skippable :type Boolean))
  (bind _returnvalue (Game|SpawnActorfromClass "/Game/Blueprints/Commands/ClientCommands/SelectActorClientCommand.SelectActorClientCommand_C" (Variables|Default|GetSpawn%20Transform) "Undefined" "MultiplyWithRoot" Target%20Controller Actors 1 Skippable true 0))
  (Default|AddCommand (CallFunction|ServerCommandManager) _returnvalue)
  (return _returnvalue))

(fn ShowCardPlaytoAllControllers(Command)
  (for _array_element (CallFunction|GetAllTBPlayerControllers)
    (bind _returnvalue (Game|SpawnActorfromClass "/Game/Blueprints/Commands/ClientCommands/ShowCardPlayClientCommand.ShowCardPlayClientCommand_C" (Variables|Default|GetSpawn%20Transform) "Undefined" "MultiplyWithRoot" _array_element 1.0 self false true 0))
    (Utilities|Array|AddUnique (LocalVariables|GetCommands%20Local) _returnvalue))
  (bind _client_command_batch (Default|MakeBatchforCommands (CallFunction|ServerCommandManager) (LocalVariables|GetCommands%20Local) true true))
  (return _client_command_batch))

(fn Controller(ServerOnly)
  (return (CallFunction|GetControllerforRace(ServerOnly) (CardProperties|CardFaction))))

(fn RelevantCountriesonPlay
  (params (Occupied%20Countries :type Array%20of%20BP%20Country%20Object%20References) (Adjacent%20Countries :type Array%20of%20BP%20Country%20Object%20References) (Placed%20Units :type Array%20of%20BP%20Unit%20Object%20References))
  (return 0))

(fn VisibleAfterPlay
  (return true))

(fn AddasStatusCard
  (Utilities|Array|Add (Variables|/Game/Blueprints/Cards/BP_PlayerDeckManager.BP_PlayerDeckManager_C|GetStatusCards (CallFunction|GetDeckManager (CardProperties|CardFaction))) self))

(fn AddasResponseCard
  (Utilities|Array|Add (Variables|/Game/Blueprints/Cards/BP_PlayerDeckManager.BP_PlayerDeckManager_C|GetResponseCards (CallFunction|GetDeckManager (CardProperties|CardFaction))) self))

(fn IsPlayedThisTurn
  (return (Utilities|Array|ContainsItem (Variables|History|GetPlayed%20In%20Turns) (Variables|/Game/Blueprints/Game/BP_TurnBasedGameState.BP_TurnBasedGameState_C|GetTurnCounter (.TB%20Game%20State (CallFunction|TBGameState))))))

(fn IsActivatedThisTurn
  (return (Utilities|Array|ContainsItem (Variables|History|GetActivated%20In%20Turns) (Variables|/Game/Blueprints/Game/BP_TurnBasedGameState.BP_TurnBasedGameState_C|GetTurnCounter (.TB%20Game%20State (CallFunction|TBGameState))))))

(fn HasCardText
  (return (and (not (Utilities|Array|ContainsItem (Utilities|Array|MakeArray (Utilities|Enum|LiteralenumCardTypeEnum "NewEnumerator0") (Utilities|Enum|LiteralenumCardTypeEnum "NewEnumerator6") (Utilities|Enum|LiteralenumCardTypeEnum "NewEnumerator1") (Utilities|Enum|LiteralenumCardTypeEnum "NewEnumerator7")) (CardProperties|CardType))) (not (Utilities|Text|TextIsEmpty (CardProperties|CardText))))))

(fn CardName
  (return (.name (Variables|Default|GetCard%20Struct%20Data))))

(fn CardText
  (return (.text (Variables|Default|GetCard%20Struct%20Data))))

(fn CardType
  (return (.type (Variables|Default|GetCard%20Struct%20Data))))

(fn CardFaction
  (return (.faction (Variables|Default|GetCard%20Struct%20Data))))

(fn SetCardPublicVisibility
  (params (Is%20Publicly%20Visible :type Boolean))
  (bind _output_get (Variables|Deck|SetIs%20Publicly%20Visible Is%20Publicly%20Visible))
  (Default|CardChangedVisibility (.TB%20Game%20State (CallFunction|TBGameState)) self _output_get))

(fn SelectCardData(Command)
  (params (Race :type FactionEnum%20Enum :default "NewEnumerator0") (Card%20Data%20Structs :type Array%20of%20Card%20Struct%20Structures) (Title :type String) (Accept%20Button%20Label :type String) (Decline%20Button%20Label :type String) (Show%20Decline%20Button :type Boolean) (Skippable :type Boolean))
  (bind _returnvalue (Game|SpawnActorfromClass "/Game/Blueprints/Commands/ClientCommands/SelectCardReferenceClientCommand.SelectCardReferenceClientCommand_C" (Variables|Default|GetSpawn%20Transform) "Undefined" "MultiplyWithRoot" (CallFunction|GetControllerforRace(ServerOnly) Race) Card%20Data%20Structs Title Accept%20Button%20Label Decline%20Button%20Label Show%20Decline%20Button Skippable true 0))
  (Default|AddCommand (CallFunction|ServerCommandManager) _returnvalue)
  (return _returnvalue))

(fn Activatable
  (params (Ability :type BP%20Ability%20Object%20Reference))
  (return false))

(fn ActivatableonActiveAbility
  (return (Activation|Activatable self (Variables|/Game/Blueprints/Game/BP_TurnBasedGameState.BP_TurnBasedGameState_C|GetActive%20Ability (.TB%20Game%20State (CallFunction|TBGameState))))))

(fn ActivatableonPlayStep
  (return false))

(fn RelevantActorsonActivation
  (params (Trigger%20Ability :type BP%20Ability%20Object%20Reference))
  (return (Play|RelevantCountriesonPlay)))

(fn VisibleAfterActivation
  (return true))