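; Japanese response card "Mobile Force" that counters a triggering ability by targeting the card it came from for a forced discard.
; It can respond only when the triggering card is of one specific card type and its own faction check passes, and it always reports as playable.
; On activation it discards itself through its faction's deck manager, then creates and stores a forced-discard ability from the ability factory.
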(event EventBeginPlay
  (|CallParentFunction))

(event EventActivateCardResponseEffect(Protected)
  (params (Ability%20Trigger :type BP%20Ability%20Object%20Reference))
  (Default|DiscardCard (CallFunction|GetDeckManager (CallFunction|CardFaction)) self)
  (bind _force_discard_ability (Default|ForceCardDiscard(Ability) (CallFunction|AbilityFactory) self (Variables|/Game/Blueprints/Abilities/BP_Ability.BP_Ability_C|GetOrigin%20Card Ability%20Trigger) true true))
  (Variables|Default|SetDiscardAbility _force_discard_ability))

(fn ConstructionScript
  (|CallParentFunction))

(fn Playable
  (return true))

(fn CanbeActivatedasResponse
  (params (Ability :type BP%20Ability%20Object%20Reference))
  (return (and (Utilities|Enum|Equal(Enum) (Default|CardType (Variables|/Game/Blueprints/Abilities/BP_Ability.BP_Ability_C|GetOrigin%20Card Ability)) "NewEnumerator3") (Utilities|Enum|Equal(Enum) (CallFunction|CardFaction) "NewEnumerator0"))))