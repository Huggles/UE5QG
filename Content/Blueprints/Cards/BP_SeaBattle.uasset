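; BP_SeaBattle is a turn-based card that attacks an enemy unit in an adjacent sea zone.
; Execution, predicted or not, makes units in enemy-owned water next to the card race's countries clickable; it is playable only if any exist.
; Selection spawns BP_GA_AttackUnit with the card as callback, and completion advances the turn.
; RelevantUnits returns inside its outer loop, so only the first occupied country's neighbours are checked.
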(event EventExecuteCard(LocalPredicted)
  (Default|ChangeUIState (Variables|Default|GetPlayer%20Controller) "NewEnumerator6")
  (Variables|/Game/Blueprints/Game/BP_TurnBasedPlayerState.BP_TurnBasedPlayerState_C|SetClickableActors (Variables|Default|GetPlayer%20State) (CallFunction|RelevantUnits)))

(event EventAbilityExecutionFinished
  (params (Gameplay%20Ability :type BP%20Gameplay%20Ability%20Object%20Reference))
  (Default|EvNextPlayerTurn(Server) (CallFunction|TBGameState)))

(event EventBeginPlay
  (|CallParentFunction))

(event EventOnUnitSelected
  (params (Unit :type BP%20Unit%20Object%20Reference) (By%20Controller :type BP%20Turn%20Based%20Player%20Controller%20Object%20Reference))
  (if (== By%20Controller (Variables|Default|GetPlayer%20Controller))
    (CallFunction|HandleonUnitSelected Unit)
    (Game|SpawnActorfromClass "/Game/GameplayAbilities/BP_GA_AttackUnit.BP_GA_AttackUnit_C" (Variables|Default|GetSpawn%20Transform) "Undefined" "MultiplyWithRoot" 0 (CallFunction|FirstSelectedUnit) self 0)))

(event EventExecuteCard
  (Default|ChangeUIState (Variables|Default|GetPlayer%20Controller) "NewEnumerator6")
  (Variables|/Game/Blueprints/Game/BP_TurnBasedPlayerState.BP_TurnBasedPlayerState_C|SetClickableActors (Variables|Default|GetPlayer%20State) (CallFunction|RelevantUnits)))

(fn ConstructionScript
  (|CallParentFunction))

(fn RelevantUnits
  (bind _country (Default|GetAllOccupiedCountriesforRace (CallFunction|TBGameState) (CallFunction|CardRace) false))
  (for _array_element _country
    (bind _adjacent_countries (Default|GetAdjacentCountires _array_element))
    (for _array_element_2 _adjacent_countries
      (if (and (Default|IsWater _array_element_2) (Default|IsEnemyOwned _array_element_2 (CallFunction|GetTeamforRace (CallFunction|CardRace))))
        (for _array_element_3 (Default|GetUnitsinCountry _array_element_2)
          (Utilities|Array|AddUnique (LocalVariables|GetRelevant%20Units%20Local) _array_element_3))))
    (return (LocalVariables|GetRelevant%20Units%20Local)))
  (return 0))

(fn Playable
  (return (> (Utilities|Array|Length (CallFunction|RelevantUnits)) 0)))