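; German event card Sturmfuhrer, which eliminates a unit in an enemy-owned Western Europe.
; It is playable only when that country holds exactly one unit and is enemy-owned relative to the card race's team.
; Executing the card offers that unit through a select-actor command.
; When the controlling player selects it, the card spawns BP_Ability_EliminateUnit on the first selected unit.
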(event EventExecuteCard
  (CallFunction|SelectActor(Command) (CallFunction|RelevantUnitsonPlay)))

(event EventBeginPlay
  (|CallParentFunction))

(event EventOnUnitSelected
  (params (Unit :type BP%20Unit%20Object%20Reference) (By%20Controller :type BP%20Turn%20Based%20Player%20Controller%20Object%20Reference))
  (if (== By%20Controller (CallFunction|Controller(ServerOnly)))
    (CallFunction|HandleonUnitSelected Unit)
    (Game|SpawnActorfromClass "/Game/Blueprints/Commands/Abilities/BP_Ability_EliminateUnit.BP_Ability_EliminateUnit_C" (Variables|Default|GetSpawn%20Transform) "Undefined" "MultiplyWithRoot" 0 (CallFunction|FirstSelectedUnit) 0 true true 0)))

(fn ConstructionScript
  (|CallParentFunction))

(fn Playable
  (return (== (Utilities|Array|Length (CallFunction|RelevantUnitsonPlay)) 1)))

(fn RelevantUnitsonPlay
  (bind _bp_world (CallFunction|BPWorld))
  (bind _countrymap (Variables|/Game/Blueprints/Countries/BP_World.BP_World_C|GetCountryMap _bp_world))
  (bind _value (Utilities|Map|Find _countrymap "/Game/Blueprints/Countries/BP_WesternEurope.BP_WesternEurope_C"))
  (if (Default|IsEnemyOwned _value (CallFunction|GetTeamforRace (Variables|Default|GetRace)))
    (return (Default|GetUnitsinCountry _value))))