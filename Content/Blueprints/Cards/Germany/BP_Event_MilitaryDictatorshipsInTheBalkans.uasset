(event EventOnUnitSelected(Protected)
  (params (Unit :type BP%20Unit%20Object%20Reference%20%28by%20ref%29))
  (bind _eliminate_unit_ability (Default|EliminateUnit(Ability) (CallFunction|AbilityFactory) self Unit true true))
  (Variables|Default|SetEliminate%20Unit%20Ability _eliminate_unit_ability))

(event EventBeginPlay
  (|CallParentFunction))

(event EventAbilityFinished
  (params (Ability :type BP%20Ability%20Object%20Reference))
  (bind _relevantunits (CallFunction|RelevantUnitsonPlay))
  (bind _returnvalue (Utilities|Array|Length _relevantunits))
  (if (== Ability (Variables|Default|GetBuild%20Unit%20Ability))
    (if (> _returnvalue 0)
      (if (== _returnvalue 1)
        (CallFunction|OnUnitSelected(Protected) (Utilities|Array|Get(acopy) _relevantunits))
        (else
          (CallFunction|SelectActor(Command) (CallFunction|Controller(ServerOnly)) _relevantunits false)))
      (else
        (CallFunction|CardExecutionFinished :!label _label)))
    (elif (== Ability (Variables|Default|GetEliminate%20Unit%20Ability))
      (goto _label))))

(event EventPlayCardImplementation
  (bind _build_unit_ability (Default|BuildUnit(Ability) (CallFunction|AbilityFactory) self (.Value (Utilities|Map|Find (Variables|/Game/Blueprints/Countries/BP_World.BP_World_C|GetCountryMap (CallFunction|BPWorld)) "/Game/Blueprints/Countries/BP_Balkans.BP_Balkans_C")) "NewEnumerator1" "NewEnumerator0" true true true))
  (Variables|Default|SetBuild%20Unit%20Ability _build_unit_ability))

(fn ConstructionScript
  (|CallParentFunction))

(fn Playable
  (bind _bp_world (CallFunction|BPWorld))
  (bind _countrymap (Variables|/Game/Blueprints/Countries/BP_World.BP_World_C|GetCountryMap _bp_world))
  (bind _value (Utilities|Map|Find _countrymap "/Game/Blueprints/Countries/BP_Balkans.BP_Balkans_C"))
  (return (or (Default|IsTeamOwned _value (CallFunction|GetTeamforRace (CallFunction|CardFaction))) (Default|IsCountryEmpty _value))))

(fn RelevantUnitsonPlay
  (params (Occupied%20Countries :type Array%20of%20BP%20Country%20Object%20References) (Adjacent%20Countries :type Array%20of%20BP%20Country%20Object%20References) (Placed%20Units :type Array%20of%20BP%20Unit%20Object%20References))
  (return (Variables|/Game/Blueprints/Countries/BP_Country.BP_Country_C|GetUnits (.Value (Utilities|Map|Find (Variables|/Game/Blueprints/Countries/BP_World.BP_World_C|GetCountryMap (CallFunction|BPWorld)) "/Game/Blueprints/Countries/BP_Ukraine.BP_Ukraine_C")))))