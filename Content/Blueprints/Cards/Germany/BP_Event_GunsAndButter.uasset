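; Germany's Guns and Butter event card, which lets the player pick and play one basic Build Army, Build Navy, Land Battle or Sea Battle card.
; It loads the faction's rows from the card data table, spawns each card and attaches those that are playable.
; A skippable selection command offers all loaded cards, not just the filtered playable list.
; The chosen card joins the faction's deck and is played through the deck manager.
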(event Custom|CommandFinished_Event_0
  (params (Command :type BP%20Command%20Object%20Reference) (Result :type Command%20Result%20Structure))
  (bind _faction (CallFunction|CardFaction))
  (bind _deck_manager (CallFunction|GetDeckManager _faction))
  (if (not (.skipped Result))
    (Variables|Default|SetSelected%20Card (.Value (Utilities|Map|Find (Variables|Default|GetCards%20Map) (.type (Utilities|Array|Get(acopy) (.referencecards Result))))))
    (Utilities|Array|Add (Variables|/Game/Blueprints/Cards/BP_PlayerDeckManager.BP_PlayerDeckManager_C|GetDeck _deck_manager) (Variables|Default|GetSelected%20Card))
    (Default|PlayCard(Server) _deck_manager (Variables|Default|GetSelected%20Card))
    (bind _values (Utilities|Map|Values (Variables|Default|GetCards%20Map)))
    (for _array_element _values
      (if (!= _array_element (Variables|Default|GetSelected%20Card))
        (Actor|DestroyActor)))))

(event EventPlayCardImplementation
  (Utilities|FlowControl|Sequence
    (:then_0
      (for _array_element (Utilities|Array|MakeArray "BuildArmy" "BuildNavy" "LandBattle" "SeaBattle")
        (bind _returnvalue (Utilities|GetDataTableRow "/Game/DataAssets/CardsDataTable.CardsDataTable" (Utilities|String|StringToName (Utilities|String|Append "BP_" (Utilities|String|EnumtoString (CallFunction|CardFaction)) _array_element)))
          (:then
            (Utilities|Array|Add (Variables|Default|GetCard%20Structs) _returnvalue)))))
    (:then_1
      (Utilities|FlowControl|Sequence
        (:then_0
          (for _array_element_2 (Variables|Default|GetCard%20Structs)
            (bind _returnvalue_2 (Game|SpawnActorfromClass (.Actor (Utilities|Struct|BreakCardStruct _array_element_2)) (Variables|Default|GetSpawn%20Transform) "Undefined" "MultiplyWithRoot" 0 (Variables|Default|GetPlayer%20Controller) (Variables|Default|GetPlayer%20State) 0 _array_element_2 0))
            (Utilities|Map|Add (Variables|Default|GetCards%20Map) (.Type (Utilities|Struct|BreakCardStruct _array_element_2)) _returnvalue_2)
            (if (CallFunction|Playable _returnvalue_2)
              (Utilities|Array|Add (Variables|Default|GetPlayable%20Card%20Structs) _array_element_2)
              (Transformation|AttachActorToActor _returnvalue_2 self "None" "KeepRelative" "KeepRelative" "KeepRelative" false)
              (else
                (Actor|DestroyActor)))))
        (:then_1
          (bind _select_card_data_command (Default|SelectCardData(Command) (CallFunction|AbilityFactory) (CallFunction|CardFaction) (Variables|Default|GetCard%20Structs) "Select A Card" "Select" "" false true))
          (EventDispatchers|AssignCommandFinished _select_card_data_command (delegate Custom|CommandFinished_Event_0)))))))

(fn ConstructionScript
  (|CallParentFunction))

(fn Playable
  (return true))