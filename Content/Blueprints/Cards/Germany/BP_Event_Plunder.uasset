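; Germany event card "Plunder" that awards the card's race one point for each relevant unit on the board when played.
; Relevant units are a fixed faction's placed units outside the Germany country, gathered uniquely from the world, with each unit's country printed along the way.
; It is playable only while the Balkans are empty or owned by the card's team.
; After scoring through the game state, it waits briefly before finishing execution.
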(event EventBeginPlay
  (|CallParentFunction))

(event EventPlayCardImplementation
  (Default|AddScoretoRace (.TB%20Game%20State (CallFunction|TBGameState)) (CallFunction|CardRace) (Utilities|Array|Length (CallFunction|RelevantUnitsonPlay)) (CallFunction|CardName))
  (Utilities|FlowControl|Delay 2.0)
  (CallFunction|CardExecutionFinished))

(fn ConstructionScript
  (|CallParentFunction))

(fn Playable
  (bind _bp_world (CallFunction|BPWorld))
  (bind _countrymap (Variables|/Game/Blueprints/Countries/BP_World.BP_World_C|GetCountryMap _bp_world))
  (bind _value (Utilities|Map|Find _countrymap "/Game/Blueprints/Countries/BP_Balkans.BP_Balkans_C"))
  (return (or (Default|IsTeamOwned _value (CallFunction|GetTeamforRace (CallFunction|CardRace))) (Default|IsCountryEmpty _value))))

(fn RelevantUnitsonPlay
  (params (Occupied%20Countries :type Array%20of%20BP%20Country%20Object%20References) (Adjacent%20Countries :type Array%20of%20BP%20Country%20Object%20References) (Placed%20Units :type Array%20of%20BP%20Unit%20Object%20References))
  (for _array_element (.Placed%20Units (Default|GetAllPlacedUnits&OccupiedCountriesforFaction (CallFunction|BPWorld) "NewEnumerator0"))
    (Development|PrintString (Utilities|GetDisplayName (Variables|/Game/Blueprints/Units/BP_Unit.BP_Unit_C|GetCountry _array_element)))
    (if (not (== (Utilities|GetClass (Variables|/Game/Blueprints/Units/BP_Unit.BP_Unit_C|GetCountry _array_element)) "/Game/Blueprints/Countries/BP_Germany.BP_Germany_C"))
      (Utilities|Array|AddUnique (LocalVariables|GetRelevant%20Units) _array_element)))
  (return (LocalVariables|GetRelevant%20Units)))