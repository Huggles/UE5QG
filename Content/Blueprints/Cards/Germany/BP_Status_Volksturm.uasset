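; Volksturm is a German status card that, when activated, deploys a unit of the card's faction to Western Europe.
; Playing it registers the card in the faction deck manager's status cards, and activation sets the turn state before calling the ability factory.
; Activation checks gather buildable land countries, with the ability check also requiring that the first holds no faction unit.
; Playable always returns false.
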(event Custom|Activate%20Card%20Status%20Effect%20%28Protected%29_1
  (params (Ability%20Trigger :type BP%20Ability%20Object%20Reference))
  (Variables|/Game/Blueprints/Game/BP_TurnBasedPlayerState.BP_TurnBasedPlayerState_C|SetTurn%20State (Variables|Default|GetPlayer%20State) "NewEnumerator0")
  (Default|DeployUnit(Ability) (CallFunction|AbilityFactory) 0 (.Value (Utilities|Map|Find (Default|GetCountryMap (CallFunction|BPWorld)) "/Game/Blueprints/Countries/BP_WesternEurope.BP_WesternEurope_C")) (CallFunction|CardFaction) "NewEnumerator0" "NewEnumerator0" true true true))

(event EventAbilityFinished
  (params (Ability :type BP%20Ability%20Object%20Reference)))

(event EventPlayCard
  (Utilities|Array|Add (Variables|/Game/Blueprints/Cards/BP_PlayerDeckManager.BP_PlayerDeckManager_C|GetStatusCards (CallFunction|GetDeckManager (CallFunction|CardFaction))) self)
  (Default|CallCardActionsFinished))

(event EventBeginPlay
  (|CallParentFunction))

(fn ConstructionScript
  (|CallParentFunction))

(fn Playable
  (return false))

(fn CanbeActivatedasStatus
  (params (Ability :type BP%20Ability%20Object%20Reference))
  (bind _relevantcountries (CallFunction|RelevantActorsonActivation Ability))
  (return (or false (and (> (Utilities|Array|Length _relevantcountries) 0) (not (.Player%20Has%20Unit (Default|HasPlayerUnit (Utilities|Array|Get(acopy) _relevantcountries) (CallFunction|CardFaction))))))))

(fn RelevantActorsonActivation
  (params (Trigger%20Ability :type BP%20Ability%20Object%20Reference))
  (for _array_element 0
    (if (and (Default|IsLand _array_element) (Default|CanRaceBuild _array_element (CallFunction|CardFaction)))
      (Utilities|Array|AddUnique (Variables|Default|GetRelevantCountriesLocal) _array_element)))
  (return (Variables|Default|GetRelevantCountriesLocal)))

(fn CanStatusbeActivatedonPlayStep
  (return (> (Utilities|Array|Length (CallFunction|RelevantActorsonActivation)) 0)))