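; Germany's Broad Front event card, which attacks three different enemy units in land countries next to German-occupied ones.
; On execution it snapshots units in adjacent enemy countries holding one specific race's units, then loops selection and attack ability, excluding prior targets until three are done.
; It also overrides status activation, checking for buildable land connected to the triggering card's selected countries, with only the first candidate tested for lacking an own unit.
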(event Custom|Select%20Next%20Country
  (CallFunction|SelectActor(Command) (CallFunction|TargetableCountries)))

(event EventOnUnitSelected(Protected)
  (params (Unit :type BP%20Unit%20Object%20Reference%20%28by%20ref%29))
  (Utilities|Array|AddUnique (Variables|Default|GetTargeted%20Units) Unit)
  (bind _attack_unit_ability (Default|AttackUnit(Ability) (CallFunction|AbilityFactory) self Unit true true))
  (Variables|Default|SetAttack%20Unit%20Ability _attack_unit_ability))

(event EventBeginPlay
  (|CallParentFunction))

(event EventAbilityFinished
  (params (Ability :type BP%20Ability%20Object%20Reference))
  (if (and (== Ability (Variables|Default|GetAttack%20Unit%20Ability)) (== (Utilities|Array|Length (Variables|Default|GetTargeted%20Units)) 3))
    (CallFunction|CardExecutionFinished)
    (else
      (CallFunction|SelectNextCountry))))

(event EventExecuteCard(Protected)
  (Variables|Default|SetInitial%20Targetable%20Units (CallFunction|RelevantUnitsonPlay))
  (CallFunction|SelectNextCountry))

(fn ConstructionScript
  (|CallParentFunction))

(fn Playable
  (return (> (Utilities|Array|Length (CallFunction|RelevantCountriesonPlay)) 0)))

(fn CanbeActivatedasStatus
  (params (Ability :type BP%20Ability%20Object%20Reference))
  (bind _relevantcountries (CallFunction|RelevantCountriesonStatus Ability))
  (return (or (|CallParentFunction Ability) (and (> (Utilities|Array|Length _relevantcountries) 0) (not (.Player%20Has%20Unit (Default|HasPlayerUnit (Utilities|Array|Get(acopy) _relevantcountries) (CallFunction|CardRace))))))))

(fn RelevantCountriesonStatus
  (params (Trigger%20Ability :type BP%20Ability%20Object%20Reference))
  (for _array_element (Variables|/Game/Blueprints/Cards/BP_Card.BP_Card_C|GetSelected%20Countries (Variables|/Game/Blueprints/Abilities/BP_Ability.BP_Ability_C|GetOrigin%20Card Trigger%20Ability))
    (for _array_element_2 (Variables|/Game/Blueprints/Countries/BP_Country.BP_Country_C|GetConnectedCountries _array_element)
      (if (and (Default|IsLand _array_element_2) (Default|CanRaceBuild _array_element_2 (CallFunction|CardRace)))
        (Utilities|Array|AddUnique (LocalVariables|GetRelevantCountriesLocal) _array_element_2))))
  (return (LocalVariables|GetRelevantCountriesLocal)))

(fn CanStatusbeActivatedonPlayStep
  (return true))

(fn TargetableCountries
  (for _array_element (Variables|Default|GetInitial%20Targetable%20Units)
    (if (not (Utilities|Array|ContainsItem (Variables|Default|GetTargeted%20Units) _array_element))
      (Utilities|Array|AddUnique (LocalVariables|GetTargetable%20Units%20Local) _array_element)))
  (return (LocalVariables|GetTargetable%20Units%20Local)))

(fn RelevantUnitsonPlay
  (for _array_element (CallFunction|RelevantCountriesonPlay)
    (if (Math|Boolean|ANDBoolean (Default|IsLand _array_element) (Default|IsEnemyOwned _array_element (CallFunction|GetTeamforRace (CallFunction|CardRace))) (.Player%20Has%20Unit (Default|HasPlayerUnit _array_element "NewEnumerator4")))
      (for _array_element_2 (Variables|/Game/Blueprints/Countries/BP_Country.BP_Country_C|GetUnits _array_element)
        (Utilities|Array|AddUnique (LocalVariables|GetRelevantUnitsLocal) _array_element_2))))
  (return (LocalVariables|GetRelevantUnitsLocal)))

(fn RelevantCountriesonPlay
  (for _array_element (Default|GetAllOccupiedCountriesforRace (CallFunction|BPWorld) (CallFunction|CardRace) false)
    (for _array_element_2 (Default|GetAdjacentCountires _array_element)
      (Utilities|Array|AddUnique (LocalVariables|GetRelevant%20Countries%20Local) _array_element_2)))
  (return (LocalVariables|GetRelevant%20Countries%20Local)))