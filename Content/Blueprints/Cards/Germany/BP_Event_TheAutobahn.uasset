(event Custom|Select%20Country
  (CallFunction|SelectActor(Command) (CallFunction|Controller(ServerOnly)) (CallFunction|RelevantCountriesonPlay) false))

(event Custom|Select%20Next%20Unit
  (CallFunction|SelectActor(Command) (CallFunction|Controller(ServerOnly)) (CallFunction|TargetableUnits) false))

(event EventOnUnitSelected(Protected)
  (params (Unit :type BP%20Unit%20Object%20Reference%20%28by%20ref%29))
  (Utilities|Array|AddUnique (Variables|Default|GetTargeted%20Units) Unit)
  (bind _eliminate_unit_ability (Default|EliminateUnit(Ability) (CallFunction|AbilityFactory) self Unit true true))
  (Variables|Default|SetEliminate%20Unit%20Ability _eliminate_unit_ability))

(event EventBeginPlay
  (|CallParentFunction))

(event EventAbilityFinished
  (params (Ability :type BP%20Ability%20Object%20Reference))
  (if (== Ability (Variables|Default|GetEliminate%20Unit%20Ability))
    (CallFunction|SelectCountry)
    (elif (== Ability (Variables|Default|GetBuild%20Unit%20Ability))
      (if (> (Utilities|Array|Length (CallFunction|TargetableUnits)) 0)
        (CallFunction|SelectNextUnit)
        (else
          (CallFunction|CardExecutionFinished))))))

(event EventOnCountrySelected(Protected)
  (params (Country :type BP%20Country%20Object%20Reference%20%28by%20ref%29))
  (bind _build_unit_ability (Default|BuildUnit(Ability) (CallFunction|AbilityFactory) self Country (CallFunction|CardRace) "NewEnumerator0" true true true))
  (Variables|Default|SetBuild%20Unit%20Ability _build_unit_ability))

(event EventPlayCardImplementation
  (Variables|Default|SetInitial%20Targetable%20Units (CallFunction|RelevantUnitsonPlay))
  (CallFunction|SelectNextUnit))

(fn ConstructionScript
  (|CallParentFunction))

(fn Playable
  (return (> (Utilities|Array|Length (CallFunction|RelevantCountriesonPlay)) 0)))

(fn TargetableUnits
  (for _array_element (Variables|Default|GetInitial%20Targetable%20Units)
    (if (not (Utilities|Array|ContainsItem (Variables|Default|GetTargeted%20Units) _array_element))
      (Utilities|Array|AddUnique (LocalVariables|GetTargetable%20Units%20Local) _array_element)))
  (return (LocalVariables|GetTargetable%20Units%20Local)))

(fn RelevantUnitsonPlay
  (params (Occupied%20Countries :type Array%20of%20BP%20Country%20Object%20References) (Adjacent%20Countries :type Array%20of%20BP%20Country%20Object%20References) (Placed%20Units :type Array%20of%20BP%20Unit%20Object%20References))
  (return Placed%20Units))

(fn RelevantCountriesonPlay
  (params (Occupied%20Countries :type Array%20of%20BP%20Country%20Object%20References) (Adjacent%20Countries :type Array%20of%20BP%20Country%20Object%20References) (Placed%20Units :type Array%20of%20BP%20Unit%20Object%20References))
  (bind _race (CallFunction|CardRace))
  (for _array_element Occupied%20Countries
    (for _array_element_2 (Default|GetAdjacentCountires _array_element)
      (if (Math|Boolean|ANDBoolean (Default|IsLand _array_element_2) (or (Default|IsCountryEmpty _array_element_2) (Default|IsTeamOwned _array_element_2 (CallFunction|GetTeamforRace _race))) (not (.Player%20Has%20Unit (Default|HasPlayerUnit _array_element_2 _race))))
        (Utilities|Array|AddUnique (LocalVariables|GetRelevant%20Countries%20Local) _array_element_2))))
  (return (LocalVariables|GetRelevant%20Countries%20Local)))