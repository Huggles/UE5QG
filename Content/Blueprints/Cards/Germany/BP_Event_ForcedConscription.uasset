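; Germany event card Forced Conscription, which deploys units of the card's faction in up to two different countries adjacent to Germany.
; Eligible targets are land countries that are empty or team-owned and lack a specific player's unit, captured once when played.
; A server-issued select command feeds a deploy ability, whose completion triggers the next pick until two are targeted.
; The first pick is mandatory, and skipping the second ends the card.
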(event Custom|Select%20Next%20Country
  (bind _select_actor_client_command (CallFunction|SelectActor(Command) (CallFunction|Controller(ServerOnly)) (CallFunction|TargetableCountries) (> (Utilities|Array|Length (Variables|Default|GetTargeted%20Countries)) 0)))
  (EventDispatchers|AssignCommandFinished _select_actor_client_command (delegate Custom|CommandFinished_Event_0)))

(event Custom|CommandFinished_Event_0
  (params (Command :type BP%20Command%20Object%20Reference) (Result :type Command%20Result%20Structure))
  (if (.skipped Result)
    (CallFunction|CardExecutionFinished)
    (elif (and (Utilities|IsValid (.country Result)) (Utilities|Array|ContainsItem (CallFunction|TargetableCountries) (.country Result)))
      (Utilities|Array|AddUnique (Variables|Default|GetTargeted%20Countries) (.country Result))
      (bind _build_unit_ability (Default|DeployUnit(Ability) (CallFunction|AbilityFactory) self (.country Result) (CallFunction|CardFaction) "NewEnumerator0" "NewEnumerator0" true true true))
      (Variables|Default|SetBuild%20Unit%20Ability _build_unit_ability))))

(event EventAbilityFinished
  (params (Ability :type BP%20Ability%20Object%20Reference))
  (if (and (== Ability (Variables|Default|GetBuild%20Unit%20Ability)) (== (Utilities|Array|Length (Variables|Default|GetTargeted%20Countries)) 2))
    (CallFunction|CardExecutionFinished)
    (else
      (CallFunction|SelectNextCountry))))

(event EventPlayCardImplementation
  (Variables|Default|SetInitial%20Targetable%20Countries (.Relevant%20Countries (CallFunction|RelevantActorsonPlay (CallFunction|CardFaction))))
  (CallFunction|SelectNextCountry))

(fn ConstructionScript
  (|CallParentFunction))

(fn Playable
  (return (> (.Number%20Of%20Relevant%20Countries (CallFunction|RelevantActorsonPlay (CallFunction|CardFaction))) 0)))

(fn RelevantCountriesonPlay
  (params (Placed%20Units :type Array%20of%20BP%20Unit%20Object%20References) (Occupied%20Countries :type Array%20of%20BP%20Country%20Object%20References) (Adjacent%20Countries :type Array%20of%20BP%20Country%20Object%20References) (Adjacent%20Supplied%20Countries :type Array%20of%20BP%20Country%20Object%20References))
  (for _array_element (Default|GetAdjacentCountriesforFaction (.Value (Utilities|Map|Find (Default|GetCountryMap (CallFunction|BPWorld)) "/Game/Blueprints/Countries/BP_Germany.BP_Germany_C")) (CallFunction|CardFaction))
    (if (Math|Boolean|ANDBoolean (Default|IsLand _array_element) (or (Default|IsCountryEmpty _array_element) (Default|IsTeamOwned _array_element (CallFunction|GetTeamforRace (CallFunction|CardFaction)))) (not (.Player%20Has%20Unit (Default|HasPlayerUnit _array_element "NewEnumerator0"))))
      (Utilities|Array|AddUnique (LocalVariables|GetRelevant%20Countries%20Local) _array_element)))
  (return (LocalVariables|GetRelevant%20Countries%20Local)))

(fn TargetableCountries
  (for _array_element (Variables|Default|GetInitial%20Targetable%20Countries)
    (if (not (Utilities|Array|ContainsItem (Variables|Default|GetTargeted%20Countries) _array_element))
      (Utilities|Array|AddUnique (LocalVariables|GetTargetable%20Countries%20Local1) _array_element)))
  (return (LocalVariables|GetTargetable%20Countries%20Local1)))