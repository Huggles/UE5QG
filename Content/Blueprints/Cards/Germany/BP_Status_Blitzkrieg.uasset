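; Germany's Blitzkrieg status card; executing it adds it to the deck manager's StatusCards for its race and signals that card actions are finished.
; It is never Playable and is Activatable only when the triggering card's first selected country has no units.
; The effect is unfinished: server activation calls the parent and checks Activatable but does nothing more, and the ability-finished callback binding is never run.
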(event Custom|AbilityFinished_Event
  (params (Gameplay%20Ability :type BP%20Gameplay%20Ability%20Object%20Reference))
  (Development|PrintString "Blitzkrieg Finished")
  (Default|EffectiveCardExecutionFinished (Variables|Default|GetCallback) self))

(event EventExecuteCard
  (Utilities|Array|Add (Variables|/Game/Blueprints/Cards/BP_PlayerDeckManager.BP_PlayerDeckManager_C|GetStatusCards (CallFunction|GetDeckManager (CallFunction|CardRace))) self)
  (Default|CallCardActionsFinished))

(event EventBeginPlay
  (|CallParentFunction))

(event EventActivateCardEffect(LocalPredicted))

(event EventActivateCardEffect(Server)
  (params (Callback :type I%20Effective%20Card%20Callback%20Interface))
  (|CallParentFunction Callback)
  (if (CallFunction|Activatable)
    _))

(fn ConstructionScript
  (|CallParentFunction))

(fn Playable
  (return false))

(fn RelevantCountries
  (return (Variables|/Game/Blueprints/Cards/BP_Card.BP_Card_C|GetSelected%20Countries (Variables|Default|GetTriggering%20Card))))

(fn Activatable
  (bind _relevantcountries (CallFunction|RelevantCountries))
  (return (and (> (Utilities|Array|Length _relevantcountries) 0) (Utilities|Array|IsEmpty (Default|GetUnitsinCountry (Utilities|Array|Get(acopy) _relevantcountries))))))