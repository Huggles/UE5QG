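; Card action Blueprint that lets the player pick a country by clicking on it.
; ExecuteAction starts listening for country clicks; the first click stores the selected country, signals that the action is finished and stops listening.
; The set of applicable countries comes unchanged from the parent class.
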(event EventExecuteAction
  (CallFunction|StartListeningtoCountryClicks))

(event EventOnCountryClicked
  (params (Country :type BP%20Country%20Object%20Reference) (Player%20State :type BP%20Turn%20Based%20Player%20State%20Object%20Reference))
  (Variables|Default|SetSelected%20Country Country)
  (Default|CallActionFinished self)
  (CallFunction|StopListeningtoCountryClicks))

(fn ConstructionScript)

(fn GetApplicableCountries
  (return (|CallParentFunction)))