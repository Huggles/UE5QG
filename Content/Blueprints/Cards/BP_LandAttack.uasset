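; BP_LandAttack is a playable card that, despite its name, builds a tank in a country the player selects, then ends the turn.
; Playing it switches the player's turn state and, on the client, registers the card with the country-selection widget.
; The country-selected callback sends build-unit and end-turn server events through the client player controller.
; Construction sets the sprite from the card asset; the spawn and unit-selected handlers are empty.
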(event Custom|Ev%20Set%20UI%20Player%20Card%20%20%28Client%29
  (bind _asbp_turn_based_player_controller (CallFunction|GetPlayerController(Client)))
  (bind _asuib_turn_state_select_country (Utilities|Casting|CastToUIB_TurnState_SelectCountry (Variables|/Game/Blueprints/Game/BP_TurnBasedPlayerController.BP_TurnBasedPlayerController_C|GetUserInterfaceWidget _asbp_turn_based_player_controller)))
  (Variables|/Game/Blueprints/UI/UIB_TurnState_SelectCountry.UIB_TurnState_SelectCountry_C|SetCountrySelectCard _asuib_turn_state_select_country self)
  (Development|PrintString (Utilities|String|Append "Setting Played Card" (Utilities|GetDisplayName _asuib_turn_state_select_country))))

(event Custom|BPI_CountrySelected
  (params (TB%20Player%20State :type BP%20Turn%20Based%20Player%20State%20Object%20Reference) (Selected%20Country :type BP%20Country%20Object%20Reference)))

(event Custom|Ev%20Spawn%20Unit%20%28Server%29
  (params (TB%20Player%20State :type BP%20Turn%20Based%20Player%20State%20Object%20Reference) (Country :type BP%20Country%20Object%20Reference)))

(fn ConstructionScript
  (Rendering|Components|Sprite|SetSprite (Variables|Default|GetPaperSprite_0) (Variables|/Game/DataAssets/PDA_Card.PDA_Card_C|GetSprite (Variables|Default|GetCardAsset_0))))

(fn CountrySelectedCallback
  (params (TB%20Player%20State :type BP%20Turn%20Based%20Player%20State%20Object%20Reference) (Selected%20Country :type BP%20Country%20Object%20Reference))
  (Development|PrintString (Utilities|String|Append "Player Selected Country: " (Variables|/Game/Blueprints/Game/BP_TurnBasedPlayerState.BP_TurnBasedPlayerState_C|GetPlayer%20Name TB%20Player%20State) " | " (Utilities|GetDisplayName Selected%20Country)) true true "(R=0.182413,G=1.000000,B=0.159507,A=1.000000)" 5.0)
  (bind _asbp_turn_based_player_controller (CallFunction|GetPlayerController(Client)))
  (Default|EvBuildUnit(Server) _asbp_turn_based_player_controller (Utilities|Struct|MakeBuildUnitPayload TB%20Player%20State "/Game/Blueprints/Units/BP_Tank.BP_Tank_C" Selected%20Country))
  (Default|EvEndTurn(Server) _asbp_turn_based_player_controller))

(fn PlayCard
  (params (TB%20PlayerState :type BP%20Turn%20Based%20Player%20State%20Object%20Reference))
  (bind _successful (|CallParentFunction TB%20PlayerState))
  (Default|EvSetPlayerTurnState(Client) (Utilities|GetTBPlayerController self) "NewEnumerator2")
  (CallFunction|EvSetUIPlayerCard(Client))
  (return _successful))

(fn UnitSelectedCallback
  (params (TB%20Player%20State :type BP%20Turn%20Based%20Player%20State%20Object%20Reference) (Selected%20Unit :type BP%20Unit%20Object%20Reference)))