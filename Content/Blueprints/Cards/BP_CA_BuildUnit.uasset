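; Card action that builds a unit for a country when executed.
; It spawns the Unit class with country, race, focus and spawn point, then attaches it to the country's available unit position, keeping a raised relative offset and snapping rotation.
; It binds to the new unit's spawned event and relays it through UnitBuilt with that unit.
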(event Custom|Unit%20Spawned_Event
  (Default|CallUnitBuilt (stale Custom|Spawn%20Unit _returnvalue)))

(event Custom|Spawn%20Unit
  (bind _country (Variables|Default|GetCountry))
  (bind _unit_position (Default|GetAvailableUnitPos _country))
  (bind _returnvalue (Game|SpawnActorfromClass (Variables|Default|GetUnit) (Math|Transform|MakeTransform "0.000000,0.000000,500.000000") "Undefined" "MultiplyWithRoot" 0 _country _unit_position (Variables|Default|GetRace) (Variables|Default|GetFocus) 0))
  (Transformation|AttachComponentToComponent _returnvalue _unit_position "None" "KeepRelative" "SnapToTarget" "KeepWorld" false)
  (EventDispatchers|AssignUnitSpawned _returnvalue (delegate Custom|Unit%20Spawned_Event)))

(event EventExecuteAction
  (CallFunction|SpawnUnit))

(fn ConstructionScript)