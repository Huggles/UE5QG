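; Turn-based card game manager that plays cards on the game state and ends the player's turn when their actions finish.
; PlayCard moves the active card from its race's hand to played, status or response piles and executes it.
; Country and unit picks run as spawned selection commands, while build and attack run as spawned ability actors.
; Finished card-triggered abilities request response cards through the game state, and enemy deck managers receive status and response prompts.
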(event Custom|On%20Card%20Finished
  (EventDispatchers|UnbindEventfromCardActionsFinished (stale Custom|Play%20Card _output_get) (delegate Custom|On%20Card%20Finished))
  (Default|EndCurrentPlayerTurn (CallFunction|TBGameState)))

(event Custom|Execute%20Attack%20Unit%20Ability
  (params (Unit :type BP%20Unit%20Object%20Reference) (Callback :type I%20Gameplay%20Ability%20Callback%20Interface) (Origin%20Card :type BP%20Card%20Object%20Reference))
  (bind _returnvalue (Game|SpawnActorfromClass "/Game/Blueprints/Commands/GameplayAbilities/BP_GA_AttackUnit.BP_GA_AttackUnit_C" (Variables|Default|GetSpawn%20Transform) "Undefined" "MultiplyWithRoot" 0 Unit self Origin%20Card 0))
  (Default|ExecuteAbility _returnvalue))

(event Custom|Request%20Country
  (params (Controller :type BP%20Turn%20Based%20Player%20Controller%20Object%20Reference) (Clickable%20Countries :type Array%20of%20BP%20Country%20Object%20References) (Number%20Of%20Countries :type Integer) (Callback :type I%20Command%20Callback%20Interface))
  (bind _returnvalue (Game|SpawnActorfromClass "/Game/Blueprints/Commands/Commands/SelectCountryCommand.SelectCountryCommand_C" (Variables|Default|GetSpawn%20Transform) "Undefined" "MultiplyWithRoot" Controller Clickable%20Countries Number%20Of%20Countries 0 Callback true 0))
  (Default|ExecuteCommand (CallFunction|TBGameState) _returnvalue))

(event Custom|Cancel%20All%20Request%20Effective%20Card%20%28Server%29
  (for _array_element (CallFunction|GetAllDeckManagers)
    (Default|CancelRequestEffectiveCard(Client) _array_element)))

(event Custom|Request%20Status%20Card
  (params (Triggered%20By%20Card :type BP%20Card%20Object%20Reference))
  (for _array_element (CallFunction|GetAllEnemyTeamDeckManagers (Default|CardRace Triggered%20By%20Card))
    (Default|RequestStatusCard(Client) _array_element)))

(event Custom|Initialize%20Card%20Controllers
  (Networking|SwitchHasAuthority))

(event Custom|Execute%20Build%20Unit%20Ability
  (params (Race :type PlayableRaceEnum%20Enum :default "NewEnumerator6") (Type :type UnitTypeEnum%20Enum :default "NewEnumerator0") (Country :type BP%20Country%20Object%20Reference) (Callback :type I%20Gameplay%20Ability%20Callback%20Interface) (Origin%20Card :type BP%20Card%20Object%20Reference) (Focus :type Boolean))
  (bind _returnvalue (Game|SpawnActorfromClass "/Game/Blueprints/Commands/GameplayAbilities/BP_GA_BuildArmy.BP_GA_BuildArmy_C" (Variables|Default|GetSpawn%20Transform) "Undefined" "MultiplyWithRoot" 0 Race Type Country Focus self Origin%20Card 0))
  (Default|ExecuteAbility _returnvalue))

(event Custom|Play%20Card
  (params (Card :type BP%20Card%20Object%20Reference))
  (bind _output_get (Variables|/Game/Blueprints/Game/BP_TurnBasedGameState.BP_TurnBasedGameState_C|SetActive%20Card (CallFunction|TBGameState) Card))
  (Utilities|Array|RemoveItem (Variables|/Game/Blueprints/Cards/BP_PlayerDeckManager.BP_PlayerDeckManager_C|GetHand (CallFunction|GetDeckManager (Default|CardRace _output_get))) _output_get)
  (Utilities|Array|Add (Variables|/Game/Blueprints/Cards/BP_PlayerDeckManager.BP_PlayerDeckManager_C|GetDeckHistory (CallFunction|GetDeckManager (Default|CardRace _output_get))) "NewEnumerator1")
  (EventDispatchers|BindEventtoCardActionsFinished _output_get (delegate Custom|On%20Card%20Finished))
  (Default|ExecuteCard _output_get)
  (Utilities|Array|Add (Variables|/Game/Blueprints/Cards/BP_PlayerDeckManager.BP_PlayerDeckManager_C|GetPlayedCards (CallFunction|GetDeckManager (Default|CardRace _output_get))) _output_get)
  (switch Utilities|FlowControl|Switch|SwitchonCardTypeEnum (Variables|/Game/DataAssets/PDA_Card.PDA_Card_C|GetType (Variables|/Game/Blueprints/Cards/BP_Card.BP_Card_C|GetCardAsset _output_get))
    (:NewEnumerator3
      (Utilities|Array|Add (Variables|/Game/Blueprints/Cards/BP_PlayerDeckManager.BP_PlayerDeckManager_C|GetStatusCards (CallFunction|GetDeckManager (Default|CardRace _output_get))) _output_get))
    (:NewEnumerator4
      (Utilities|Array|Add (Variables|/Game/Blueprints/Cards/BP_PlayerDeckManager.BP_PlayerDeckManager_C|GetResponseCards (CallFunction|GetDeckManager (Default|CardRace _output_get))) 0))))

(event Custom|Request%20Unit
  (params (Controller :type BP%20Turn%20Based%20Player%20Controller%20Object%20Reference) (Clickable%20Units :type Array%20of%20BP%20Unit%20Object%20References) (Number%20Of%20Units :type Integer))
  (bind _returnvalue (Game|SpawnActorfromClass "/Game/Blueprints/Commands/Commands/SelectCountryCommand.SelectCountryCommand_C" (Variables|Default|GetSpawn%20Transform) "Undefined" "MultiplyWithRoot" Controller Clickable%20Units Number%20Of%20Units 0 0 true 0))
  (Default|ExecuteCommand (CallFunction|TBGameState) _returnvalue))

(event Custom|Request%20Response%20Card%20%28Server%29
  (params (Triggered%20By%20Card :type BP%20Card%20Object%20Reference))
  (for _array_element (CallFunction|GetAllEnemyTeamDeckManagers (Default|CardRace Triggered%20By%20Card))
    (Default|RequestResponseCard(Client) _array_element)))

(event EventBeginPlay
  (CallFunction|InitializeCardControllers))

(event EventAbilityExecutionFinished
  (params (Gameplay%20Ability :type BP%20Gameplay%20Ability%20Object%20Reference))
  (if (Default|IsTriggeredbyCard Gameplay%20Ability)
    (Default|RequestResponseCard(Server) (CallFunction|TBGameState) (Variables|/Game/Blueprints/Commands/GameplayAbilities/BP_GameplayAbility.BP_GameplayAbility_C|GetOrigin%20Card Gameplay%20Ability) Gameplay%20Ability)))

(fn ConstructionScript)