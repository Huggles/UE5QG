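; BP_BuildArmy is a card for a turn-based game that builds a unit, presumably an army, in a country the player selects.
; Playing it runs the parent logic and starts server-side country selection; the callback then asks the server to add the unit.
; Both the callback and the server spawn event call end turn.
; The construction script sets the sprite from the card asset, and the unit-selection callback is empty.
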(event Custom|Ev%20Spawn%20Unit%20%28Server%29
  (params (TB%20Player%20State :type BP%20Turn%20Based%20Player%20State%20Object%20Reference) (Country :type BP%20Country%20Object%20Reference))
  (Default|FnAddUnit Country "NewEnumerator0" TB%20Player%20State)
  (Default|EvEndTurn(Server) (Utilities|GetTBPlayerController self)))

(fn ConstructionScript
  (Rendering|Components|Sprite|SetSprite (Variables|Default|GetPaperSprite_0) (Variables|/Game/DataAssets/PDA_Card.PDA_Card_C|GetImage (Variables|Default|GetCardAsset_0))))

(fn CountrySelectedCallback
  (params (TB%20Player%20State :type BP%20Turn%20Based%20Player%20State%20Object%20Reference) (Selected%20Country :type BP%20Country%20Object%20Reference))
  (Development|PrintString (Utilities|String|Append "Player Selected Country: " (Variables|/Game/Blueprints/Game/BP_TurnBasedPlayerState.BP_TurnBasedPlayerState_C|GetPlayer%20Name TB%20Player%20State) " | " (Utilities|GetDisplayName Selected%20Country)) true true "(R=0.182413,G=1.000000,B=0.159507,A=1.000000)" 5.0)
  (CallFunction|EvSpawnUnit(Server) TB%20Player%20State Selected%20Country)
  (Default|EvEndTurn(Server) (Utilities|GetTBPlayerController self)))

(fn PlayCard
  (params (TB%20PlayerState :type BP%20Turn%20Based%20Player%20State%20Object%20Reference))
  (bind _successful (|CallParentFunction TB%20PlayerState))
  (CallFunction|EvHandleCountrySelect(Server))
  (return _successful))

(fn UnitSelectedCallback
  (params (TB%20Player%20State :type BP%20Turn%20Based%20Player%20State%20Object%20Reference) (Selected%20Unit :type BP%20Unit%20Object%20Reference)))