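; Base card Blueprint for building a naval unit for the card's race.
; On execute, it offers water countries adjacent to any country that race occupies, supplied or not, excluding enemy-owned waters and those already holding its unit.
; The selected country goes to the ability factory's build-unit ability.
; The card is playable only when at least one such country exists.
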(event EventOnCountrySelected(Protected)
  (params (Country :type BP%20Country%20Object%20Reference%20%28by%20ref%29))
  (Default|BuildUnit(Ability) (CallFunction|AbilityFactory) self Country (CallFunction|CardRace) "NewEnumerator1" true true true))

(event EventExecuteCard(Protected)
  (CallFunction|SelectActor(Command) (CallFunction|RelevantCountriesonPlay)))

(event EventBeginPlay
  (|CallParentFunction))

(fn ConstructionScript
  (|CallParentFunction))

(fn RelevantCountriesonPlay
  (for _array_element (Default|GetAllOccupiedCountriesforRace (CallFunction|BPWorld) (CallFunction|CardRace) false)
    (for _array_element_2 (Default|GetAdjacentCountires _array_element)
      (if (Math|Boolean|ANDBoolean (Default|IsWater _array_element_2) (not (Default|IsEnemyOwned _array_element_2 (CallFunction|GetTeamforRace (Variables|Default|GetRace)))) (not (.Player%20Has%20Unit (Default|HasPlayerUnit _array_element_2 (CallFunction|CardRace)))))
        (Utilities|Array|AddUnique (LocalVariables|GetRelevant%20Countries) _array_element_2))))
  (return (LocalVariables|GetRelevant%20Countries)))

(fn Playable
  (return (> (Utilities|Array|Length (CallFunction|RelevantCountriesonPlay)) 0)))

(fn FirstSelectedUnit
  (return (|CallParentFunction)))