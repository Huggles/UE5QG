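; Deck manager that handles a player's card deck and hand in a turn-based, networked card game.
; Server events shuffle the deck or copy valid cards from its front into the hand without removing them, logging each action to DeckHistory.
; DeckHistory's RepNotify reads the latest entry to fire draw, discard or play callbacks, with draws reassigning the array to trigger it.
; ReloadDeck is an empty stub.
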(event Custom|Shuffle%20Deck%20%28Server%29
  (Utilities|Array|Shuffle (Variables|Default|GetDeck))
  (Utilities|Array|Add (Variables|Default|GetDeckHistory) "NewEnumerator3"))

(event Custom|Draw%20Cards%20%28Server%29
  (params (Number :type Integer))
  (if (> (Utilities|Array|Length (Variables|Default|GetDeck)) 0)
    (for _index (range 0 (Math|Integer|Min(Integer) Number (Utilities|Array|Length (Variables|Default|GetDeck))))
      (if (Utilities|IsValid (Utilities|Array|Get(acopy) (Variables|Default|GetDeck) _index))
        (Utilities|Array|Add (Variables|Default|GetHand) (Utilities|Array|Get(acopy) (Variables|Default|GetDeck) _index))))
    (Utilities|Array|Add (Variables|Default|GetDeckHistory) "NewEnumerator0")
    (Variables|Default|SetDeckHistory (Variables|Default|GetDeckHistory))))

(fn ReloadDeck)

(fn OnRepDeckHistory
  (bind _deckhistory (Variables|Default|GetDeckHistory))
  (switch Utilities|FlowControl|Switch|SwitchonPlayerDeckAction (Utilities|Array|Get(acopy) _deckhistory (- (Utilities|Array|Length _deckhistory) 1))
    (:NewEnumerator0
      (Default|CallAfterCardDraw))
    (:NewEnumerator1
      (Default|CallAfterCardDiscard))
    (:NewEnumerator2
      (Default|CallAfterCardPlayed))))