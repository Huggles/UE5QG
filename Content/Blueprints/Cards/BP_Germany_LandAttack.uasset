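; Germany's Land Attack card, which lets the player who plays it attack a clicked unit and then ends their turn.
; The server records the played card, while the playing client runs the card animation and turns on unit selection.
; The unit click callback sends the attack through the client's player controller, disables selection, finishes the card and updates turn state.
; A separate UnitSelectedCallback function repeats only the attack and end-turn calls.
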(event EventPlayCard(Server/Logic)
  (params (TB%20PlayerState :type BP%20Turn%20Based%20Player%20State%20Object%20Reference))
  (Networking|SwitchHasAuthority
    (:Authority
      (|CallParentFunction TB%20PlayerState)
      (Default|AddPlayedCard (Variables|Default|GetPlayerState) self))))

(event EventPlayCardSelf(Client/Animation)
  (params (TB%20PlayerState :type BP%20Turn%20Based%20Player%20State%20Object%20Reference))
  (Networking|SwitchHasAuthority
    (:Remote
      (bind _is_current_client (Default|IsCurrentClientPlayerState TB%20PlayerState))
      (if _is_current_client
        (|CallParentFunction TB%20PlayerState)
        (CallFunction|ToggleUnitSelection true)))))

(event EventUnitClickedCallback
  (params (Unit :type BP%20Unit%20Object%20Reference) (TB%20Player%20State :type BP%20Turn%20Based%20Player%20State%20Object%20Reference))
  (Development|PrintString " Unit Clicked Callback" true true "(R=0.541493,G=0.000000,B=1.000000,A=1.000000)" 5.0)
  (bind _asbp_turn_based_player_controller (CallFunction|GetPlayerController(Client)))
  (Default|EvAttackUnit(Server) _asbp_turn_based_player_controller (Utilities|Struct|MakeAttackUnitPayload TB%20Player%20State Unit (Variables|/Game/Blueprints/Units/BP_Unit.BP_Unit_C|GetCountry Unit)))
  (CallFunction|ToggleUnitSelection false)
  (CallFunction|CardFinishedExecution(Server))
  (Default|EvSetPlayerTurnState(Server) _asbp_turn_based_player_controller "NewEnumerator0")
  (Default|EvEndTurn(Server) _asbp_turn_based_player_controller))

(event EventSetupCard(Server))

(event EventSetupCard(Client)
  (CallFunction|StartListeningtoUnitClicks))

(fn ConstructionScript
  (Rendering|Components|Sprite|SetSprite (Variables|Default|GetPaperSprite_0) (Variables|/Game/DataAssets/PDA_Card.PDA_Card_C|GetSprite (Variables|Default|GetCardAsset_0))))

(fn UnitSelectedCallback
  (params (Clicked%20Actor :type Actor%20Object%20Reference) (TB%20Player%20State :type BP%20Turn%20Based%20Player%20State%20Object%20Reference))
  (bind _asbp_unit (Utilities|Casting|CastToBP_Unit Clicked%20Actor))
  (bind _asbp_turn_based_player_controller (CallFunction|GetPlayerController(Client)))
  (Default|EvAttackUnit(Server) _asbp_turn_based_player_controller (Utilities|Struct|MakeAttackUnitPayload TB%20Player%20State _asbp_unit (Variables|/Game/Blueprints/Units/BP_Unit.BP_Unit_C|GetCountry _asbp_unit)))
  (Default|EvEndTurn(Server) _asbp_turn_based_player_controller))