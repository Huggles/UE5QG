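; BP_CA_SelectUnit is a card action that has the player pick a unit by clicking it.
; On execution it starts listening for unit clicks; the first click stores the unit as SelectedUnit, signals the action as finished and stops listening.
; Applicable countries come unchanged from the parent implementation.
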(event EventExecuteAction
  (CallFunction|StartListeningtoUnitClicks))

(event EventOnUnitClicked
  (params (Unit :type BP%20Unit%20Object%20Reference) (Player%20State :type BP%20Turn%20Based%20Player%20State%20Object%20Reference))
  (Variables|Default|SetSelected%20Unit Unit)
  (Default|CallActionFinished self)
  (CallFunction|StopListeningtoUnitClicks))

(fn ConstructionScript)

(fn GetApplicableCountries
  (return (|CallParentFunction)))