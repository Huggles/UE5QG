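; Card Blueprint that builds a naval unit for the card's race in a chosen sea country.
; Valid targets are water countries adjacent to those the race occupies, supplied or not, excluding enemy-owned ones and ones already holding its unit.
; The card is playable only when a target exists.
; Local prediction highlights targets, while CardExecutionManager handles the country request and runs the build-unit ability after the server-side click.
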(event EventExecuteCard(LocalPredicted)
  (Default|ChangeUIState (Variables|Default|GetPlayer%20Controller) "NewEnumerator2")
  (Variables|/Game/Blueprints/Game/BP_TurnBasedPlayerState.BP_TurnBasedPlayerState_C|SetClickableActors (Variables|Default|GetPlayer%20State) (CallFunction|RelevantCountries)))

(event EventAbilityExecutionFinished
  (params (Gameplay%20Ability :type BP%20Gameplay%20Ability%20Object%20Reference)))

(event EventExecuteCard
  (Default|RequestCountry (CallFunction|CardExecutionManager) (Variables|Default|GetPlayer%20Controller) (CallFunction|RelevantCountries) self 1))

(event EventOnCountryClicked(Server)
  (params (TB%20Controller :type BP%20Turn%20Based%20Player%20Controller%20Object%20Reference) (Country :type BP%20Country%20Object%20Reference))
  (bind _self self)
  (if (== TB%20Controller (Variables|Default|GetPlayer%20Controller))
    (CallFunction|HandleonCountrySelected Country)
    (Default|ExecuteBuildUnitAbility (CallFunction|CardExecutionManager) (CallFunction|CardRace) "NewEnumerator1" (CallFunction|FirstSelectedCountry) _self _self true)))

(fn ConstructionScript
  (|CallParentFunction))

(fn RelevantCountries
  (bind _country (Default|GetAllOccupiedCountriesforRace (CallFunction|TBGameState) (CallFunction|CardRace) false))
  (for _array_element _country
    (bind _adjacent_countries (Default|GetAdjacentCountires _array_element))
    (for _array_element_2 _adjacent_countries
      (if (Math|Boolean|ANDBoolean (Default|IsWater _array_element_2) (not (Default|IsEnemyOwned _array_element_2 (CallFunction|GetTeamforRace (Variables|/Game/DataAssets/PDA_Card.PDA_Card_C|GetRace (Variables|Default|GetCardAsset))))) (not (Default|HasPlayerUnit _array_element_2 (CallFunction|CardRace))))
        (Utilities|Array|AddUnique (LocalVariables|GetRelevant%20Countries) _array_element_2))))
  (return (LocalVariables|GetRelevant%20Countries)))

(fn Playable
  (return (> (Utilities|Array|Length (CallFunction|RelevantCountries)) 0)))