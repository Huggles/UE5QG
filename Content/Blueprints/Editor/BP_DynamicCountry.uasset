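; Editor-side generated dynamic mesh actor that builds country terrain geometry from a displacement texture when Compute is enabled.
; On rebuild, it copies SourceMesh and scales X and Y to the texture's size divided by PixelsPerUnit.
; Geometry Script then applies PN tessellation, texture displacement, iterative smoothing and normal recomputation.
; A final flipped plane cut at CutFrameLocationZ trims the displaced mesh by height.
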(event EventBeginPlay)

(event Collision|EventActorBeginOverlap
  (params (OtherActor :type Actor%20Object%20Reference)))

(event EventTick
  (params (DeltaSeconds :type Float%20%28single-precision%29)))

(event Events|EventOnRebuildGeneratedMesh
  (params (TargetMesh :type Dynamic%20Mesh%20Object%20Reference))
  (if (Variables|Default|GetCompute)
    (CallFunction|FnGenerateMesh TargetMesh)))

(fn ConstructionScript)

(fn FnGenerateMesh
  (params (Target%20Mesh :type Dynamic%20Mesh%20Object%20Reference))
  (bind _pixelsperunit (Variables|Default|GetPixelsPerUnit))
  (bind _displacemap (Variables|Default|GetDisplaceMap))
  (bind _sourcemesh (Variables|Default|GetSourceMesh)
    (:then
      (bind _returnvalue (GeometryScript|StaticMesh|CopyMeshFromStaticMesh :FromStaticMeshAsset _sourcemesh :ToDynamicMesh Target%20Mesh :Debug 0)
        (:Success
          (bind _returnvalue_2 (Class|GeometryScriptLibraryMeshTransformFunctions|ScaleMesh _returnvalue (Math|Vector|MakeVector (/ (Math|Conversions|ToFloat(Integer) (Class|Texture2D|BlueprintGetSizeX _displacemap)) _pixelsperunit) (/ (Math|Conversions|ToFloat(Integer) (Class|Texture2D|BlueprintGetSizeY _displacemap)) _pixelsperunit) 1.0) "0.000000,0.000000,0.000000" true 0))
          (bind _returnvalue_3 (Class|GeometryScriptLibraryMeshSubdivideFunctions|ApplyPNTessellation _returnvalue_2 (Utilities|Struct|MakeGeometryScriptPNTessellateOptions true) (Variables|Default|GetTessellation) 0))
          (bind _displacemap_2 (Variables|Default|GetDisplaceMap)
            (:then
              (bind _returnvalue_4 (Class|GeometryScriptLibraryMeshDeformFunctions|ApplyDisplacefromTextureMap :TargetMesh _returnvalue_3 :Texture _displacemap_2 :Options (Utilities|Struct|MakeGeometryScriptDisplaceFromTextureOptions (Variables|Default|GetOptions%20Magnitude) "(X=1.000000,Y=1.000000)" "(X=0.000000,Y=0.000000)" 0.5 0 "FullMeshSelection") :Debug 0))
              (bind _returnvalue_5 (Class|GeometryScriptLibraryMeshDeformFunctions|ApplyIterativeSmoothingtoMesh :TargetMesh _returnvalue_4 :Debug 0))
              (bind _returnvalue_6 (GeometryScript|Normals|RecomputeNormals :TargetMesh _returnvalue_5 :Debug 0))
              (Class|GeometryScriptLibraryMeshBooleanFunctions|ApplyMeshPlaneCut _returnvalue_6 (Math|Transform|MakeTransform (Math|Vector|MakeVector 0.0 0.0 (Variables|Default|GetCut%20Frame%20Location%20Z)) "0, 0, 0" "1.000000,1.000000,1.000000") (Utilities|Struct|MakeGeometryScriptMeshPlaneCutOptions true true true 1.0) 0))
            (:else)))))
    (:else)))