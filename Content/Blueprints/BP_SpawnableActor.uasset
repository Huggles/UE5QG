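; BP_SpawnableActor is an actor that tracks which TB player controllers have had its spawn reported to it.
; On BeginPlay it registers itself with the first local TB player controller.
; AddActorSpawnedForController records each controller uniquely and fires a per-controller spawned call.
; When the recorded count matches the count of all TB player controllers, it fires the spawned-on-all call.
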(event Custom|Add%20Actor%20Spawned%20For%20Controller
  (params (Controller :type BP%20Turn%20Based%20Player%20Controller%20Object%20Reference))
  (bind _self self)
  (bind _spawned_for_controllers (Variables|Default|GetSpawned%20For%20Controllers))
  (Utilities|Array|AddUnique _spawned_for_controllers Controller)
  (Default|CallActorSpawnedforController Controller _self)
  (if (== (Utilities|Array|Length _spawned_for_controllers) (Utilities|Array|Length (CallFunction|GetAllTBPlayerControllers)))
    (Default|CallActorSpawnedonAll _self)))

(event EventBeginPlay
  (Default|RegisterActorSpawned (CallFunction|GetFirstLocalTBPlayerController) self))

(fn ConstructionScript)