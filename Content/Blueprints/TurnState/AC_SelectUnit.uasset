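; AC_SelectUnit is a turn-state component for unit selection that manages its client UI and clears unit click bindings.
; BeginPlay runs client setup, which creates a UIB_TurnState_SelectCountry widget for the client player controller and adds it to the viewport; EndPlay removes it.
; UnregisterUnitSelectCallback makes every BP_Unit in the world unselectable and unbinds all its UnitClicked events.
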(event Custom|Setup%20%28Client%29
  ;[1 1 1] Setup UI
  (bind _asbp_turn_based_player_controller (CallFunction|GetPlayerController(Client)))
  (bind _returnvalue (UserInterface|CreateWidget "/Game/Blueprints/UI/UIB_TurnState_SelectCountry.UIB_TurnState_SelectCountry_C" _asbp_turn_based_player_controller 0))
  (bind _output_get (Variables|Default|SetUserInterfaceWidget _returnvalue))
  (UserInterface|Viewport|AddtoViewport _output_get 0))

(event EventBeginPlay
  (CallFunction|Setup(Client)))

(event EventEndPlay
  (params (EndPlayReason :type EEndPlayReason%20Enum :default "Destroyed"))
  (Widget|RemovefromParent (Variables|Default|GetUserInterfaceWidget)))

(fn UnregisterUnitSelectCallback
  (bind _outactors (Actor|GetAllActorsOfClass "/Game/Blueprints/Units/BP_Unit.BP_Unit_C"))
  (for _array_element _outactors
    (Variables|/Game/Blueprints/Units/BP_Unit.BP_Unit_C|SetSelectable _array_element false)
    (EventDispatchers|UnbindallEventsfromUnitClicked _array_element)))