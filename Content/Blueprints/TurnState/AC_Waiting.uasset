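; AC_Waiting is a turn-state component that shows the waiting screen on the client while it is active.
; On BeginPlay it runs client setup, which on the remote side creates a UIB_TurnState_Waiting widget for the client player controller and adds it to the viewport.
; EndPlay removes that widget on the remote side, so the UI lasts only as long as the component.
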(event Custom|Setup%20%28Client%29
  (Networking|SwitchHasAuthority
    (:Remote
      (bind _asbp_turn_based_player_controller (CallFunction|GetPlayerController(Client)))
      (bind _returnvalue (UserInterface|CreateWidget "/Game/Blueprints/UI/UIB_TurnState_Waiting.UIB_TurnState_Waiting_C" _asbp_turn_based_player_controller))
      (bind _output_get (Variables|Default|SetUserInterfaceWidget _returnvalue))
      (UserInterface|Viewport|AddtoViewport _output_get 0))))

(event EventBeginPlay
  (CallFunction|Setup(Client)))

(event EventEndPlay
  (params (EndPlayReason :type EEndPlayReason%20Enum :default "Destroyed"))
  (Networking|SwitchHasAuthority
    (:Remote
      (Widget|RemovefromParent (Variables|Default|GetUserInterfaceWidget)))))