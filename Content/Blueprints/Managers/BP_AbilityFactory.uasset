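; Factory that spawns ability and command actors for card-driven unit deployment, attacks, discards and player selections in a turn-based board game.
; Ability functions spawn and immediately execute their actor, drawing deployed units from per-faction pools in the game state.
; Command functions spawn commands for the ServerCommandManager, optionally queuing unit builds and batching card reveals to all controllers as blocking.
; "If Possible" variants validate board or country state first and return a success flag.
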(fn ConstructionScript)

(fn DeployUnit(Ability)
  (params (Origin%20Card :type BP%20Card%20Object%20Reference) (Country :type BP%20Country%20Object%20Reference) (Race :type FactionEnum%20Enum :default "NewEnumerator0") (Type :type UnitTypeEnum%20Enum :default "NewEnumerator0") (Deploy%20Type :type UnitDeployTypeEnum%20Enum :default "NewEnumerator0"))
  (bind _unit (Default|PopAvailableUnit (.Value (Utilities|Map|Find (Variables|/Game/Blueprints/Game/BP_TurnBasedGameState.BP_TurnBasedGameState_C|GetUnit%20Pool%20By%20Faction (.TB%20Game%20State (CallFunction|TBGameState))) Race)) Type))
  (bind _returnvalue (Game|SpawnActorfromClass "/Game/Blueprints/Abilities/BP_Ability_DeployUnit.BP_Ability_DeployUnit_C" (Variables|Default|GetSpawn%20Transform) "Undefined" "MultiplyWithRoot" 0 Deploy%20Type _unit Country Origin%20Card 0))
  (Default|ExecuteAbility _returnvalue)
  (return _returnvalue))

(fn DeployUnitifPossible(Ability)
  (params (Origin%20Card :type BP%20Card%20Object%20Reference) (Country :type BP%20Country%20Object%20Reference) (Faction :type FactionEnum%20Enum :default "NewEnumerator0") (Unit%20Type :type UnitTypeEnum%20Enum :default "NewEnumerator0") (Deploy%20Type :type UnitDeployTypeEnum%20Enum :default "NewEnumerator0"))
  (Utilities|FlowControl|Sequence
    (:then_0
      (Utilities|FlowControl|Sequence
        (:then_0
          (LocalVariables|SetOrigin%20Card%20Local Origin%20Card))
        (:then_1
          (LocalVariables|SetCountry%20Local Country))
        (:then_2
          (LocalVariables|SetFaction%20Local Faction))
        (:then_3
          (LocalVariables|SetUnit%20Type%20Local Unit%20Type))
        (:then_4
          (LocalVariables|SetDeploy%20Type%20Local Deploy%20Type))))
    (:then_1
      (if (Default|CanDeployUnitinCountry (CallFunction|BoardManager) (LocalVariables|GetCountry%20Local) (LocalVariables|GetFaction%20Local) (LocalVariables|GetUnit%20Type%20Local) (LocalVariables|GetDeploy%20Type%20Local))
        (bind _unit (Default|PopAvailableUnit (.Value (Utilities|Map|Find (Variables|/Game/Blueprints/Game/BP_TurnBasedGameState.BP_TurnBasedGameState_C|GetUnit%20Pool%20By%20Faction (.TB%20Game%20State (CallFunction|TBGameState))) (LocalVariables|GetFaction%20Local))) (LocalVariables|GetUnit%20Type%20Local)))
        (bind _returnvalue (Game|SpawnActorfromClass "/Game/Blueprints/Abilities/BP_Ability_DeployUnit.BP_Ability_DeployUnit_C" (Variables|Default|GetSpawn%20Transform) "Undefined" "MultiplyWithRoot" 0 "NewEnumerator0" _unit (LocalVariables|GetCountry%20Local) (LocalVariables|GetOrigin%20Card%20Local) 0))
        (Default|ExecuteAbility _returnvalue)
        (return true _returnvalue)
        (else
          (return false 0))))))

(fn EliminateUnit(Ability)
  (params (Origin%20Card :type BP%20Card%20Object%20Reference) (Unit :type BP%20Unit%20Object%20Reference))
  (bind _returnvalue (Game|SpawnActorfromClass "/Game/Blueprints/Abilities/BP_Ability_EliminateUnit.BP_Ability_EliminateUnit_C" (Variables|Default|GetSpawn%20Transform) "Undefined" "MultiplyWithRoot" 0 Unit Origin%20Card 0))
  (Default|ExecuteAbility _returnvalue)
  (return _returnvalue))

(fn ForceCardDiscard(Ability)
  (params (Origin%20Card :type BP%20Card%20Object%20Reference) (Target%20Card :type BP%20Card%20Object%20Reference))
  (bind _returnvalue (Game|SpawnActorfromClass "/Game/Blueprints/Abilities/BP_Ability_ForceStatusCardDiscard.BP_Ability_ForceStatusCardDiscard_C" (Variables|Default|GetSpawn%20Transform) "Undefined" "MultiplyWithRoot" 0 Target%20Card Origin%20Card 0))
  (Default|ExecuteAbility _returnvalue)
  (return _returnvalue))

(fn AttackCountry(Ability)
  (params (Origin%20Card :type BP%20Card%20Object%20Reference) (Country :type BP%20Country%20Object%20Reference))
  (bind _returnvalue (Game|SpawnActorfromClass "/Game/Blueprints/Abilities/BP_Ability_AttackCountry.BP_Ability_AttackCountry_C" (Variables|Default|GetSpawn%20Transform) "Undefined" "MultiplyWithRoot" 0 Country Origin%20Card 0))
  (Default|ExecuteAbility _returnvalue))

(fn AttackUnit(Ability)
  (params (Origin%20Card :type BP%20Card%20Object%20Reference) (Unit :type BP%20Unit%20Object%20Reference))
  (bind _returnvalue (Game|SpawnActorfromClass "/Game/Blueprints/Abilities/BP_Ability_AttackUnit.BP_Ability_AttackUnit_C" (Variables|Default|GetSpawn%20Transform) "Undefined" "MultiplyWithRoot" 0 Unit Origin%20Card 0))
  (Default|ExecuteAbility _returnvalue)
  (return _returnvalue))

(fn ShowCardPlaytoAllControllers(Command)
  (params (Card :type BP%20Card%20Object%20Reference))
  (for _array_element (CallFunction|GetAllTBPlayerControllers)
    (bind _returnvalue (Game|SpawnActorfromClass "/Game/Blueprints/Commands/ClientCommands/ShowCardPlayClientCommand.ShowCardPlayClientCommand_C" (Variables|Default|GetSpawn%20Transform) "Undefined" "MultiplyWithRoot" _array_element (.Time (Default|GameSpeed (.TB%20Game%20State (CallFunction|TBGameState)))) Card false true 0))
    (Utilities|Array|AddUnique (LocalVariables|GetCommands%20Local) _returnvalue))
  (bind _client_command_batch (Default|MakeBatchforCommands (CallFunction|ServerCommandManager) (LocalVariables|GetCommands%20Local) true true))
  (return _client_command_batch))

(fn BuildUnit(Command)
  (params (Faction :type FactionEnum%20Enum :default "NewEnumerator0") (Type :type UnitTypeEnum%20Enum :default "NewEnumerator0") (Country :type BP%20Country%20Object%20Reference) (Blocking :type Boolean) (Skip%20Animation :type Boolean) (Add%20To%20Queue :type Boolean))
  (bind _unit (Default|PopAvailableUnit (.Value (Utilities|Map|Find (Variables|/Game/Blueprints/Game/BP_TurnBasedGameState.BP_TurnBasedGameState_C|GetUnit%20Pool%20By%20Faction (.TB%20Game%20State (CallFunction|TBGameState))) Faction)) Type))
  (bind _returnvalue (Game|SpawnActorfromClass "/Game/Blueprints/Commands/ServerCommands/DeployUnitCommand.DeployUnitCommand_C" (Variables|Default|GetSpawn%20Transform) "Undefined" "MultiplyWithRoot" 0 _unit Country Skip%20Animation 0 Blocking 0))
  (if Add%20To%20Queue
    (Default|AddCommand (CallFunction|ServerCommandManager) _returnvalue))
  (return _returnvalue))

(fn SelectEnemyUnitifPossible(Command)
  (params (Target%20Controller :type BP%20Turn%20Based%20Player%20Controller%20Object%20Reference) (Faction :type FactionEnum%20Enum :default "NewEnumerator0") (Country :type BP%20Country%20Object%20Reference))
  (if (Default|IsEnemyOwned Country (CallFunction|GetTeamforFaction Faction))
    (bind _select_actor_client_command (Command|SelectActor(Command) Target%20Controller (Default|GetUnits Country) false))
    (return true _select_actor_client_command)
    (else
      (return false 0))))

(fn SelectActor(Command)
  (params (Target%20Controller :type BP%20Turn%20Based%20Player%20Controller%20Object%20Reference) (Actors :type Array%20of%20Actor%20Object%20References) (Skippable :type Boolean))
  (bind _returnvalue (Game|SpawnActorfromClass "/Game/Blueprints/Commands/ClientCommands/SelectActorClientCommand.SelectActorClientCommand_C" (Variables|Default|GetSpawn%20Transform) "Undefined" "MultiplyWithRoot" Target%20Controller Actors 1 Skippable true 0))
  (Default|AddCommand (CallFunction|ServerCommandManager) _returnvalue)
  (return _returnvalue))

(fn SelectCardData(Command)
  (params (Race :type FactionEnum%20Enum :default "NewEnumerator0") (Card%20Data%20Structs :type Array%20of%20Card%20Struct%20Structures) (Title :type String) (Accept%20Button%20Label :type String) (Decline%20Button%20Label :type String) (Show%20Decline%20Button :type Boolean) (Skippable :type Boolean))
  (bind _returnvalue (Game|SpawnActorfromClass "/Game/Blueprints/Commands/ClientCommands/SelectCardReferenceClientCommand.SelectCardReferenceClientCommand_C" (Variables|Default|GetSpawn%20Transform) "Undefined" "MultiplyWithRoot" (CallFunction|GetControllerforRace(ServerOnly) Race) Card%20Data%20Structs Title Accept%20Button%20Label Decline%20Button%20Label Show%20Decline%20Button Skippable true 0))
  (Default|AddCommand (CallFunction|ServerCommandManager) _returnvalue)
  (return _returnvalue))