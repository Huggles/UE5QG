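; BP_SFXManager is a manager Blueprint that plays background music and 2D sound effects.
; On BeginPlay, only in builds packaged for distribution, it spawns a random track from BackgroundMusicAssets, stores it as ActiveMusic and lowers its volume.
; A separate event pauses that music, with no resume event.
; ShowPlaySoundEffect plays a sound after an optional wait; any positive Duration triggers StopDelayed with zero delay, so the value itself is unused.
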(event Custom|Show%20Play%20Sound%20Effect
  (params (Sound :type Sound%20Base%20Object%20Reference) (Wait :type Float%20%28double-precision%29) (Duration :type Float%20%28single-precision%29) (VolumeMultiplier :type Float%20%28single-precision%29))
  (if (> Wait 0.0)
    (Utilities|FlowControl|Delay Wait))
  (bind _returnvalue (Audio|SpawnSound2D Sound VolumeMultiplier 1.0 0.0 0))
  (if (> Duration 0.0)
    (Audio|Components|Audio|StopDelayed _returnvalue 0.0)))

(event Custom|Pauze%20Background%20Music
  (Class|AudioComponent|SetPaused (Variables|Default|GetActive%20Music) true))

(event Custom|Play%20Background%20Music
  (bind _returnvalue (Audio|SpawnSound2D (.OutItem (Utilities|Array|Random (Variables|Default|GetBackground%20Music%20Assets))) 1.0 1.0 0.0 0))
  (bind _output_get (Variables|Default|SetActive%20Music _returnvalue))
  (Audio|Components|Audio|AdjustVolume _output_get 0.0 0.1 "Linear" :!class /Script/Engine.AudioComponent))

(event EventBeginPlay
  (if (Class|KismetSystemLibrary|IsPackagedforDistribution)
    (CallFunction|PlayBackgroundMusic)))

(fn ConstructionScript)