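; Debug gizmo that visualizes country connections and build options for one faction at a time.
; Releasing U advances a counter, mapped to a faction through a hand-ordered Select, and resets it after the last entry.
; For that faction, timed debug lines in its color link occupied countries to their faction-specific neighbors from the game state.
; Neighbors get green circles where a navy can be built and orange where an army can.
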(event Custom|Toggle
  (bind _height (Variables|Default|GetHeight))
  (bind _output_get (Variables|Default|SetFaction%20Counter (+ (Variables|Default|GetFaction%20Counter) 1)))
  (if (> _output_get -1)
    (if (< _output_get (|GetNumEnumEntries))
      (Development|PrintString (Utilities|String|EnumtoString (CallFunction|Faction)))
      (for _array_element (.occupiedcountries (Default|GetFactionState (.TB%20Game%20State (CallFunction|TBGameState)) (CallFunction|Faction)))
        (for _array_element_2 (Default|GetAdjacentCountriesforFaction _array_element (CallFunction|Faction))
          (Rendering|Debug|DrawDebugLine (Math|Vector|MakeVector (.x (Transformation|GetActorLocation _array_element_2)) (.y (Transformation|GetActorLocation _array_element_2)) (+ (.z (Transformation|GetActorLocation _array_element_2)) _height)) (Math|Vector|MakeVector (.x (Transformation|GetActorLocation _array_element)) (.y (Transformation|GetActorLocation _array_element)) (+ (.z (Transformation|GetActorLocation _array_element)) _height)) (Math|Conversions|ToLinearColor(Color) (.color (Default|GetRaceStructStructforRace (.TB%20Game%20State (CallFunction|TBGameState)) (CallFunction|Faction)))) 1e+01 1e+01)
          (if (Default|CanBuildNavy _array_element_2 (CallFunction|Faction))
            (Rendering|Debug|DrawDebugCircle (Math|Vector|MakeVector (.x (Transformation|GetActorLocation _array_element_2)) (.y (Transformation|GetActorLocation _array_element_2)) (+ (.z (Transformation|GetActorLocation _array_element_2)) (Variables|Default|GetHeight))) 5e+01 12 "(R=0.032606,G=1.000000,B=0.013192,A=1.000000)" 1e+01 1e+01 "1.000000,0.000000,0.000000" "0.000000,1.000000,0.000000"))
          (if (Default|CanBuildArmy _array_element_2 (CallFunction|Faction))
            (Rendering|Debug|DrawDebugCircle (Math|Vector|MakeVector (.x (Transformation|GetActorLocation _array_element_2)) (.y (Transformation|GetActorLocation _array_element_2)) (+ (.z (Transformation|GetActorLocation _array_element_2)) (Variables|Default|GetHeight))) 5e+01 12 "(R=1.000000,G=0.273160,B=0.000000,A=1.000000)" 1e+01 1e+01 "1.000000,0.000000,0.000000" "0.000000,1.000000,0.000000"))))
      (else
        (Variables|Default|SetFaction%20Counter -1)))))

(event Input|EnhancedActionEvents|EnhancedInputActionIA_Toggle_Debug
  (params (ActionValue :type Vector%202D%20Structure) (ElapsedSeconds :type Float%20%28double-precision%29) (TriggeredSeconds :type Float%20%28double-precision%29) (InputAction :type Input%20Action%20Object%20Reference :default "/Game/Input/IA_Toggle_Debug.IA_Toggle_Debug")))

(event Input|KeyboardEvents|U
  (params (Key :type Key%20Structure :default "None"))
  (:Released
    (Development|PrintString "Toggle DEbug")
    (CallFunction|Toggle)))

(fn ConstructionScript)

(fn Faction
  (return (Utilities|Select :Index (Variables|Default|GetFaction%20Counter) :Option%200 "NewEnumerator0" :Option%201 "NewEnumerator3" :Option%202 "NewEnumerator2" :Option%203 "NewEnumerator4" :Option%204 "NewEnumerator1" :Option%205 "NewEnumerator5")))