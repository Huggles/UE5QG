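; Debug utility Blueprint that visualizes and refreshes board state by faction through three debug input actions.
; The first two actions cycle a faction counter and a debug-function counter, each wrapping to -1, then run the selected function.
; The only wired function tints countries the BoardManager reports as occupied by that faction.
; The third recalculates board state on authority only; line and circle drawing code is left disconnected.
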(event Custom|Increment%20Faction%20Counter
  (bind _output_get (Variables|Default|SetFaction%20Counter (+ (Variables|Default|GetFaction%20Counter) 1)))
  (if (> _output_get -1)
    (if (not (< _output_get (|GetNumEnumEntries)))
      (Variables|Default|SetFaction%20Counter -1))))

(event Custom|Show%20Occupied%20Countries
  (for _array_element (Default|GetOccupiedCountries (CallFunction|BoardManager) (CallFunction|Faction))
    (Default|SetDebugColor _array_element "(R=0.000000,G=0.761661,B=1.000000,A=1.000000)")))

(event Custom|Increment%20Debug%20Counter
  (bind _output_get (Variables|Default|SetDebug%20Function%20Counter (+ (Variables|Default|GetDebug%20Function%20Counter) 1)))
  (if (> _output_get -1)
    (if (not (< _output_get 1))
      (Variables|Default|SetDebug%20Function%20Counter -1))))

(event Input|EnhancedActionEvents|EnhancedInputActionIA_Toggle_Debug_1
  (params (ActionValue :type Vector%202D%20Structure) (ElapsedSeconds :type Float%20%28double-precision%29) (TriggeredSeconds :type Float%20%28double-precision%29) (InputAction :type Input%20Action%20Object%20Reference :default "/Game/Input/IA_Toggle_Debug_1.IA_Toggle_Debug_1"))
  (:Completed
    (CallFunction|IncrementFactionCounter)
    (switch int (Variables|Default|GetDebug%20Function%20Counter)
      (:0
        (CallFunction|ShowOccupiedCountries)))))

(event Input|EnhancedActionEvents|EnhancedInputActionIA_Toggle_Debug_2
  (params (ActionValue :type Vector%202D%20Structure) (ElapsedSeconds :type Float%20%28double-precision%29) (TriggeredSeconds :type Float%20%28double-precision%29) (InputAction :type Input%20Action%20Object%20Reference :default "/Game/Input/IA_Toggle_Debug_2.IA_Toggle_Debug_2"))
  (:Completed
    (CallFunction|IncrementDebugCounter)
    (switch int (Variables|Default|GetDebug%20Function%20Counter)
      (:0
        (CallFunction|ShowOccupiedCountries)))))

(event Input|EnhancedActionEvents|EnhancedInputActionIA_Toggle_Debug_3
  (params (ActionValue :type Vector%202D%20Structure) (ElapsedSeconds :type Float%20%28double-precision%29) (TriggeredSeconds :type Float%20%28double-precision%29) (InputAction :type Input%20Action%20Object%20Reference :default "/Game/Input/IA_Toggle_Debug_3.IA_Toggle_Debug_3"))
  (:Completed
    (Networking|SwitchHasAuthority
      (:Authority
        (Default|RecalculateBoardState (CallFunction|BoardManager))))))

(fn ConstructionScript)

(fn Faction
  (return (Utilities|Select :Index (Variables|Default|GetFaction%20Counter) :Option%200 "NewEnumerator0" :Option%201 "NewEnumerator3" :Option%202 "NewEnumerator2" :Option%203 "NewEnumerator4" :Option%204 "NewEnumerator1" :Option%205 "NewEnumerator5")))