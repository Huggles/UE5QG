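; BP_Ability_EliminateUnit is an ability that attacks a single unit with an explosion effect, framed by camera moves.
; AbilityCommands spawns and returns three command actors in order: move the camera to show the unit, attack it with a scaled explosion emitter, then return the camera.
; PrefillAbilityOutcome fills the ability outcome with the target unit, its race and its country.
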(fn ConstructionScript
  (|CallParentFunction))

(fn AbilityCommands
  (bind _unit (Variables|Default|GetUnit))
  (bind _returnvalue (Game|SpawnActorfromClass "/Game/Blueprints/Commands/ClientCommands/MoveCameraClientCommand.MoveCameraClientCommand_C" (Variables|Default|GetSpawn%20Transform) "Undefined" "MultiplyWithRoot" 0 1.0 (CallFunction|GetCameraPositiontoShowActor _unit) true 0 0 0))
  (bind _returnvalue_2 (Game|SpawnActorfromClass "/Game/Blueprints/Commands/ServerCommands/AttackUnitCommand.AttackUnitCommand_C" (Variables|Default|GetSpawn%20Transform) "Undefined" "MultiplyWithRoot" 0 _unit 1.0 1.0 "5.000000,5.000000,5.000000" "/Game/StarterContent/Particles/P_Explosion.P_Explosion" true 0 0 0))
  (bind _returnvalue_3 (Game|SpawnActorfromClass "/Game/Blueprints/Commands/ClientCommands/ReturnCameraClientCommand.ReturnCameraClientCommand_C" (Variables|Default|GetSpawn%20Transform) "Undefined" "MultiplyWithRoot" 0 true 0 0 0))
  (return (Utilities|Array|MakeArray _returnvalue _returnvalue_2 _returnvalue_3)))

(fn PrefillAbilityOutcome
  (params (Empty%20Ability%20Outcome :type Ability%20Outcome%20Structure))
  (bind _unit (Variables|Default|GetUnit))
  (bind _structout (Utilities|Struct|SetmembersinAbilityOutcome Empty%20Ability%20Outcome "NewEnumerator0" (Variables|/Game/Blueprints/Units/BP_Unit.BP_Unit_C|GetRace _unit) (Variables|/Game/Blueprints/Units/BP_Unit.BP_Unit_C|GetCountry _unit) _unit))
  (return _structout))