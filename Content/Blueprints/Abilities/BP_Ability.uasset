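; Base actor for a card-triggered ability in a turn-based, race-based card game, with overridable hooks for preprocessing, commands and outcome.
; On authority it queues server commands; when the last finishes, optional Response (enemy) and Status (owner) card windows follow, each repeating after a played card finishes.
; Each window sets player turn states and the game state's active card and ability.
; Finishing resets turn states, notifies the origin card and destroys the actor.
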(event Custom|CommandFinished_Event
  (params (Command :type BP%20Command%20Object%20Reference) (Result :type Command%20Result%20Structure))
  (Utilities|FlowControl|Delay 1.0)
  (CallFunction|AbilityExecuted))

(event Custom|No%20Status%20Card%20Played
  ;[0.5996 0.474 1] Status Card
  (CallFunction|SetActiveCardandAbility)
  (CallFunction|AbilityFinished))

(event Custom|Ability%20Finished
  (bind _origin_card (Variables|Default|GetOrigin%20Card))
  (Variables|Default|SetStage "NewEnumerator5")
  (CallFunction|SetFinishedStates)
  (Utilities|FlowControl|Sequence
    (:then_0
      (if (Utilities|IsValid _origin_card)
        (Default|AbilityFinished _origin_card self)))
    (:then_1
      (Variables|Default|SetProcessed true))
    (:then_2
      (Utilities|FlowControl|Delay 1.0)
      (Actor|DestroyActor))))

(event Custom|No%20Response%20Card%20Played
  ;[1 0.6267 0.6842] Response
  (CallFunction|SetActiveCardandAbility)
  (CallFunction|RequestStatusCard))

(event Custom|Set%20Active%20Card%20And%20Ability
  (Variables|/Game/Blueprints/Game/BP_TurnBasedGameState.BP_TurnBasedGameState_C|SetActive%20Card (.TB%20Game%20State (CallFunction|TBGameState)) (Variables|Default|GetOrigin%20Card))
  (Variables|/Game/Blueprints/Game/BP_TurnBasedGameState.BP_TurnBasedGameState_C|SetActive%20Ability (.TB%20Game%20State (CallFunction|TBGameState)) self))

(event Custom|Execute%20Ability
  (bind _origin_card (Variables|Default|GetOrigin%20Card))
  (bind _output_get (Variables|Default|SetAbility%20Outcome ""))
  (bind _prefilled_ability_outcome (AbilityOutcome|PrefillAbilityOutcome _output_get))
  (Variables|Default|SetAbility%20Outcome _prefilled_ability_outcome)
  (if (Utilities|IsValid _origin_card)
    (Transformation|AttachActorToActor _origin_card "None" "KeepRelative" "KeepRelative" "KeepRelative" true))
  (Networking|SwitchHasAuthority
    (:Authority
      (Variables|Default|SetStage "NewEnumerator3")
      (CallFunction|SetActiveCardandAbility)
      (CallFunction|PreprocessAbility)
      (CallFunction|ExecuteCommands))))

(event Custom|Request%20Status%20Card
  (bind _origin_card (Variables|Default|GetOrigin%20Card))
  ;[0.5996 0.474 1] Status Card
  (CallFunction|SetActiveCardandAbility)
  (CallFunction|SetStatusStates)
  (if (CallFunction|ActiveAbilityPlayerHasPlayableStatusCard)
    (bind _returnvalue (Game|SpawnActorfromClass "/Game/Blueprints/Commands/ClientCommands/SelectStatusClientCommand.SelectStatusClientCommand_C" (Variables|Default|GetSpawn%20Transform) "Undefined" "MultiplyWithRoot" (Default|Controller(ServerOnly) _origin_card) _origin_card self false true 0))
    (Default|AddCommand (CallFunction|ServerCommandManager) _returnvalue)
    (else
      (Default|SendWarningMessagetoAll (CallFunction|MessageManager) "" (Utilities|Text|ToText(String) (Utilities|String|Append (Utilities|String|EnumtoString (Default|CardRace (Variables|Default|GetOrigin%20Card))) " does not have status for card: " (Default|CardName (Variables|Default|GetOrigin%20Card)))))
      (Utilities|FlowControl|Delay 2.0)
      (CallFunction|AbilityFinished))))

(event Custom|Preprocess%20Ability)

(event Custom|Execute%20Commands
  (Networking|SwitchHasAuthority
    (:Authority
      (Variables|Default|SetStage "NewEnumerator0")
      (bind _server_commands (CallFunction|SpawnAbilityServerCommands))
      (Default|AddCommands (CallFunction|ServerCommandManager) _server_commands)
      (EventDispatchers|AssignCommandFinished (Utilities|Array|Get(acopy) _server_commands (Utilities|Array|LastIndex _server_commands)) (delegate Custom|CommandFinished_Event)))))

(event Custom|Request%20Response%20Card
  ;[1 0.6267 0.6842] Response
  (CallFunction|SetActiveCardandAbility)
  (CallFunction|SetResponseStates)
  (if (CallFunction|EnemyHasPlayableResponseCard)
    (for _array_element (CallFunction|GetAllEnemyTeamControllers (Default|CardRace (Variables|Default|GetOrigin%20Card)))
      (Game|SpawnActorfromClass "/Game/Blueprints/Commands/ClientCommands/SelectResponseClientCommand.SelectResponseClientCommand_C" (Variables|Default|GetSpawn%20Transform) "Undefined" "MultiplyWithRoot" _array_element (Variables|Default|GetOrigin%20Card) 0 false true 0))
    (else
      (Default|SendWarningMessagetoAll (CallFunction|MessageManager) "" (Utilities|Text|ToText(String) (Utilities|String|Append (Utilities|String|EnumtoString (CallFunction|GetEnemyTeamforRace (Default|CardRace (Variables|Default|GetOrigin%20Card)))) " do not have response for card: " (Default|CardName (Variables|Default|GetOrigin%20Card)))))
      (Utilities|FlowControl|Delay 2.0)
      (CallFunction|RequestStatusCard))))

(event Custom|Ability%20Executed
  (bind _postiflled_ability_outcome (AbilityOutcome|PostfillAbilityOutcome (Variables|Default|GetAbility%20Outcome)))
  (Variables|Default|SetAbility%20Outcome _postiflled_ability_outcome)
  (if (Variables|Default|GetTriggerResponse)
    (CallFunction|RequestResponseCard)
    (elif (Variables|Default|GetTriggerStatus)
      (CallFunction|RequestStatusCard)
      (else
        (CallFunction|AbilityFinished)))))

(event Custom|Status%20Card%20Finished
  (params (Card :type BP%20Card%20Object%20Reference) (Controller :type BP%20Turn%20Based%20Player%20Controller%20Object%20Reference))
  ;[0.5996 0.474 1] Status Card
  (AbilityOutcome|AddStatusCardtoOutcome Card)
  (CallFunction|SetActiveCardandAbility)
  (CallFunction|RequestStatusCard))

(event Custom|Set%20Finished%20States
  (bind _tb_game_state (CallFunction|TBGameState))
  (bind _race (CallFunction|OriginCardRace))
  (if (CallFunction|HasOriginCard)
    (Default|SetPlayerTurnStateforAlliesOfRace _tb_game_state _race "NewEnumerator0")
    (Default|SetPlayerTurnStateforRace _tb_game_state _race "NewEnumerator0")
    (Default|SetEnemiesPlayerTurnState _tb_game_state _race "NewEnumerator0")))

(event Custom|Set%20Response%20States
  (bind _tb_game_state (CallFunction|TBGameState))
  (bind _race (CallFunction|OriginCardRace))
  (if (CallFunction|HasOriginCard)
    (Default|SetPlayerTurnStateforAlliesOfRace _tb_game_state _race "NewEnumerator7")
    (Default|SetPlayerTurnStateforRace _tb_game_state _race "NewEnumerator7")
    (Default|SetEnemiesPlayerTurnState _tb_game_state _race "NewEnumerator3")))

(event Custom|Set%20Status%20States
  (bind _tb_game_state (CallFunction|TBGameState))
  (bind _race (CallFunction|OriginCardRace))
  (if (CallFunction|HasOriginCard)
    (Default|SetPlayerTurnStateforAlliesOfRace _tb_game_state _race "NewEnumerator7")
    (Default|SetPlayerTurnStateforRace _tb_game_state _race "NewEnumerator4")
    (Default|SetEnemiesPlayerTurnState _tb_game_state _race "NewEnumerator7")))

(event Custom|Status%20Card%20Played
  (params (Card :type BP%20Card%20Object%20Reference) (Controller :type BP%20Turn%20Based%20Player%20Controller%20Object%20Reference))
  (bind _race (Default|CardRace Card))
  (bind _deck_manager (CallFunction|GetDeckManager _race))
  ;[0.5996 0.474 1] Status Card
  (Variables|Default|SetStage "NewEnumerator2")
  (CallFunction|SetActiveCardandAbility)
  (if (Utilities|Array|ContainsItem (Variables|/Game/Blueprints/Game/BP_TurnBasedPlayerController.BP_TurnBasedPlayerController_C|GetDeck%20Managers Controller) _deck_manager)
    (Default|ActivateCard _deck_manager Card self)
    (else
      (Development|PrintString "Status Played by player who is not that race"))))

(event Custom|Postprocess%20Ability
  (Networking|SwitchHasAuthority
    (:Authority
      (Variables|Default|SetStage "NewEnumerator0"))))

(event Custom|Response%20Card%20Played
  (params (Card :type BP%20Card%20Object%20Reference) (Controller :type BP%20Turn%20Based%20Player%20Controller%20Object%20Reference))
  (bind _race (Default|CardRace Card))
  (bind _deck_manager (CallFunction|GetDeckManager _race))
  ;[1 0.6267 0.6842] Response
  (Variables|Default|SetStage "NewEnumerator1")
  (CallFunction|SetActiveCardandAbility)
  (if (Utilities|Array|ContainsItem (Variables|/Game/Blueprints/Game/BP_TurnBasedPlayerController.BP_TurnBasedPlayerController_C|GetDeck%20Managers Controller) _deck_manager)
    (Default|ActivateCard _deck_manager Card self)
    (else
      (Development|PrintString "Response Played by player who is not that race"))))

(event Custom|Response%20Card%20Finished
  (params (Card :type BP%20Card%20Object%20Reference) (Controller :type BP%20Turn%20Based%20Player%20Controller%20Object%20Reference))
  ;[1 0.6267 0.6842] Response
  (AbilityOutcome|AddResponseCardtoOutcome Card)
  (CallFunction|SetActiveCardandAbility)
  (CallFunction|RequestResponseCard))

(event EventBeginPlay
  (bind _origin_card (Variables|Default|GetOrigin%20Card))
  (if (Utilities|IsValid _origin_card)
    (Variables|Default|SetAbility%20Outcome (Utilities|Struct|MakeAbilityOutcome "NewEnumerator0" (select (Utilities|IsValid _origin_card) (Default|CardRace _origin_card) "NewEnumerator0") "NewEnumerator0" 0 0))))

(fn ConstructionScript)

(fn TBPawn
  (return (.AsBP%20Turn%20Based%20Pawn (Utilities|Casting|CastToBP_TurnBasedPawn (Pawn|GetControlledPawn (CallFunction|GetFirstLocalTBPlayerController))))))

(fn AbilityCommands
  (return 0))

(fn IsTriggeredbyCard
  (return (Utilities|IsValid (Variables|Default|GetOrigin%20Card))))

(fn AreAbilityCommandsFinished
  (bind _array_element (Utilities|Array|ForEachLoopwithBreak (Variables|Default|Get_CommandInstances))
    (:LoopBody
      (LocalVariables|SetfinishedSum (and (LocalVariables|GetfinishedSum) (Variables|/Game/Blueprints/Commands/BP_Command.BP_Command_C|GetFinished _array_element))))
    (:Completed
      (return (LocalVariables|GetfinishedSum)))))

(fn PrefillAbilityOutcome
  (params (Empty%20Ability%20Outcome :type Ability%20Outcome%20Structure))
  (return Empty%20Ability%20Outcome))

(fn PostfillAbilityOutcome
  (params (Ability%20Outcome :type Ability%20Outcome%20Structure))
  (return Ability%20Outcome))

(fn AddResponseCardtoOutcome
  (params (Response%20Card :type BP%20Card%20Object%20Reference%20%28by%20ref%29))
  (bind _output_get (LocalVariables|SetResponse%20Cards%20Local (.responscards (Variables|Default|GetAbility%20Outcome))))
  (Utilities|Array|AddUnique _output_get Response%20Card)
  (bind _structout (Utilities|Struct|SetmembersinAbilityOutcome (Variables|Default|GetAbility%20Outcome) (LocalVariables|GetResponse%20Cards%20Local)))
  (Variables|Default|SetAbility%20Outcome _structout)
  (return (Variables|Default|GetAbility%20Outcome)))

(fn AddStatusCardtoOutcome
  (params (Status%20Card :type BP%20Card%20Object%20Reference%20%28by%20ref%29))
  (bind _output_get (LocalVariables|SetStatus%20Cards%20Local (.statuscards (Variables|Default|GetAbility%20Outcome))))
  (Utilities|Array|AddUnique _output_get Status%20Card)
  (bind _structout (Utilities|Struct|SetmembersinAbilityOutcome (Variables|Default|GetAbility%20Outcome) (LocalVariables|GetStatus%20Cards%20Local)))
  (Variables|Default|SetAbility%20Outcome _structout)
  (return (Variables|Default|GetAbility%20Outcome)))

(fn HasOriginCard
  (return (Utilities|IsValid (Variables|Default|GetOrigin%20Card))))

(fn OriginCardRace
  (if (CallFunction|HasOriginCard)
    (return (Default|CardRace (Variables|Default|GetOrigin%20Card)))
    (else
      (return "NewEnumerator0"))))

(fn SpawnAbilityServerCommands
  (return 0))

(fn InitAbilityOutcome
  (bind _origin_card (Variables|Default|GetOrigin%20Card))
  (bind _returnvalue (Utilities|IsValid _origin_card))
  (if _returnvalue
    (return (Utilities|Struct|MakeAbilityOutcome "NewEnumerator0" (select _returnvalue (Default|CardRace _origin_card) "NewEnumerator0") "NewEnumerator0" 0 0))
    (else
      (return (Utilities|Struct|MakeAbilityOutcome "NewEnumerator0" "NewEnumerator0" "NewEnumerator0" 0 0)))))