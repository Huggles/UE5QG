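; Turn-based ability Blueprint that deploys a Unit to a Country.
; It writes both into the ability outcome and spawns an ordered list of server command actors targeting all player controllers.
; The sequence moves the camera to show the country, deploys the unit as a command owned by the current controller, then returns the camera.
; Camera move durations follow the game state's speed setting.
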(fn ConstructionScript
  (|CallParentFunction))

(fn PostfillAbilityOutcome
  (params (Ability%20Outcome :type Ability%20Outcome%20Structure))
  (bind _structout (Utilities|Struct|SetmembersinAbilityOutcome Ability%20Outcome "NewEnumerator0" "NewEnumerator0" (Variables|Default|GetCountry) (Variables|Default|GetUnit)))
  (return _structout))

(fn SpawnAbilityServerCommands
  (bind _returnvalue (Game|SpawnActorfromClass "/Game/Blueprints/Commands/ServerCommands/MoveCameraCommand.MoveCameraCommand_C" (Variables|Default|GetSpawn%20Transform) "Undefined" "MultiplyWithRoot" 0 (.Time (Default|GameSpeed (.TB%20Game%20State (CallFunction|TBGameState)))) (CallFunction|GetCameraPositiontoShowActor (Variables|Default|GetCountry)) true (CallFunction|GetAllTBPlayerControllers) true 0))
  (bind _returnvalue_2 (Game|SpawnActorfromClass "/Game/Blueprints/Commands/ServerCommands/DeployUnitCommand.DeployUnitCommand_C" (LocalVariables|GetDefault%20Spawn%20Transform%20Local) "Undefined" "MultiplyWithRoot" (LocalVariables|GetCurrent%20Controller%20) (Variables|Default|GetUnit) (Variables|Default|GetCountry) false (CallFunction|GetAllTBPlayerControllers) true 0))
  (bind _returnvalue_3 (Game|SpawnActorfromClass "/Game/Blueprints/Commands/ServerCommands/ReturnCameraCommand.ReturnCameraCommand_C" (Variables|Default|GetSpawn%20Transform) "Undefined" "MultiplyWithRoot" 0 (.Time (Default|GameSpeed (.TB%20Game%20State (CallFunction|TBGameState)))) (CallFunction|GetAllTBPlayerControllers) true 0))
  (return (Utilities|Array|MakeArray _returnvalue _returnvalue_2 _returnvalue_3)))