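; Build-unit ability for the turn-based game that places a unit of a given type and race in a country.
; Preprocessing takes an available unit from the race's faction pool in the game state and announces its addition to the country through the game event manager.
; The outcome records race, country and unit.
; Server commands wrap the build command between camera move and return commands sent to all players.
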(event EventPreprocessAbility
  (bind _unit (Default|GetAvailableUnit (.Value (Utilities|Map|Find (Variables|/Game/Blueprints/Game/BP_TurnBasedGameState.BP_TurnBasedGameState_C|GetUnit%20Pool%20By%20Faction (.TB%20Game%20State (CallFunction|TBGameState))) (Variables|Default|GetRace))) (Variables|Default|GetType)))
  (bind _output_get (Variables|Default|SetUnit _unit))
  (Default|CallAddUnittoCountry (CallFunction|GameEventManager) (Variables|Default|GetCountry) _output_get))

(fn ConstructionScript
  (|CallParentFunction))

(fn PostfillAbilityOutcome
  (params (Ability%20Outcome :type Ability%20Outcome%20Structure))
  (bind _structout (Utilities|Struct|SetmembersinAbilityOutcome Ability%20Outcome "NewEnumerator0" (Variables|Default|GetRace) (Variables|Default|GetCountry) (Variables|Default|GetUnit)))
  (return _structout))

(fn SpawnAbilityServerCommands
  (bind _returnvalue (Game|SpawnActorfromClass "/Game/Blueprints/Commands/ServerCommands/MoveCameraCommand.MoveCameraCommand_C" (Variables|Default|GetSpawn%20Transform) "Undefined" "MultiplyWithRoot" 0 1.0 (CallFunction|GetCameraPositiontoShowActor (Variables|Default|GetCountry)) true (CallFunction|GetAllTBPlayerControllers) true 0))
  (bind _returnvalue_2 (Game|SpawnActorfromClass "/Game/Blueprints/Commands/ServerCommands/BuildUnitCommand.BuildUnitCommand_C" (LocalVariables|GetDefault%20Spawn%20Transform%20Local) "Undefined" "MultiplyWithRoot" (LocalVariables|GetCurrent%20Controller%20) (Variables|Default|GetUnit) (Variables|Default|GetCountry) 0 true 0))
  (bind _returnvalue_3 (Game|SpawnActorfromClass "/Game/Blueprints/Commands/ServerCommands/ReturnCameraCommand.ReturnCameraCommand_C" (Variables|Default|GetSpawn%20Transform) "Undefined" "MultiplyWithRoot" 0 (CallFunction|GetAllTBPlayerControllers) true 0))
  (return (Utilities|Array|MakeArray _returnvalue _returnvalue_2 _returnvalue_3)))