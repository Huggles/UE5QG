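; Card ability that forces a target card, by its name a status card, to be discarded.
; Preprocessing discards the card through the deck manager for that card's race.
; The ability returns a spawned discard command, given all TB player controllers and a faster playback speed, as its only command.
; Outcome post-fill records a tag and the target card's race.
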(event EventPreprocessAbility
  (bind _target_card (Variables|Default|GetTarget%20Card))
  (Default|DiscardCard (CallFunction|GetDeckManager (Default|CardRace _target_card)) _target_card))

(fn ConstructionScript
  (|CallParentFunction))

(fn AbilityCommands
  (bind _returnvalue (Game|SpawnActorfromClass "/Game/Blueprints/Commands/Commands/DiscardCardCommand.DiscardCardCommand_C" (Variables|Default|GetSpawn%20Transform) "Undefined" "MultiplyWithRoot" 0 (Variables|Default|GetTarget%20Card) 2.0 2.0 (CallFunction|GetAllTBPlayerControllers) true (Variables|Default|GetOrigin%20Card) self 0))
  (return (Utilities|Array|MakeArray _returnvalue)))

(fn PostfillAbilityOutcome
  (params (Ability%20Outcome :type Ability%20Outcome%20Structure))
  (Utilities|Struct|SetmembersinAbilityOutcome Ability%20Outcome "NewEnumerator5" (Variables|/Game/Blueprints/Cards/BP_Card.BP_Card_C|GetRace (Variables|Default|GetTarget%20Card)))
  (return ""))