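; Card ability that attacks a Unit with an explosion effect while the camera cuts to it and back.
; Ability Commands returns a move-camera, attack, return-camera sequence; the server variant spawns camera commands per player controller and wraps them in blocking batches around one attack command.
; Prefill Ability Outcome records the unit, its country and its faction.
; PostprocessAbility is empty, leaving the remove-unit-from-country call disconnected.
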(event EventPostprocessAbility)

(fn ConstructionScript
  (|CallParentFunction))

(fn AbilityCommands
  (bind _unit (Variables|Default|GetUnit))
  (bind _returnvalue (Game|SpawnActorfromClass "/Game/Blueprints/Commands/ClientCommands/MoveCameraClientCommand.MoveCameraClientCommand_C" (Variables|Default|GetSpawn%20Transform) "Undefined" "MultiplyWithRoot" 0 1.0 (CallFunction|GetCameraPositiontoShowActor _unit) false true 0))
  (bind _returnvalue_2 (Game|SpawnActorfromClass "/Game/Blueprints/Commands/ServerCommands/AttackUnitCommand.AttackUnitCommand_C" (Variables|Default|GetSpawn%20Transform) "Undefined" "MultiplyWithRoot" 0 _unit 1.0 1.0 "1.000000,1.000000,1.000000" "/Game/StarterContent/Particles/P_Explosion.P_Explosion" true 0))
  (bind _returnvalue_3 (Game|SpawnActorfromClass "/Game/Blueprints/Commands/ClientCommands/ReturnCameraClientCommand.ReturnCameraClientCommand_C" (Variables|Default|GetSpawn%20Transform) "Undefined" "MultiplyWithRoot" 0 false true 0))
  (return (Utilities|Array|MakeArray _returnvalue _returnvalue_2 _returnvalue_3)))

(fn PrefillAbilityOutcome
  (params (Empty%20Ability%20Outcome :type Ability%20Outcome%20Structure))
  (bind _unit (Variables|Default|GetUnit))
  (bind _structout (Utilities|Struct|SetmembersinAbilityOutcome Empty%20Ability%20Outcome "NewEnumerator2" (Variables|/Game/Blueprints/Units/BP_Unit.BP_Unit_C|GetFaction _unit) (Variables|/Game/Blueprints/Units/BP_Unit.BP_Unit_C|GetCountry _unit) _unit))
  (return _structout))

(fn SpawnAbilityServerCommands
  (Utilities|FlowControl|Sequence
    (:then_0
      (for _array_element (CallFunction|GetAllTBPlayerControllers)
        (LocalVariables|SetCurrent%20Controller%20 _array_element)
        (bind _returnvalue (Game|SpawnActorfromClass "/Game/Blueprints/Commands/ClientCommands/MoveCameraClientCommand.MoveCameraClientCommand_C" (LocalVariables|GetDefault%20Spawn%20Transform%20Local) "Undefined" "MultiplyWithRoot" (LocalVariables|GetCurrent%20Controller%20) 3.0 (CallFunction|GetCameraPositiontoShowActor (Variables|Default|GetUnit)) false true 0))
        (Utilities|Array|Add (LocalVariables|GetMoveCamera%20Client%20Commands%20Local) _returnvalue))
      (bind _client_command_batch (Default|MakeBatchforCommands (CallFunction|ServerCommandManager) (LocalVariables|GetMoveCamera%20Client%20Commands%20Local) false true))
      (LocalVariables|SetMoveCameraClientCommandBatch _client_command_batch))
    (:then_1
      (bind _returnvalue_2 (Game|SpawnActorfromClass "/Game/Blueprints/Commands/ServerCommands/AttackUnitCommand.AttackUnitCommand_C" (LocalVariables|GetDefault%20Spawn%20Transform%20Local) "Undefined" "MultiplyWithRoot" 0 (Variables|Default|GetUnit) 1.0 1.0 "1.000000,1.000000,1.000000" "/Game/StarterContent/Particles/P_Explosion.P_Explosion" true 0))
      (LocalVariables|SetDestroyUnitCommand _returnvalue_2))
    (:then_2
      (for _array_element_2 (CallFunction|GetAllTBPlayerControllers)
        (LocalVariables|SetCurrent%20Controller%20 _array_element_2)
        (bind _returnvalue_3 (Game|SpawnActorfromClass "/Game/Blueprints/Commands/ClientCommands/ReturnCameraClientCommand.ReturnCameraClientCommand_C" (LocalVariables|GetDefault%20Spawn%20Transform%20Local) "Undefined" "MultiplyWithRoot" (LocalVariables|GetCurrent%20Controller%20) false true 0))
        (Utilities|Array|Add (LocalVariables|GetReturnCamera%20Client%20Commands%20Local) _returnvalue_3))
      (bind _client_command_batch_2 (Default|MakeBatchforCommands (CallFunction|ServerCommandManager) (LocalVariables|GetReturnCamera%20Client%20Commands%20Local) false true))
      (LocalVariables|SetReturnCameraClientCommandBatch _client_command_batch_2))
    (:then_3
      (return (Utilities|Array|MakeArray (LocalVariables|GetMoveCameraClientCommandBatch) (LocalVariables|GetDestroyUnitCommand) (LocalVariables|GetReturnCameraClientCommandBatch))))))