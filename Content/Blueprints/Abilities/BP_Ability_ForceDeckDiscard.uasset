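; BP_Ability_ForceDeckDiscard is a card ability that forces a target card to be discarded by its deck manager.
; On preprocess it looks up the deck manager for the target card's race and calls DiscardCard on it.
; Its ability commands spawn an actor of this same class with the target card passed in.
; The outcome postfill sets an outcome tag and records that card's race as the target race.
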(event EventPreprocessAbility
  (bind _target_card (Variables|Default|GetTarget%20Card))
  (Default|DiscardCard (CallFunction|GetDeckManager (Default|CardRace _target_card)) _target_card))

(fn ConstructionScript
  (|CallParentFunction))

(fn AbilityCommands
  (Game|SpawnActorfromClass "BP_Ability_ForceDeckDiscard_C" (Variables|Default|GetSpawn%20Transform) "Undefined" "MultiplyWithRoot" 0 (Variables|Default|GetTarget%20Card) 0 true true 0)
  (return (Utilities|Array|MakeArray 0)))

(fn PostfillAbilityOutcome
  (params (Ability%20Outcome :type Ability%20Outcome%20Structure))
  (Utilities|Struct|SetmembersinAbilityOutcome Ability%20Outcome "NewEnumerator5" (Default|CardRace (Variables|Default|GetTarget%20Card)))
  (return ""))