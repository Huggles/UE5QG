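; Command manager that queues command actors and executes them in order, allowing overlap until a blocking command is running.
; Added commands attach to the manager and join a pending list, which moves into the current list one command per run attempt.
; On authority, a finished command notifies its card and ability, fires a finished event, is destroyed, and triggers the next run.
; OnCommandQueueEmpty is an empty event that nothing here calls.
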(event Custom|Add%20Commands
  (params (Commands :type Array%20of%20BP%20Command%20Object%20References))
  (for _array_element Commands
    (CallFunction|AddCommand _array_element)))

(event Custom|Run%20Next%20Command
  (bind _next_command (CallFunction|NextCommand))
  (bind _currentcommands (Variables|Default|GetCurrentCommands))
  (Utilities|FlowControl|Sequence
    (:then_1
      (if (CallFunction|CanPlayNextCommand)
        (bind _returnvalue (Utilities|Array|Add _currentcommands _next_command))
        (Utilities|Array|RemoveItem (Variables|Default|GetPendingCommands) _next_command)
        (Default|ExecuteCommand (Utilities|Array|Get(acopy) _currentcommands _returnvalue))))))

(event Custom|On%20Command%20Queue%20Empty)

(event Custom|Add%20Command
  (params (Command :type BP%20Command%20Object%20Reference%20%28by%20ref%29))
  (Utilities|FlowControl|Sequence
    (:then_1
      (Transformation|AttachActorToActor Command self "None" "KeepRelative" "KeepRelative" "KeepRelative" true)
      (Utilities|Array|Add (Variables|Default|GetPendingCommands) Command)
      (CallFunction|RunNextCommand))))

(event EventCommandFinished
  (params (Command :type BP%20Command%20Object%20Reference))
  (bind _ability (Variables|/Game/Blueprints/Commands/BP_Command.BP_Command_C|GetAbility Command))
  (bind _card (Variables|/Game/Blueprints/Commands/BP_Command.BP_Command_C|GetCard Command))
  (Networking|SwitchHasAuthority
    (:Authority
      (Utilities|FlowControl|Sequence
        (:then_1
          (Utilities|Array|RemoveItem (Variables|Default|GetCurrentCommands) Command)
          (if (Utilities|IsValid _card)
            (Default|CommandFinished _card Command))
          (if (Utilities|IsValid _ability)
            (Default|CommandFinished _ability Command))
          (Default|CallCommandFinishedEvent Command)
          (Actor|DestroyActor Command)
          (if (CallFunction|IsWorking)
            (CallFunction|RunNextCommand)))))))

(fn ConstructionScript)

(fn NextCommand
  (return (Utilities|Array|Get(acopy) (Variables|Default|GetPendingCommands))))

(fn IsPlayingCommand
  (return (> (Utilities|Array|Length (Variables|Default|GetCurrentCommands)) 0)))

(fn HasPendingCommand
  (return (> (Utilities|Array|Length (Variables|Default|GetPendingCommands)) 0)))

(fn IsWorking
  (return (or (CallFunction|IsPlayingCommand) (CallFunction|HasPendingCommand))))

(fn IsPlayingBlockingCommand
  (for _array_element (Variables|Default|GetCurrentCommands)
    (if (Variables|/Game/Blueprints/Commands/BP_Command.BP_Command_C|GetBlocking _array_element)
      (return true)))
  (return false))

(fn CanPlayNextCommand
  (return (and (CallFunction|HasPendingCommand) (or (not (CallFunction|IsPlayingCommand)) (and (CallFunction|IsPlayingCommand) (not (CallFunction|IsPlayingBlockingCommand)))))))