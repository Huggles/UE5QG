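; Client command manager that queues command payloads and plays each as a spawned, attached animation actor.
; Commands start in arrival order, running concurrently unless a current one is marked Blocking; finished actors are destroyed and trigger the next.
; When the queue empties, client and server events relay completion to an all-commands-finished dispatch with the local TB player controller.
; On authority, InitOwner sets the owner to the parent actor.
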(event Custom|Add%20Commands
  (params (Payload :type Array%20of%20Client%20Command%20Payload%20Structures))
  (for _array_element Payload
    (CallFunction|AddCommand _array_element)))

(event Custom|Run%20Next%20Command
  (bind _next_command (CallFunction|NextCommand))
  (if (CallFunction|CanPlayNextCommand)
    (Utilities|Array|Add (Variables|Default|GetCurrentCommands) _next_command)
    (Default|ExecuteCommand _next_command)
    (Utilities|Array|RemoveItem (Variables|Default|GetPendingCommands) _next_command)))

(event Custom|On%20Command%20Queue%20Empty%20%28Server%29
  (params (TB%20Player%20Controller :type BP%20Turn%20Based%20Player%20Controller%20Object%20Reference))
  (Default|CallAllCommandsFinished TB%20Player%20Controller self))

(event Custom|Init%20Owner
  (Networking|SwitchHasAuthority
    (:Authority
      (Actor|SetOwner (Actor|GetParentActor self)))))

(event Custom|On%20Command%20Queue%20Empty%20%28Client%29
  (CallFunction|OnCommandQueueEmpty(Server) (CallFunction|GetFirstLocalTBPlayerController)))

(event Custom|Handle%20Animation%20Finished
  (params (Command :type BP%20Client%20Command%20Object%20Reference)))

(event Custom|Add%20Command
  (params (Payload :type Client%20Command%20Payload%20Structure%20%28by%20ref%29))
  (bind _returnvalue (Game|SpawnActorfromClass (.AnimationClass (Utilities|Struct|BreakClientCommandPayload Payload)) (Math|Transform|MakeTransform "0, 0, 0") "Undefined" "MultiplyWithRoot" (Components|GetOwner) Payload self 0))
  (Transformation|AttachActorToActor _returnvalue self "None" "KeepRelative" "KeepRelative" "KeepRelative" true)
  (Utilities|Array|Add (Variables|Default|GetPendingCommands) _returnvalue)
  (CallFunction|RunNextCommand))

(event EventBeginPlay)

(event EventClientCommandFinished
  (params (Client%20Command :type BP%20Client%20Command%20Object%20Reference))
  (Utilities|Array|RemoveItem (Variables|Default|GetCurrentCommands) Client%20Command)
  (Actor|DestroyActor Client%20Command)
  (if (CallFunction|IsWorking)
    (CallFunction|RunNextCommand)
    (else
      (CallFunction|OnCommandQueueEmpty(Client)))))

(fn ConstructionScript)

(fn NextCommand
  (return (Utilities|Array|Get(acopy) (Variables|Default|GetPendingCommands))))

(fn IsPlayingCommand
  (return (> (Utilities|Array|Length (Variables|Default|GetCurrentCommands)) 0)))

(fn HasPendingCommand
  (return (> (Utilities|Array|Length (Variables|Default|GetPendingCommands)) 0)))

(fn IsWorking
  (return (or (CallFunction|IsPlayingCommand) (CallFunction|HasPendingCommand))))

(fn IsPlayingBlockingCommand
  (for _array_element (Variables|Default|GetCurrentCommands)
    (if (.Blocking (Utilities|Struct|BreakClientCommandPayload (Variables|/Game/Blueprints/Commands/BP_ClientCommand.BP_ClientCommand_C|GetPayload _array_element)))
      (return true)))
  (return false))

(fn CanPlayNextCommand
  (return (and (CallFunction|HasPendingCommand) (or (not (CallFunction|IsPlayingCommand)) (and (CallFunction|IsPlayingCommand) (not (CallFunction|IsPlayingBlockingCommand)))))))