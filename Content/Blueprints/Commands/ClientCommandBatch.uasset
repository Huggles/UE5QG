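; A command that groups several client commands so they start together and finish as one.
; Added commands take the batch as envelope, attach to it and are tracked until spawned on all relevant clients.
; Once all are spawned, and autostart or an execute request allows it, the batch executes them all, with Tick retrying requested starts.
; It registers itself finished when the count of finished commands matches its targets.
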(event Custom|On%20Controller%20Finished%20%28Server%29
  (params (Controller :type BP%20Turn%20Based%20Player%20Controller%20Object%20Reference%20%28by%20ref%29) (Client%20Command :type Client%20Command%20Object%20Reference)))

(event Custom|Batch%20Finished
  (CallFunction|RegisterCommandFinished))

(event EventTick
  (params (DeltaSeconds :type Float%20%28single-precision%29))
  (if (Math|Boolean|ANDBoolean (not (Variables|Default|GetBatch%20Started)) (not (Variables|Default|GetFinished)) (Variables|Default|GetShould%20Start))
    (CallFunction|TryStartBatch)))

(event EventExecuteCommandProtected
  (Variables|Default|SetShould%20Start true))

(fn ConstructionScript)

(fn GetCommandforController
  (params (Owning%20Controller :type Controller%20Object%20Reference))
  (for _array_element (Variables|Default|GetTarget%20Commands)
    (if (== (Default|OwningController _array_element) Owning%20Controller)
      (return 0))))

(fn AddCommand
  (params (Command :type Client%20Command%20Object%20Reference))
  (LocalVariables|SetCurrent%20Command Command)
  (Variables|/Game/Blueprints/Commands/BP_Command.BP_Command_C|SetEnvelope Command self)
  (Utilities|Array|AddUnique (Variables|Default|GetTarget%20Commands) Command)
  (EventDispatchers|BindEventtoCommandFinished Command (EventDispatchers|CreateEvent :!event OnCommandFinished(Server)))
  (Transformation|AttachActorToActor Command self "None" "KeepRelative" "KeepRelative" "KeepRelative" true)
  (if (Default|IsSpawnedonAllRelevantClients Command)
    (Utilities|Array|AddUnique (Variables|Default|GetSpawned%20Commands) Command)
    (CallFunction|TryStartBatch)
    (else
      (bind _asclient_command (Utilities|Casting|CastToClientCommand Command))
      (EventDispatchers|BindEventtoClientCommandSpawnedonClient _asclient_command (EventDispatchers|CreateEvent :!event ClientCommandSpawned)))))

(fn AddCommands
  (params (Commands :type Array%20of%20Client%20Command%20Object%20References))
  (for _array_element Commands
    (CallFunction|AddCommand _array_element)))

(fn ClientCommandSpawned
  (params (Client%20Command :type Client%20Command%20Object%20Reference%20%28by%20ref%29) (Autostarted :type Boolean))
  (Utilities|Array|AddUnique (Variables|Default|GetSpawned%20Commands) Client%20Command)
  (CallFunction|TryStartBatch))

(fn StartCommands
  (Variables|Default|SetBatch%20Started true)
  (for _array_element (Variables|Default|GetTarget%20Commands)
    (Default|ExecuteCommand _array_element)))

(fn AreAllCommandsSpawned?
  (bind _target_commands (Variables|Default|GetTarget%20Commands))
  (for _array_element _target_commands
    (LocalVariables|SetAll%20Marked%20As%20Spawned (and (LocalVariables|GetAll%20Marked%20As%20Spawned) (Default|IsSpawnedonAllRelevantClients _array_element))))
  (return (and (== (Utilities|Array|Length _target_commands) (Utilities|Array|Length (Variables|Default|GetSpawned%20Commands))) (LocalVariables|GetAll%20Marked%20As%20Spawned))))

(fn TryStartBatch
  (if (and (CallFunction|AreAllCommandsSpawned?) (or (Variables|Default|GetAutostart) (Variables|Default|GetShould%20Start)))
    (Default|CallBatchStartedCommands)
    (CallFunction|StartCommands)))

(fn OnCommandFinished(Server)
  (params (Command :type BP%20Command%20Object%20Reference) (Result :type Command%20Result%20Structure))
  (Development|PrintString (Utilities|String|Append "Client Command Finished: " (Utilities|GetDisplayName Command)))
  (bind _asclient_command (Utilities|Casting|CastToClientCommand Command))
  (Utilities|Array|Add (Variables|Default|GetFinished%20Commands) _asclient_command)
  (if (== (Utilities|Array|Length (Variables|Default|GetTarget%20Commands)) (Utilities|Array|Length (Variables|Default|GetFinished%20Commands)))
    (CallFunction|BatchFinished)))