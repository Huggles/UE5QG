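; Card ability Blueprint that forces its target card to be discarded.
; PreprocessAbility discards the target through the deck manager matching that card's race.
; AbilityCommands spawns and returns a DiscardCardCommand actor carrying the target, the ability itself and all TB player controllers, set to double playback speed.
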(event EventPreprocessAbility
  (bind _target_card (Variables|Default|GetTarget%20Card))
  (Default|DiscardCard (CallFunction|GetDeckManager (Default|CardRace _target_card)) _target_card))

(fn ConstructionScript
  (|CallParentFunction))

(fn AbilityCommands
  (bind _returnvalue (Game|SpawnActorfromClass "/Game/Blueprints/Commands/Commands/DiscardCardCommand.DiscardCardCommand_C" (Variables|Default|GetSpawn%20Transform) "Undefined" "MultiplyWithRoot" 0 (Variables|Default|GetTarget%20Card) 2.0 2.0 (CallFunction|GetAllTBPlayerControllers) true self 0 0))
  (return (Utilities|Array|MakeArray _returnvalue)))