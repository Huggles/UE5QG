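; Card ability that builds an army unit of a given type for a country in a turn-based game.
; Preprocessing takes an available unit from the race's unit pool and adds it to the country.
; It then spawns command actors: with Focus on, a camera move to the unit's spawn point, the build and a camera return.
; Without Focus, it returns only a non-blocking build command.
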(event EventPreprocessAbility
  (bind _unit_pool (CallFunction|GetUnitPool (Variables|Default|GetRace)))
  (bind _unit (Default|GetAvailableUnit _unit_pool (Variables|Default|GetType)))
  (bind _output_get (Variables|Default|SetUnit _unit))
  (Default|AddUnittoCountry _output_get (Variables|Default|GetCountry)))

(fn ConstructionScript
  (|CallParentFunction))

(fn AbilityCommands
  (if (Variables|Default|GetFocus)
    (bind _returnvalue (Game|SpawnActorfromClass "/Game/Blueprints/Commands/Commands/MoveCameraCommand.MoveCameraCommand_C" (Variables|Default|GetSpawn%20Transform) "Undefined" "MultiplyWithRoot" 0 1.0 (Transformation|GetWorldLocation (Variables|/Game/Blueprints/Units/BP_Unit.BP_Unit_C|GetSpawn%20Point (Variables|Default|GetUnit))) (CallFunction|GetAllTBPlayerControllers) true (Variables|Default|GetOrigin%20Card) self 0))
    (bind _returnvalue_2 (Game|SpawnActorfromClass "/Game/Blueprints/Commands/Commands/BuildUnitCommand.BuildUnitCommand_C" (Variables|Default|GetSpawn%20Transform) "Undefined" "MultiplyWithRoot" 0 (Variables|Default|GetUnit) 0 true (Variables|Default|GetOrigin%20Card) self 0))
    (bind _returnvalue_3 (Game|SpawnActorfromClass "/Game/Blueprints/Commands/Commands/ReturnCameraCommand.ReturnCameraCommand_C" (Variables|Default|GetSpawn%20Transform) "Undefined" "MultiplyWithRoot" 0 (CallFunction|GetAllTBPlayerControllers) true (Variables|Default|GetOrigin%20Card) self 0))
    (return (Utilities|Array|MakeArray _returnvalue _returnvalue_2 _returnvalue_3))
    (else
      (bind _returnvalue_4 (Game|SpawnActorfromClass "/Game/Blueprints/Commands/Commands/BuildUnitCommand.BuildUnitCommand_C" (Variables|Default|GetSpawn%20Transform) "Undefined" "MultiplyWithRoot" 0 (Variables|Default|GetUnit) 0 false (Variables|Default|GetOrigin%20Card) self 0))
      (return (Utilities|Array|MakeArray _returnvalue_4)))))