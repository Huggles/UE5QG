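; Card ability that eliminates a unit with an explosion, built as a sequence of commands.
; Spawns three command actors: move the camera to the unit's spawn point, destroy the unit with an enlarged explosion effect, then return the camera.
; Each command receives all turn-based player controllers, the origin card and this ability, and the ordered list is returned for execution.
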(fn ConstructionScript
  (|CallParentFunction))

(fn AbilityCommands
  (bind _unit (Variables|Default|GetUnit))
  (bind _returnvalue (Game|SpawnActorfromClass "/Game/Blueprints/Commands/Commands/MoveCameraCommand.MoveCameraCommand_C" (Variables|Default|GetSpawn%20Transform) "Undefined" "MultiplyWithRoot" 0 1.0 (Transformation|GetWorldLocation (Variables|/Game/Blueprints/Units/BP_Unit.BP_Unit_C|GetSpawn%20Point _unit)) (CallFunction|GetAllTBPlayerControllers) true (Variables|Default|GetOrigin%20Card) self 0))
  (bind _returnvalue_2 (Game|SpawnActorfromClass "/Game/Blueprints/Commands/Commands/DestroyUnitCommand.DestroyUnitCommand_C" (Variables|Default|GetSpawn%20Transform) "Undefined" "MultiplyWithRoot" 0 _unit 1.0 1.0 "5.000000,5.000000,5.000000" "/Game/StarterContent/Particles/P_Explosion.P_Explosion" (CallFunction|GetAllTBPlayerControllers) true (Variables|Default|GetOrigin%20Card) self 0))
  (bind _returnvalue_3 (Game|SpawnActorfromClass "/Game/Blueprints/Commands/Commands/ReturnCameraCommand.ReturnCameraCommand_C" (Variables|Default|GetSpawn%20Transform) "Undefined" "MultiplyWithRoot" 0 (CallFunction|GetAllTBPlayerControllers) true (Variables|Default|GetOrigin%20Card) self 0))
  (return (Utilities|Array|MakeArray _returnvalue _returnvalue_2 _returnvalue_3)))