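; Base card ability actor for a turn-based card game, running its commands and follow-up card reactions.
; On execution it attaches to its origin card and, on authority, queues commands from the empty AbilityCommands hook into the CommandManager.
; Once all finish, optional TriggerResponse and TriggerStatus phases let enemies play response cards, then the owner status cards, via spawned selection commands.
; It tracks stage, active card and turn state throughout, finally notifying the origin card.
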(event Custom|Postprocess%20Ability
  (Networking|SwitchHasAuthority
    (:Authority
      (Variables|Default|SetStage "NewEnumerator0"))))

(event Custom|Execute%20Ability
  (bind _origin_card (Variables|Default|GetOrigin%20Card))
  (if (Utilities|IsValid _origin_card)
    (Transformation|AttachActorToActor _origin_card "None" "KeepRelative" "KeepRelative" "KeepRelative" true))
  (Networking|SwitchHasAuthority
    (:Authority
      (Variables|Default|SetStage "NewEnumerator3")
      (CallFunction|SetActiveCardandAbility)
      (CallFunction|PreprocessAbility)
      (CallFunction|ExecuteCommands))))

(event Custom|No%20Status%20Card%20Played
  ;[0.5996 0.474 1] Status Card
  (CallFunction|SetActiveCardandAbility)
  (CallFunction|AbilityFinished))

(event Custom|Ability%20Finished
  (bind _origin_card (Variables|Default|GetOrigin%20Card))
  (Variables|Default|SetStage "NewEnumerator5")
  (CallFunction|SetAbilityPlayerTurnState "NewEnumerator0")
  (Utilities|FlowControl|Sequence
    (:then_0
      (if (Utilities|IsValid _origin_card)
        (Default|AbilityFinished _origin_card self)))
    (:then_1
      (Variables|Default|SetProcessed true))))

(event Custom|No%20Response%20Card%20Played
  ;[1 0.6267 0.6842] Response
  (CallFunction|SetActiveCardandAbility)
  (CallFunction|RequestStatusCard))

(event Custom|Set%20Active%20Card%20And%20Ability
  (Variables|/Game/Blueprints/Game/BP_TurnBasedGameState.BP_TurnBasedGameState_C|SetActive%20Card (CallFunction|TBGameState) (Variables|Default|GetOrigin%20Card))
  (Variables|/Game/Blueprints/Game/BP_TurnBasedGameState.BP_TurnBasedGameState_C|SetActive%20Ability (CallFunction|TBGameState) self))

(event Custom|Request%20Status%20Card
  (bind _origin_card (Variables|Default|GetOrigin%20Card))
  ;[0.5996 0.474 1] Status Card
  (CallFunction|SetActiveCardandAbility)
  (CallFunction|SetAbilityPlayerTurnState "NewEnumerator7")
  (if (CallFunction|ActiveAbilityPlayerHasPlayableStatusCard)
    (bind _returnvalue (Game|SpawnActorfromClass "/Game/Blueprints/Commands/Commands/SelectStatusCommand.SelectStatusCommand_C" (Variables|Default|GetSpawn%20Transform) "Undefined" "MultiplyWithRoot" _origin_card 0 (Utilities|Array|MakeArray (Default|Controller(ServerOnly) (Variables|Default|GetOrigin%20Card))) true _origin_card self 0))
    (Default|AddCommand (CallFunction|CommandManager) _returnvalue)
    (else
      (CallFunction|SendWarningGameNotificationtoAll (Utilities|Text|ToText(String) (Utilities|String|Append (Utilities|String|EnumtoString (Default|CardRace (Variables|Default|GetOrigin%20Card))) " does not have status for card: " (Variables|/Game/Blueprints/Cards/BP_Card.BP_Card_C|GetCard%20Name (Variables|Default|GetOrigin%20Card)))) true)
      (Utilities|FlowControl|Delay 2.0)
      (CallFunction|AbilityFinished))))

(event Custom|Set%20Ability%20Player%20Turn%20State
  (params (Turn%20State :type PlayerTurnStateEnum%20Enum :default "NewEnumerator5"))
  (bind _origin_card (Variables|Default|GetOrigin%20Card))
  (bind _controller (Default|Controller(ServerOnly) _origin_card))
  (if (Utilities|IsValid _origin_card)
    (if (Utilities|IsValid _controller)
      (Variables|/Game/Blueprints/Game/BP_TurnBasedPlayerState.BP_TurnBasedPlayerState_C|SetTurn%20State (Default|TBPlayerState _controller) Turn%20State))))

(event Custom|Request%20Response%20Card
  (bind _origin_card (Variables|Default|GetOrigin%20Card))
  ;[1 0.6267 0.6842] Response
  (CallFunction|SetActiveCardandAbility)
  (CallFunction|SetAbilityPlayerTurnState "NewEnumerator7")
  (if (CallFunction|EnemyHasPlayableResponseCard)
    (bind _returnvalue (Game|SpawnActorfromClass "/Game/Blueprints/Commands/Commands/SelectResponseCommand.SelectResponseCommand_C" (Variables|Default|GetSpawn%20Transform) "Undefined" "MultiplyWithRoot" 0 _origin_card (CallFunction|EnemieswithPlayableResponseCard) true _origin_card self 0))
    (Default|AddCommand (CallFunction|CommandManager) _returnvalue)
    (else
      (CallFunction|SendWarningGameNotificationtoAll (Utilities|Text|ToText(String) (Utilities|String|Append (Utilities|String|EnumtoString (CallFunction|GetEnemyTeamforRace (Default|CardRace (Variables|Default|GetOrigin%20Card)))) " do not have response for card: " (Variables|/Game/Blueprints/Cards/BP_Card.BP_Card_C|GetCard%20Name (Variables|Default|GetOrigin%20Card)))) true)
      (Utilities|FlowControl|Delay 2.0)
      (CallFunction|RequestStatusCard))))

(event Custom|Status%20Card%20Finished
  (params (Card :type BP%20Card%20Object%20Reference) (Controller :type BP%20Turn%20Based%20Player%20Controller%20Object%20Reference))
  ;[0.5996 0.474 1] Status Card
  (CallFunction|SetActiveCardandAbility)
  (CallFunction|RequestStatusCard))

(event Custom|Execute%20Commands
  (Networking|SwitchHasAuthority
    (:Authority
      (Variables|Default|SetStage "NewEnumerator0")
      (bind _output_get (Variables|Default|Set_CommandInstances (CallFunction|AbilityCommands)))
      (for _array_element _output_get
        (Variables|/Game/Blueprints/Commands/BP_Command.BP_Command_C|SetAbility _array_element self))
      (Default|AddCommands (CallFunction|CommandManager) _output_get))))

(event Custom|Command%20Finished
  (params (Command :type BP%20Command%20Object%20Reference))
  (bind __commandinstances (Variables|Default|Get_CommandInstances))
  (if (Utilities|Array|ContainsItem __commandinstances Command)
    (Utilities|Array|RemoveItem __commandinstances Command)
    (Utilities|FlowControl|Sequence
      (:then_0
        (Development|PrintString (Utilities|String|Append "Ability Command Finished" (Utilities|GetDisplayName Command))))
      (:then_1
        (if (Utilities|Array|IsEmpty __commandinstances)
          (Utilities|FlowControl|Delay 1.0)
          (if (Variables|Default|GetTriggerResponse)
            (CallFunction|RequestResponseCard)
            (elif (Variables|Default|GetTriggerStatus)
              (CallFunction|RequestStatusCard)
              (else
                (CallFunction|AbilityFinished)))))))))

(event Custom|Status%20Card%20Played
  (params (Card :type BP%20Card%20Object%20Reference) (Controller :type BP%20Turn%20Based%20Player%20Controller%20Object%20Reference))
  (bind _race (Default|CardRace Card))
  (bind _deck_manager (CallFunction|GetDeckManager _race))
  ;[0.5996 0.474 1] Status Card
  (Variables|Default|SetStage "NewEnumerator2")
  (CallFunction|SetActiveCardandAbility)
  (if (Utilities|Array|ContainsItem (Variables|/Game/Blueprints/Game/BP_TurnBasedPlayerController.BP_TurnBasedPlayerController_C|GetDeck%20Managers Controller) _deck_manager)
    (Default|ActivateStatusCard _deck_manager Card self)
    (else
      (Development|PrintString "Status Played by player who is not that race"))))

(event Custom|Preprocess%20Ability)

(event Custom|Response%20Card%20Played
  (params (Card :type BP%20Card%20Object%20Reference) (Controller :type BP%20Turn%20Based%20Player%20Controller%20Object%20Reference))
  (bind _race (Default|CardRace Card))
  (bind _deck_manager (CallFunction|GetDeckManager _race))
  ;[1 0.6267 0.6842] Response
  (Variables|Default|SetStage "NewEnumerator1")
  (CallFunction|SetActiveCardandAbility)
  (if (Utilities|Array|ContainsItem (Variables|/Game/Blueprints/Game/BP_TurnBasedPlayerController.BP_TurnBasedPlayerController_C|GetDeck%20Managers Controller) _deck_manager)
    (Default|ActivateResponseCard(Server) _deck_manager Card self)
    (else
      (Development|PrintString "Response Played by player who is not that race"))))

(event Custom|Response%20Card%20Finished
  (params (Card :type BP%20Card%20Object%20Reference) (Controller :type BP%20Turn%20Based%20Player%20Controller%20Object%20Reference))
  ;[1 0.6267 0.6842] Response
  (CallFunction|SetActiveCardandAbility)
  (CallFunction|RequestResponseCard))

(event EventBeginPlay)

(fn ConstructionScript)

(fn TBPawn
  (return (.AsBP%20Turn%20Based%20Pawn (Utilities|Casting|CastToBP_TurnBasedPawn (Pawn|GetControlledPawn (CallFunction|GetFirstLocalTBPlayerController))))))

(fn AbilityCommands
  (return 0))

(fn IsTriggeredbyCard
  (return (Utilities|IsValid (Variables|Default|GetOrigin%20Card))))

(fn AreAbilityCommandsFinished
  (bind _array_element (Utilities|Array|ForEachLoopwithBreak (Variables|Default|Get_CommandInstances))
    (:LoopBody
      (LocalVariables|SetfinishedSum (and (LocalVariables|GetfinishedSum) (Variables|/Game/Blueprints/Commands/BP_Command.BP_Command_C|GetIs%20Command%20Finished _array_element))))
    (:Completed
      (return (LocalVariables|GetfinishedSum)))))