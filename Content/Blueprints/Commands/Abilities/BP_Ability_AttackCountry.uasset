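; Card ability that attacks a target country in a turn-based game.
; Its Ability Commands function spawns three command actors in order: move the camera to the country, attack it, then return the camera.
; Each command receives all turn-based player controllers, the origin card and the ability, and the list is returned for execution.
; PostprocessAbility is left empty.
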(event EventPostprocessAbility)

(fn ConstructionScript
  (|CallParentFunction))

(fn AbilityCommands
  (bind _returnvalue (Game|SpawnActorfromClass "/Game/Blueprints/Commands/Commands/MoveCameraCommand.MoveCameraCommand_C" (Variables|Default|GetSpawn%20Transform) "Undefined" "MultiplyWithRoot" 0 1.0 (Transformation|GetWorldLocation (Variables|/Script/Engine.Actor|GetRootComponent (Variables|Default|GetCountry))) (CallFunction|GetAllTBPlayerControllers) true (Variables|Default|GetOrigin%20Card) self 0))
  (bind _returnvalue_2 (Game|SpawnActorfromClass "/Game/Blueprints/Commands/Commands/AttackCountryCommand.AttackCountryCommand_C" (Variables|Default|GetSpawn%20Transform) "Undefined" "MultiplyWithRoot" 0 (Variables|Default|GetCountry) (CallFunction|GetAllTBPlayerControllers) true (Variables|Default|GetOrigin%20Card) self 0))
  (bind _returnvalue_3 (Game|SpawnActorfromClass "/Game/Blueprints/Commands/Commands/ReturnCameraCommand.ReturnCameraCommand_C" (Variables|Default|GetSpawn%20Transform) "Undefined" "MultiplyWithRoot" 0 (CallFunction|GetAllTBPlayerControllers) true (Variables|Default|GetOrigin%20Card) self 0))
  (return (Utilities|Array|MakeArray _returnvalue _returnvalue_2 _returnvalue_3)))