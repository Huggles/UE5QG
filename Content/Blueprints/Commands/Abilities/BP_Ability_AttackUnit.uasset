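; BP_Ability_AttackUnit is an ability command that attacks a unit, removing it from its country in post-processing.
; Its animation list spawns command actors that move all turn-based player controllers' cameras to the unit's spawn point and later return them, with another instance of this ability spawned between.
; Its animation processing event is empty, and an explosion-effect client payload sequence with a destroy-unit step sits unused.
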(event Custom|Process%20Ability%20Animations_1)

(event EventPostprocessAbility
  (Default|RemoveUnitfromCountry (Variables|Default|GetUnit)))

(fn ConstructionScript
  (|CallParentFunction))

(fn AbilityAnimationCommands
  (bind _tb_player_controllers (CallFunction|GetAllTBPlayerControllers))
  (bind _spawn_transform (Variables|Default|GetSpawn%20Transform))
  (bind _unit (Variables|Default|GetUnit))
  (bind _returnvalue (Game|SpawnActorfromClass "/Game/Blueprints/Commands/Commands/MoveCameraCommand.MoveCameraCommand_C" _spawn_transform "Undefined" "MultiplyWithRoot" 0 1.0 (Transformation|GetWorldLocation (Variables|/Game/Blueprints/Units/BP_Unit.BP_Unit_C|GetSpawn%20Point _unit)) _tb_player_controllers true 0 0))
  (Game|SpawnActorfromClass "BP_Ability_AttackUnit_C" _spawn_transform "Undefined" "MultiplyWithRoot" 0 _unit 0 0 0)
  (bind _returnvalue_2 (Game|SpawnActorfromClass "/Game/Blueprints/Commands/Commands/ReturnCameraCommand.ReturnCameraCommand_C" _spawn_transform "Undefined" "MultiplyWithRoot" 0 _tb_player_controllers true 0 0))
  (return (Utilities|Array|MakeArray _returnvalue 0 _returnvalue_2)))