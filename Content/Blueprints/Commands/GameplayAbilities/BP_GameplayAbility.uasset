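; Base gameplay ability actor for a turn-based game, optionally triggered by a card, that runs as a batch of commands.
; On authority, it runs a preprocess hook, then builds commands from AbilityAnimationCommands, an empty stub here.
; It links each command to itself and passes them to the CommandManager.
; As commands report finishing, it checks the batch and notifies its Callback once all are done.
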(event Custom|Postprocess%20Ability
  (Default|AbilityExecutionFinished (Variables|Default|GetCallback) self))

(event Custom|Execute%20Ability
  (Networking|SwitchHasAuthority
    (:Authority
      (CallFunction|PreprocessAbility)
      (CallFunction|ExecuteCommands))))

(event Custom|Execute%20Commands
  (bind _output_get (Variables|Default|Set_CommandInstances (CallFunction|AbilityAnimationCommands)))
  (Development|PrintString (Utilities|String|Append "Executing Commands AS:" (Default|GetDebugString (CallFunction|GetFirstLocalTBPlayerController))))
  (for _array_element _output_get
    (Variables|/Game/Blueprints/Commands/BP_Command.BP_Command_C|SetAbility _array_element self))
  (Default|AddCommands (CallFunction|CommandManager) _output_get))

(event Custom|Handle%20Command%20Finished
  (params (Command :type BP%20Command%20Object%20Reference))
  (Development|PrintString (Utilities|String|Append "Ability Command Finished" (Utilities|GetDisplayName Command)))
  (if (CallFunction|AreAbilityCommandsFinished)
    (Default|AbilityExecutionFinished (Variables|Default|GetCallback) self)))

(event Custom|Preprocess%20Ability)

(event EventBeginPlay)

(fn ConstructionScript)

(fn TBPawn
  (return (.AsBP%20Turn%20Based%20Pawn (Utilities|Casting|CastToBP_TurnBasedPawn (Pawn|GetControlledPawn (CallFunction|GetFirstLocalTBPlayerController))))))

(fn AbilityAnimationCommands
  (return 0))

(fn IsTriggeredbyCard
  (return (Utilities|IsValid (Variables|Default|GetOrigin%20Card))))

(fn AreAbilityCommandsFinished
  (bind _array_element (Utilities|Array|ForEachLoopwithBreak (Variables|Default|Get_CommandInstances))
    (:LoopBody
      (LocalVariables|SetfinishedSum (and (LocalVariables|GetfinishedSum) (Variables|/Game/Blueprints/Commands/BP_Command.BP_Command_C|GetIs%20Command%20Finished _array_element))))
    (:Completed
      (return (LocalVariables|GetfinishedSum)))))