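; Client animation command that plays the destruction of the payload's target unit.
; It attaches a particle effect to the unit's mesh and tweens the unit through a 90-degree rotation over the payload's duration.
; After a cooldown timer, it hides the mesh, resets the rotation, removes the unit from its country and signals that the animation has finished.
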(event Custom|On%20Timer%20Completed
  (bind _target_unit (Utilities|TargetUnit))
  (Rendering|SetVisibility (Variables|/Game/Blueprints/Units/BP_Unit.BP_Unit_C|GetUnitMesh _target_unit) false true)
  (Transformation|SetActorRelativeRotation _target_unit)
  (Default|RemoveUnitfromCountry _target_unit)
  (CallFunction|NotifyAnimationFinished))

(event EventExecuteAnimation
  (bind _target_unit (Utilities|TargetUnit))
  (bind _payload (Variables|Default|GetPayload))
  (bind _returnvalue (Transformation|GetActorRotation _target_unit))
  (Effects|SpawnEmitterAttached (.particlesystem _payload) (Variables|/Game/Blueprints/Units/BP_Unit.BP_Unit_C|GetUnitMesh (Utilities|TargetUnit)) "None" "0, 0, 0" "0, 0, 0" (.scale _payload))
  (bind _value (|TweenRotator _returnvalue (Math|Rotator|CombineRotators _returnvalue "90.000000,0.000000,0.000000") (.duration _payload) "InOutQuad")
    (:ApplyEasing
      (Transformation|SetActorRelativeRotation (Utilities|TargetUnit) _value))
    (:OnComplete
      (Utilities|Time|SetTimerbyEvent (delegate Custom|On%20Timer%20Completed) (+ (.cooldowntime _payload) 0.001)))))

(fn ConstructionScript)