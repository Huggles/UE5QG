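; BP_Command is a base command object that runs an action and reports completion to a Command Manager.
; ExecuteCommand calls ExecuteCommandProtected, an empty event that serves as an override hook, as does OnCommandFinished.
; Each NotifyControllerFinished increments a counter until it reaches the TBControllers count.
; NotifyCommandFinished then flags the command finished, fires OnCommandFinished and passes the command to the manager's CommandFinished.
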(event Custom|Execute%20Command%20Protected)

(event Custom|Execute%20Command
  (CallFunction|ExecuteCommandProtected))

(event Custom|Notify%20Command%20Finished
  (Variables|Default|SetIs%20Command%20Finished true)
  (CallFunction|OnCommandFinished)
  (Default|CommandFinished (CallFunction|CommandManager) self))

(event Custom|Notify%20Controller%20Finished
  (bind _all_controllers_finished (CallFunction|HandleControllerFinished))
  (if _all_controllers_finished
    (CallFunction|NotifyCommandFinished)))

(event Custom|On%20Command%20Finished)

(fn ConstructionScript)

(fn HandleControllerFinished
  (bind _output_get (Variables|Default|SetNumber%20of%20finished%20controllers (+ (Variables|Default|GetNumber%20of%20finished%20controllers) 1)))
  (return (>= _output_get (Utilities|Array|Length (Variables|Default|GetTB%20Controllers)))))

(fn AreAllControllersFinished
  (return (>= (Variables|Default|GetNumber%20of%20finished%20controllers) (Utilities|Array|Length (Variables|Default|GetTB%20Controllers)))))