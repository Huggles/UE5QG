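; BP_DiscardStepManager runs the discard step of the active player's turn on the server.
; ExecuteStep announces the step start and queues a SelectDiscardCardsClientCommand, owned by the active player's controller, offering an optional discard of up to two cards from the active race's hand.
; When that command finishes, it updates the active player's TurnState and fires the discard-step-finished event through the game event manager.
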(event Custom|CommandFinished_Event
  (params (Command :type BP%20Command%20Object%20Reference) (Result :type Command%20Result%20Structure))
  (Development|PrintString "Discard Command Finished")
  (Variables|/Game/Blueprints/Game/BP_TurnBasedPlayerState.BP_TurnBasedPlayerState_C|SetTurn%20State (Default|GetActivePlayerState (Variables|Default|GetGamestate)) "NewEnumerator0")
  (Default|CallDiscardStepFinished (CallFunction|GameEventManager)))

(event EventExecuteStep
  (bind _gamestate (Variables|Default|GetGamestate))
  (Default|CallDiscardStepStarted (CallFunction|GameEventManager))
  (bind _returnvalue (Game|SpawnActorfromClass "/Game/Blueprints/Commands/ClientCommands/SelectDiscardCardsClientCommand.SelectDiscardCardsClientCommand_C" (Variables|Default|GetSpawn%20Transform) "Undefined" "MultiplyWithRoot" (Default|GetActivePlayerController(Server) _gamestate) "Do you want to discard cards?" "DISCARD" "Do Not Select A Card" true (Variables|/Game/Blueprints/Cards/BP_PlayerDeckManager.BP_PlayerDeckManager_C|GetHand (CallFunction|GetDeckManager (Default|GetActiveRace _gamestate))) 2 0 false true 0))
  (Default|AddCommand (CallFunction|ServerCommandManager) _returnvalue)
  (EventDispatchers|AssignCommandFinished _returnvalue (delegate Custom|CommandFinished_Event)))

(fn ConstructionScript)