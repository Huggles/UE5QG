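; BP_DrawStepManager runs the Draw Step of the card game for the active faction, signalling step start, step change and finish through the GameEventManager.
; If the hand is short and the deck yields cards, it queues a ShowCardDrawClientCommand on the ServerCommandManager to show the drawn cards.
; When that command finishes, it refills the hand and ends the step.
; Otherwise it sends a deck-empty check notification and ends immediately.
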(event Custom|Draw%20Step%20Finished
  (Default|CallDrawStepFinished (CallFunction|GameEventManager)))

(event Custom|Command%20Finished%20Event_Event_0
  (params (Command :type BP%20Command%20Object%20Reference) (Result :type Command%20Result%20Structure))
  (Default|RefillHand (CallFunction|GetDeckManager (.Active%20Faction (CallFunction|ActiveFaction))) true)
  (CallFunction|DrawStepFinished))

(event EventExecuteStep
  (bind _active_faction (CallFunction|ActiveFaction))
  (bind (_active_faction_2 _controller) (CallFunction|ActiveFaction))
  (bind _game_event_manager (CallFunction|GameEventManager))
  (bind _deck_manager (CallFunction|GetDeckManager _active_faction))
  (bind _number_of_missing_cards_in_hand (Default|NumberOfMissingCardsinHand _deck_manager))
  (bind (_deck_top_cards _number_of_cards_drawn) (Default|GetDeckTopCards _deck_manager _number_of_missing_cards_in_hand))
  (Default|CallDrawStepStarted _game_event_manager)
  (Default|CallGameStepChanged _game_event_manager self)
  (if (and (> _number_of_missing_cards_in_hand 0) (> _number_of_cards_drawn 0))
    (bind _returnvalue (Game|SpawnActorfromClass "/Game/Blueprints/Commands/ClientCommands/ShowCardDrawClientCommand.ShowCardDrawClientCommand_C" (Variables|Default|GetSpawn%20Transform) "Undefined" "MultiplyWithRoot" _controller _deck_top_cards false true 0))
    (Default|AddCommand (CallFunction|ServerCommandManager) _returnvalue)
    (EventDispatchers|BindEventtoCommandFinished _returnvalue (delegate Custom|Command%20Finished%20Event_Event_0))
    (else
      (Default|NotifyifDeckEmpty (CallFunction|GetDeckManager _active_faction_2))
      (CallFunction|DrawStepFinished))))

(fn ConstructionScript)

(fn StepName
  (return "Draw Step"))