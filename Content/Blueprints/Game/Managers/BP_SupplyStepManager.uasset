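; Supply step manager for a turn-based board game that destroys the active faction's out-of-supply armies and navies.
; ExecuteStep finds unsupplied units, announces each to all players, then queues server commands that move every player's camera to each unit and blow it up.
; A final return-camera command's completion triggers a board state recalculation, after which the step signals finished.
; If every unit is supplied, it finishes immediately.
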(event Custom|CommandFinished_Event
  (params (Command :type BP%20Command%20Object%20Reference) (Result :type Command%20Result%20Structure))
  (bind _gamestate (Variables|Default|GetGamestate))
  (EventDispatchers|AssignBoardStateRecalculated _gamestate (delegate Custom|Board%20State%20Recalculated_Event))
  (Default|RecalculateBoardState _gamestate))

(event Custom|Finish%20Supply%20Step
  (Utilities|Array|Clear (Variables|Default|GetUnsupplied%20Units))
  (Utilities|Array|Clear (Variables|Default|GetAll%20Server%20Commands))
  (Default|CallSupplyStepFinished (CallFunction|GameEventManager)))

(event Custom|Send%20Out%20Of%20Supply%20Notification
  (params (Unit :type BP%20Unit%20Object%20Reference))
  (bind _country (Variables|/Game/Blueprints/Units/BP_Unit.BP_Unit_C|GetCountry Unit))
  (Default|SendPositiveMessagetoAll (CallFunction|MessageManager) "System" (Utilities|Text|ToText(String) (Utilities|String|Append (Utilities|String|EnumtoString (Variables|/Game/Blueprints/Units/BP_Unit.BP_Unit_C|GetFaction Unit)) " " (select (Default|IsLand _country) "Army" "Navy") " is out of supply in " (Utilities|String|ToString(Name) (.label (Variables|/Game/Blueprints/Countries/BP_Country.BP_Country_C|GetCountry%20Data%20Struct _country))) " and will be destroyed."))))

(event Custom|Board%20State%20Recalculated_Event
  (params (New%20Board%20State :type Board%20State%20Structure))
  (EventDispatchers|UnbindEventfromBoardStateRecalculated (Variables|Default|GetGamestate) (delegate Custom|Board%20State%20Recalculated_Event))
  (CallFunction|FinishSupplyStep))

(event EventExecuteStep
  (bind _all_server_commands (Variables|Default|GetAll%20Server%20Commands))
  (Default|CallSupplyStepStarted (CallFunction|GameEventManager))
  (for _array_element (.placedunits (Default|GetFactionState (Variables|Default|GetGamestate) (.Active%20Faction (CallFunction|ActiveFaction))))
    (if (not (Default|IsSupplied _array_element))
      (Utilities|Array|Add (Variables|Default|GetUnsupplied%20Units) _array_element)))
  (if (Utilities|Array|IsNotEmpty (Variables|Default|GetUnsupplied%20Units))
    (for (_array_element_2 _array_index) (Variables|Default|GetUnsupplied%20Units)
      (Utilities|FlowControl|Sequence
        (:then_0
          (CallFunction|SendOutOfSupplyNotification _array_element_2))
        (:then_1
          (bind _array (CallFunction|CreateCommandsforUnit _array_element_2 (== _array_index 0)))
          (Utilities|Array|AppendArray (Variables|Default|GetAll%20Server%20Commands) _array))))
    (bind _returnvalue (Game|SpawnActorfromClass "/Game/Blueprints/Commands/ServerCommands/ReturnCameraCommand.ReturnCameraCommand_C" (Variables|Default|GetSpawn%20Transform) "Undefined" "MultiplyWithRoot" 0 (CallFunction|GetAllTBPlayerControllers) true 0))
    (EventDispatchers|AssignCommandFinished _returnvalue (delegate Custom|CommandFinished_Event))
    (Utilities|Array|Add _all_server_commands _returnvalue)
    (Default|AddCommands (CallFunction|ServerCommandManager) _all_server_commands)
    (else
      (CallFunction|FinishSupplyStep))))

(fn ConstructionScript)

(fn CreateCommandsforUnit
  (params (Unit :type BP%20Unit%20Object%20Reference) (Set%20Return%20Location :type Boolean))
  (LocalVariables|SetCurrent%20Unit Unit)
  (bind _returnvalue (Game|SpawnActorfromClass "/Game/Blueprints/Commands/ServerCommands/MoveCameraCommand.MoveCameraCommand_C" (Variables|Default|GetSpawn%20Transform) "Undefined" "MultiplyWithRoot" 0 1.0 (CallFunction|GetCameraPositiontoShowActor (LocalVariables|GetCurrent%20Unit)) Set%20Return%20Location (CallFunction|GetAllTBPlayerControllers) true 0))
  (bind _returnvalue_2 (Game|SpawnActorfromClass "/Game/Blueprints/Commands/ServerCommands/AttackUnitCommand.AttackUnitCommand_C" (Variables|Default|GetSpawn%20Transform) "Undefined" "MultiplyWithRoot" 0 (LocalVariables|GetCurrent%20Unit) 1.0 1.0 "1.000000,1.000000,1.000000" "/Game/StarterContent/Particles/P_Explosion.P_Explosion" (CallFunction|GetAllTBPlayerControllers) true 0))
  (return (Utilities|Array|MakeArray _returnvalue _returnvalue_2)))