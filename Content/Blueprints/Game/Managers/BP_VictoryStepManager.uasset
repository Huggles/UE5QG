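; BP_VictoryStepManager runs the victory step of a faction's turn, scoring points for the active race.
; ExecuteStep signals the step start, awards the calculated points, waits briefly, then signals completion through the GameEventManager.
; Each occupied supply country is worth more the fewer units it holds, with a guaranteed minimum.
; AddScoreToFaction updates the race's victory points in game state and broadcasts a message naming the active faction.
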(event EventExecuteStep
  (bind _gamestate (Variables|Default|GetGamestate))
  (bind _active_race (Default|GetActiveRace _gamestate))
  (Default|CallVictoryStepStarted (CallFunction|GameEventManager))
  (bind _score_for_race (CallFunction|CalculateTurnPointsforRace _active_race))
  (CallFunction|AddScoretoFaction _active_race _score_for_race "Scoring Phase")
  (Utilities|FlowControl|Delay 3.0)
  (Development|PrintString "Call Victory Step Finished")
  (Default|CallVictoryStepFinished (CallFunction|GameEventManager)))

(fn ConstructionScript)

(fn CalculateTurnPointsforRace
  (params (Playable%20Race :type FactionEnum%20Enum :default "NewEnumerator6"))
  (bind _gamestate (Variables|Default|GetGamestate))
  (if (>= (Variables|/Game/Blueprints/Game/BP_TurnBasedGameState.BP_TurnBasedGameState_C|GetTurnCounter _gamestate) 0)
    (for _array_element (.occupiedsupplycountries (Default|GetFactionState _gamestate Playable%20Race))
      (LocalVariables|SetScoreDelta (+ (LocalVariables|GetScoreDelta) (Math|Integer|Max(Integer) (- 3 (Utilities|Array|Length (Variables|/Game/Blueprints/Countries/BP_Country.BP_Country_C|GetUnits _array_element))) 1))))
    (return (LocalVariables|GetScoreDelta))))

(fn AddScoretoFaction
  (params (Faction :type FactionEnum%20Enum :default "NewEnumerator0") (Points :type Integer) (Reason :type String))
  (bind _gamestate (Variables|Default|GetGamestate))
  (LocalVariables|SetFaction%20Local Faction)
  (LocalVariables|SetPointsLocal Points)
  (LocalVariables|SetReasonLocal Reason)
  (Utilities|Struct|SetmembersinFactionStruct (Utilities|Array|Get(acopy) (Variables|/Game/Blueprints/Game/BP_TurnBasedGameState.BP_TurnBasedGameState_C|GetPlayableRaceStructs _gamestate) (.Index (Default|RaceStructforRace _gamestate (LocalVariables|GetFaction%20Local)))) (+ (.VictoryPoints (Utilities|Struct|BreakFactionStruct (Utilities|Array|Get(acopy) (Variables|/Game/Blueprints/Game/BP_TurnBasedGameState.BP_TurnBasedGameState_C|GetPlayableRaceStructs _gamestate) (.Index (Default|RaceStructforRace _gamestate (LocalVariables|GetFaction%20Local)))))) (LocalVariables|GetPointsLocal)))
  (Default|SendPositiveMessagetoAll (CallFunction|MessageManager) "" (Utilities|Text|ToText(String) (Utilities|String|Append (Utilities|String|EnumtoString (.Active%20Faction (CallFunction|ActiveFaction))) " gained " (Utilities|String|ToString(Integer) (LocalVariables|GetPointsLocal)) " points for " (LocalVariables|GetReasonLocal)))))