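; BP_PlayStepManager runs the play step of a turn-based game, opening the active faction's turn.
; ExecuteStep announces the step through the GameEventManager, then spawns a turn-transition client command per player controller, naming the active faction.
; The ServerCommandManager runs these as an auto-started, blocking batch.
; When the batch finishes, it clears the commands, sets the active player's turn state and notifies that controller its turn has started.
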(event Custom|CommandFinished_Event
  (params (Command :type BP%20Command%20Object%20Reference) (Result :type Command%20Result%20Structure))
  (bind (_active_faction _controller) (CallFunction|ActiveFaction))
  (Utilities|Array|Clear (Variables|Default|GetTurn%20Transition%20Commands))
  (Variables|/Game/Blueprints/Game/BP_TurnBasedPlayerState.BP_TurnBasedPlayerState_C|SetTurn%20State (Default|TBPlayerState _controller) "NewEnumerator1")
  (Default|EvPlayerTurnStarted _controller "NewEnumerator1" _active_faction))

(event EventExecuteStep
  (Default|CallPlayStepStarted (CallFunction|GameEventManager))
  (for _array_element (CallFunction|GetAllTBPlayerControllers)
    (bind _returnvalue (Game|SpawnActorfromClass "/Game/Blueprints/Commands/ClientCommands/ShowTurnTransitionClientCommand.ShowTurnTransitionClientCommand_C" (Variables|Default|GetSpawn%20Transform) "Undefined" "MultiplyWithRoot" _array_element (.Active%20Faction (CallFunction|ActiveFaction)) false false 0))
    (Utilities|Array|Add (Variables|Default|GetTurn%20Transition%20Commands) _returnvalue))
  (bind _client_command_batch (Default|MakeBatchforCommands (CallFunction|ServerCommandManager) (Variables|Default|GetTurn%20Transition%20Commands) true true))
  (EventDispatchers|AssignCommandFinished _client_command_batch (delegate Custom|CommandFinished_Event)))

(fn ConstructionScript)