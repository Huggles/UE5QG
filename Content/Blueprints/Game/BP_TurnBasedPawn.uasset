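; BP_TurnBasedPawn is the turn-based player pawn, tweened to and from targets as a camera move.
; Tween.MovePawn saves the current position, then eases to a fixed offset from the target.
; ReturnPawn eases back to the saved position, which the construction script initializes.
; Both use InOutSine tweens and notify a callback with pawn and controller on completion, while Debug forwards to the player state.
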(event Custom|Return%20Pawn
  (params (DurationSecs :type Float%20%28single-precision%29) (Callback :type I%20Camera%20Movement%20Callback%20Interface))
  (bind _self self)
  (bind _self_2 self)
  (Variables|BP_TurnBasedPawn_C|SetOriginalPosition _self (|Copy (Variables|BP_TurnBasedPawn_C|GetOriginalPosition _self)))
  (bind _value (|TweenVector (Transformation|GetActorLocation _self) (Variables|BP_TurnBasedPawn_C|GetOriginalPosition _self) DurationSecs "InOutSine")
    (:ApplyEasing
      (Transformation|SetActorLocation _self _value false false))
    (:OnComplete
      (Default|CameraMovementFinished Callback _self_2 (.AsBP%20Turn%20Based%20Player%20Controller (Utilities|Casting|CastToBP_TurnBasedPlayerController (Pawn|GetController _self_2)))))))

(event Custom|Move%20Pawn%20%28Tween%29
  (params (Target :type Vector) (DurationSecs :type Float%20%28single-precision%29) (Callback :type I%20Camera%20Movement%20Callback%20Interface))
  (bind _self self)
  (bind _output_get (Variables|BP_TurnBasedPawn_C|SetOriginalPosition _self (Transformation|GetActorLocation _self)))
  (bind _value (|TweenVector _output_get (+ Target "0.000000,700.000000,1000.000000") DurationSecs "InOutSine")
    (:ApplyEasing
      (Transformation|SetActorLocation _self _value false true))
    (:OnComplete
      (Default|CameraMovementFinished Callback self (.AsBP%20Turn%20Based%20Player%20Controller (Utilities|Casting|CastToBP_TurnBasedPlayerController (Pawn|GetController self)))))))

(event Custom|Debug
  (bind _asbp_turn_based_player_state (Utilities|Casting|CastToBP_TurnBasedPlayerState (Variables|GetPlayerState)))
  (Default|DebugPlayerState _asbp_turn_based_player_state))

(event EventBeginPlay)

(fn ConstructionScript
  (Variables|Default|SetOriginalPosition (Transformation|GetActorLocation)))