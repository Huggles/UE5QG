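; Player controller for the game menu and lobby, relaying session and player setup requests to the menu game state.
; A server event starts the QG_Game map through BP_MenuGameState with this controller as host, while LockGameRoom fires the GameRoomLocked dispatcher.
; Player name and race add or remove events forward directly to the game state, and a helper returns the player state cast to BP_MenuPlayerState.
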(event Custom|Lock%20Game%20Room
  (Default|CallGameRoomLocked))

(event Custom|Start%20Game%20Session%20%28Server%29
  (Default|StartGame (.AsBP%20Menu%20Game%20State (Utilities|Casting|CastToBP_MenuGameState (Game|GetGameState))) "QG_Game" self))

(event Custom|Set%20Player%20Name
  (params (Menu%20Player%20Controller :type BP%20Menu%20Player%20Controller%20Object%20Reference) (Player%20Name :type String))
  (Default|SetPlayerName (CallFunction|MenuGameState) Menu%20Player%20Controller Player%20Name))

(event Custom|Add%20Race%20For%20Player
  (params (Menu%20Player%20Controller :type BP%20Menu%20Player%20Controller%20Object%20Reference) (Race :type PlayableRaceEnum%20Enum :default "NewEnumerator0"))
  (Default|AddRaceforPlayer (CallFunction|MenuGameState) Menu%20Player%20Controller Race))

(event Custom|Remove%20Race%20For%20Player
  (params (Menu%20Player%20Controller :type BP%20Menu%20Player%20Controller%20Object%20Reference) (Race :type PlayableRaceEnum%20Enum :default "NewEnumerator0"))
  (Default|RemoveRaceforPlayer (CallFunction|MenuGameState) Menu%20Player%20Controller Race))

(event EventBeginPlay)

(fn ConstructionScript)

(fn MenuPlayerState
  (bind _asbp_menu_player_state (Utilities|Casting|CastToBP_MenuPlayerState (Variables|GetPlayerState)))
  (return _asbp_menu_player_state))