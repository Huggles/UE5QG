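; Menu player state that holds a player's name and chosen races for the game menu.
; RepNotify handlers on both values tell the menu game state that player data changed.
; CopyProperties casts the new state to the turn-based player state but only prints a message, copying nothing.
; InitPlayerDetails is an empty stub, and a Debug function prints the name and races on screen.
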(event EventBeginPlay)

(event EventCopyProperties
  (params (NewPlayerState :type Player%20State%20Object%20Reference))
  (Utilities|Casting|CastToBP_TurnBasedPlayerState NewPlayerState)
  (Development|PrintString "!!Copy Properties!!"))

(fn ConstructionScript)

(fn InitPlayerDetails
  (params (Player%20Index :type Integer)))

(fn Debug
  (bind _linearcolor (Utilities|Struct|MakeLinearColor 255.0 0.0 0.0 1.0))
  (bind _duration_0 (LocalVariables|GetDuration_0))
  (Development|PrintString "Debugging Player State" true true _linearcolor _duration_0)
  (Development|PrintString (Class|KismetStringLibrary|ToUpper (Variables|Default|GetName)) true true _linearcolor _duration_0)
  (for _array_element (Variables|Default|GetPlayer%20Races)
    (Development|PrintString (Class|KismetStringLibrary|ToUpper (Utilities|String|EnumtoString _array_element)) true true _linearcolor _duration_0)))

(fn OnRepName
  (Default|CallMenuPlayerDataChanged (Utilities|MenuGameState)))

(fn OnRepPlayerRaces
  (Default|CallMenuPlayerDataChanged (Utilities|MenuGameState)))