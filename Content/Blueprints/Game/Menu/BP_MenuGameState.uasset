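; Lobby game state for the menu, tracking joined player states, their names and race picks, and the selected game mode.
; Name and race edits write to each player state, then Notify events fire dispatchers; name changes always report index 0.
; RepNotifies on the player list and game mode broadcast join and mode changes.
; StartGame issues a servertravel console command using the map and selected mode; LockSession is an empty loop.
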(event Custom|Lock%20Session
  (for _array_element (Variables|Default|GetMenu%20Player%20States)
    _))

(event Custom|Start%20Game
  (params (MapName :type String) (Host :type BP%20Menu%20Player%20Controller%20Object%20Reference))
  (bind _selected_game_mode (Variables|Default|GetSelected%20Game%20Mode))
  (bind _returnvalue (Utilities|Select :Index _selected_game_mode :NewEnumerator0 "QG_Standard" :NewEnumerator1 "QG_Advanced_Debug"))
  (bind _returnvalue_2 (Utilities|String|Append "servertravel " MapName "?Game=" _returnvalue))
  (Development|PrintString "Starting Game")
  (Development|PrintString _returnvalue_2)
  (Development|ExecuteConsoleCommand _returnvalue_2 Host))

(event Custom|Notify%20Clients%20Race%20Change
  (params (Player%20State :type BP%20Menu%20Player%20State%20Object%20Reference) (Race :type FactionEnum%20Enum :default "NewEnumerator0") (Selected :type Boolean))
  (Default|CallPlayerRaceSelectionChanged Player%20State Race Selected (Utilities|Array|FindItem (Variables|Default|GetMenu%20Player%20States) Player%20State)))

(event Custom|Notify%20Clients%20Name%20Change
  (params (Player%20State :type BP%20Menu%20Player%20State%20Object%20Reference) (Name :type String))
  (Default|CallPlayerNameChanged Player%20State Name))

(event Custom|Notify%20Clients%20Player%20Joined
  (Default|CallPlayerJoined))

(event Custom|Set%20Player%20Name
  (params (Menu%20Player%20Controller :type BP%20Menu%20Player%20Controller%20Object%20Reference) (Player%20Name :type String))
  (bind _menu_player_state (Default|MenuPlayerState Menu%20Player%20Controller))
  (bind _output_get (Variables|/Game/Blueprints/Game/BP_QG_PlayerState.BP_QG_PlayerState_C|SetPlayer%20Name _menu_player_state Player%20Name))
  (CallFunction|NotifyClientsNameChange _menu_player_state _output_get))

(event Custom|Add%20Race%20For%20Player
  (params (Menu%20Player%20Controller :type BP%20Menu%20Player%20Controller%20Object%20Reference) (Race :type FactionEnum%20Enum :default "NewEnumerator0"))
  (bind _menu_player_state (Default|MenuPlayerState Menu%20Player%20Controller))
  (Utilities|Array|AddUnique (Variables|/Game/Blueprints/Game/BP_QG_PlayerState.BP_QG_PlayerState_C|GetPlayer%20Races _menu_player_state) Race)
  (CallFunction|NotifyClientsRaceChange _menu_player_state Race true))

(event Custom|Remove%20Race%20For%20Player
  (params (Menu%20Player%20Controller :type BP%20Menu%20Player%20Controller%20Object%20Reference) (Race :type FactionEnum%20Enum :default "NewEnumerator0"))
  (bind _menu_player_state (Default|MenuPlayerState Menu%20Player%20Controller))
  (Utilities|Array|RemoveItem (Variables|/Game/Blueprints/Game/BP_QG_PlayerState.BP_QG_PlayerState_C|GetPlayer%20Races _menu_player_state) Race)
  (CallFunction|NotifyClientsRaceChange _menu_player_state Race false))

(event EventBeginPlay)

(fn ConstructionScript)

(fn AddPlayerState
  (params (Menu%20Player%20State :type BP%20Menu%20Player%20State%20Object%20Reference))
  (Utilities|Array|Add (Variables|Default|GetMenu%20Player%20States) Menu%20Player%20State)
  (Variables|Default|SetMenu%20Player%20States (Variables|Default|GetMenu%20Player%20States)))

(fn RemovePlayerState
  (params (Menu%20Player%20State :type BP%20Menu%20Player%20State%20Object%20Reference))
  (Utilities|Array|RemoveItem (Variables|Default|GetMenu%20Player%20States) Menu%20Player%20State)
  (Variables|Default|SetMenu%20Player%20States (Variables|Default|GetMenu%20Player%20States)))

(fn OnRepMenuPlayerStates
  (CallFunction|NotifyClientsPlayerJoined (CallFunction|MenuGameState)))

(fn OnRepSelectedGameMode
  (Default|CallSelectedGameModeChanged))