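; Game mode for the menu, registering joining players with the turn-based game state.
; PostLogin passes the new controller's menu player state to AddPlayerState, while the matching removal logic is disconnected from OnLogout.
; Helper functions gather player states and controllers as turn-based types, with optional debug printing.
; InitPlayerState only casts, and the game state getter's cast to BP_MenuGameState is unused.
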(event EventOnLogout
  (params (ExitingController :type Controller%20Object%20Reference)))

(event EventPostLogin
  (params (NewPlayer :type Player%20Controller%20Object%20Reference))
  (Default|AddPlayerState (Utilities|TurnBasedGameState) (.AsBP%20Menu%20Player%20State (Utilities|Casting|CastToBP_MenuPlayerState (Variables|/Script/Engine.Controller|GetPlayerState (.AsBP%20Menu%20Player%20Controller (Utilities|Casting|CastToBP_MenuPlayerController NewPlayer)))))))

(fn ConstructionScript)

(fn InitPlayerState
  (params (Player%20Controller :type BP%20Turn%20Based%20Player%20Controller%20Object%20Reference))
  (for _index (range 0 (- (Class|GameplayStatics|GetNumPlayerStates) 1))
    (Utilities|Casting|CastToBP_TurnBasedPlayerState (Game|GetPlayerState _index))))

(fn GetTBPlayerStates
  (params (Debug :type Boolean))
  (Utilities|Array|Clear (LocalVariables|Get_PlayerStates))
  (for _index (range 0 (- (Class|GameplayStatics|GetNumPlayerStates) 1))
    (Utilities|Array|Add (LocalVariables|Get_PlayerStates) (.AsBP%20Turn%20Based%20Player%20State (Utilities|Casting|CastToBP_TurnBasedPlayerState (Game|GetPlayerState _index))))
    (if Debug
      (Development|PrintString (Utilities|String|Append "Found Player With Player Id: " (Utilities|String|ToString(Integer) (Variables|/Script/Engine.PlayerState|GetPlayerId (.AsBP%20Turn%20Based%20Player%20State (Utilities|Casting|CastToBP_TurnBasedPlayerState (Game|GetPlayerState _index)))))))))
  (return (LocalVariables|Get_PlayerStates)))

(fn GetTBPlayerState
  (params (Player%20Controller :type Player%20Controller%20Object%20Reference))
  (return (.AsBP%20Turn%20Based%20Player%20State (Utilities|Casting|CastToBP_TurnBasedPlayerState (Variables|/Script/Engine.Controller|GetPlayerState (.AsBP%20Turn%20Based%20Player%20Controller (Utilities|Casting|CastToBP_TurnBasedPlayerController Player%20Controller)))))))

(fn GetTBPlayerControllers
  (params (Debug :type Boolean))
  (Utilities|Array|Clear (LocalVariables|Get_PlayerControllers))
  (for _index (range 0 (- (Class|GameplayStatics|GetNumPlayerControllers) 1))
    (Utilities|Array|Add (LocalVariables|Get_PlayerControllers) (.AsBP%20Turn%20Based%20Player%20Controller (Utilities|Casting|CastToBP_TurnBasedPlayerController (Game|GetPlayerController _index))))
    (if Debug
      (Development|PrintString (Utilities|String|Append "Found Controller:" (Utilities|GetDisplayName (.AsBP%20Turn%20Based%20Player%20Controller (Utilities|Casting|CastToBP_TurnBasedPlayerController (Game|GetPlayerController _index))))))))
  (return (LocalVariables|Get_PlayerControllers)))