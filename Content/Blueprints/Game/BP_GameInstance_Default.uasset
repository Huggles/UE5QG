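; Default game instance Blueprint that configures a networking setting at startup and carries a debug test for the game notification system.
; On Init it runs a console command enabling seamless travel in PIE, then prints the variable's value to confirm it.
; A separate debug event waits briefly, then sends a batch of numbered, styled test notifications to the first local TB player controller.
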(event Custom|Debug%20Notification%20System
  (Utilities|FlowControl|Delay 3.0)
  (for _index (range 0 10)
    (Default|ShowGameNotification (CallFunction|GetFirstLocalTBPlayerController) (Utilities|Struct|MakeGameNotificationPayload (Utilities|Text|ToText(String) (Utilities|String|Append (Utilities|String|ToString(Integer) _index) "Test TestTestTestTestTestTestTestTest")) 3.0 3e+01 (Math|Color|MakeColor 255 255 255 255) (Math|Color|MakeColor 0 0 255 255)) false)))

(event EventInit
  (Development|ExecuteConsoleCommand "net.AllowPIESeamlessTravel true" 0)
  (bind _returnvalue (Development|GetConsoleVariableBoolValue "net.AllowPIESeamlessTravel"))
  (Development|PrintString (Utilities|String|ToString(Boolean) _returnvalue)))