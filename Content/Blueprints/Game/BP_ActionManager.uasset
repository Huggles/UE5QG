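; BP_ActionManager is an unfinished manager that tracks gameplay actions in a played list and a pending queue.
; AddAction records the action class in PlayedActions and appends an entry to PendingActions, though that entry's input is not connected.
; ActionFinished removes the front pending entry.
; ExecuteTopPendingAction only checks whether the queue has entries and does not yet execute anything.
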(event Custom|Add%20Action
  (params (Action%20Class :type BP%20CA%20Base%20Object%20Reference))
  (Utilities|FlowControl|Sequence
    (:then_0
      (Utilities|Array|Add (Variables|Default|GetPlayed%20Actions) Action%20Class)
      (Variables|Default|SetPlayed%20Actions (Variables|Default|GetPlayed%20Actions))
      (Utilities|Array|Add (Variables|Default|GetPending%20Actions) 0)
      (Variables|Default|SetPending%20Actions (Variables|Default|GetPending%20Actions)))))

(event Custom|Action%20Finished
  (Utilities|Array|RemoveIndex (Variables|Default|GetPending%20Actions)))

(fn ConstructionScript)

(fn ExecuteTopPendingAction
  (if (> (Utilities|Array|Length (Variables|Default|GetPending%20Actions)) 0)
    _))