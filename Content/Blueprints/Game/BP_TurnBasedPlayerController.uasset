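; Player controller for a turn-based multiplayer strategy game with countries, units, cards and playable races.
; Client country clicks, unit clicks and end-turn requests pass through server events to the game state, which arbitrates selection and turns.
; Turn events update the player state's turn state and the race displayed by the UI.
; It also creates the base HUD, tracks selectable actors, exposes client animation and ability managers, and handles camera pan and zoom.
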(event Custom|Controller%20Init%20%28Client%29
  (CallFunction|ChangeUIState "NewEnumerator0")
  (UI|SetUIDisplayRace (Utilities|Array|Get(acopy) (Variables|/Game/Blueprints/Game/BP_TurnBasedPlayerState.BP_TurnBasedPlayerState_C|GetPlayer%20Races (CallFunction|TBPlayerState))))
  (CallFunction|EvAddInputMapping)
  (if (Pawn|IsLocalController)
    (CallFunction|SetupBaseUI)))

(event Custom|Register%20Controller%20Remotely%20Initialized
  (Default|EvRegisterControllerStartedPlayLocally (.AsBP%20Turn%20Based%20Game%20State (Utilities|Casting|CastToBP_TurnBasedGameState (Game|GetGameState))) self))

(event Custom|Ev%20End%20Turn%20%28Server%29
  ;[1 1 1] End Turn (Server)
  (Default|EvNextPlayerTurn(Server) (Utilities|TBGameState)))

(event Custom|Ev%20End%20Turn%20%28Client%29
  ;[1 1 1] End Turn (Server)
  (CallFunction|ChangeUIState "NewEnumerator0")
  (CallFunction|EvEndTurn(Server)))

(event Custom|Setup%20Base%20UI
  ;[1 1 1] Set UI Client
  (Viewport|RemoveAllWidgets)
  (bind _returnvalue (UserInterface|CreateWidget "/Game/Blueprints/UI/UIB_GameInterface_Base.UIB_GameInterface_Base_C"))
  (UserInterface|Viewport|AddtoViewport _returnvalue 0)
  (Variables|Default|SetUserInterfaceWidget _returnvalue))

(event Custom|Debug
  (bind _asbp_turn_based_player_state (Utilities|Casting|CastToBP_TurnBasedPlayerState (Variables|GetPlayerState self)))
  (Default|DebugPlayerState _asbp_turn_based_player_state))

(event Custom|Register%20Card%20Spawned
  (params (Remote :type Boolean))
  ;[1 1 1] Remote Spawn Notification
  (Default|CardSpawned (CallFunction|TBGameState) Remote))

(event Custom|Ev%20Turn%20Has%20Ended
  ;[1 1 1] End Turn (Server)
  (CallFunction|ChangeUIState "NewEnumerator0"))

(event Custom|Ev%20Set%20Local%20Race
  (params (Playable%20Race :type PlayableRaceEnum%20Enum :default "NewEnumerator6"))
  (UI|SetUIDisplayRace Playable%20Race))

(event Custom|Register%20Unit%20Spawned
  (params (Remote :type Boolean))
  ;[1 1 1] Remote Spawn Notification
  (Default|UnitSpawned (CallFunction|TBGameState) Remote))

(event Custom|Ev%20Player%20Turn%20Started
  (params (Turn%20State :type PlayerTurnStateEnum%20Enum :default "NewEnumerator5") (Race :type PlayableRaceEnum%20Enum :default "NewEnumerator6"))
  (Development|PrintString (Utilities|String|Append "Turn Started" (Utilities|String|EnumtoString Race)))
  (CallFunction|ChangeUIState Turn%20State)
  (CallFunction|EvSetLocalRace Race))

(event Custom|Change%20UI%20State
  (params (Turn%20State :type PlayerTurnStateEnum%20Enum :default "NewEnumerator5"))
  (Variables|/Game/Blueprints/Game/BP_TurnBasedPlayerState.BP_TurnBasedPlayerState_C|SetTurn%20State (CallFunction|TBPlayerState) Turn%20State))

(event EventBeginPlay
  (Networking|SwitchHasAuthority
    (:Remote
      (CallFunction|RegisterControllerRemotelyInitialized))))

(event Custom|On%20Clicked%20Unit%20%28Client%29
  (params (Unit :type BP%20Unit%20Object%20Reference))
  (CallFunction|OnClickedUnit(Server) Unit))

(event Custom|On%20Clicked%20Country%20%28Server%29
  (params (Country :type BP%20Country%20Object%20Reference))
  (Default|CountrySelected (CallFunction|TBGameState) Country self))

(event Custom|On%20Clicked%20Country%20%28Client%29
  (params (Country :type BP%20Country%20Object%20Reference))
  (CallFunction|OnClickedCountry(Server) Country))

(event Custom|On%20Clicked%20Unit%20%28Server%29
  (params (Unit :type BP%20Unit%20Object%20Reference))
  (Default|UnitSelected (CallFunction|TBGameState) Unit self))

(event Custom|Ev%20Add%20Input%20Mapping
  ;[1 1 1] Input
  (Input|AddMappingContext (PlayerController|LocalPlayerSubsystems|GetEnhancedInputLocalPlayerSubsystem self) "/Game/Input/IMC_Camera.IMC_Camera" 0 (Utilities|Struct|MakeModifyContextOptions true false false)))

(event Custom|Spawn%20Unit%20TEST%20Multicast)

(event Custom|Spawn%20Unit%20TEST)

(event Input|EnhancedActionEvents|EnhancedInputActionIA_Move
  (params (ActionValue :type Vector%202D%20Structure) (ElapsedSeconds :type Float%20%28double-precision%29) (TriggeredSeconds :type Float%20%28double-precision%29) (InputAction :type Input%20Action%20Object%20Reference :default "/Game/Input/IA_Move.IA_Move"))
  ;[1 1 1] Input
  (Transformation|AddActorWorldOffset (Utilities|MyPosessedPawn) (* (Math|Conversions|ToVector(Vector2D) ActionValue) (Variables|Default|GetCameraMovementSpeed))))

(event Input|EnhancedActionEvents|EnhancedInputActionIA_Interact
  (params (ActionValue :type Boolean) (ElapsedSeconds :type Float%20%28double-precision%29) (TriggeredSeconds :type Float%20%28double-precision%29) (InputAction :type Input%20Action%20Object%20Reference :default "/Game/Input/IA_Interact.IA_Interact"))
  ;[1 1 1] Input
)

(event Custom|Show%20Cards
  (params (Card%20Type :type CardTypeEnum%20Enum :default "NewEnumerator0")))

(fn ConstructionScript)

(fn HandleZoom
  (params (Input :type Float%20%28double-precision%29))
  (bind __originalzoom (Variables|Default|Get_originalZoom))
  (bind _maxzoom (Variables|Default|GetMaxZoom))
  (LocalVariables|SetpawnCamera (Variables|/Game/Blueprints/Game/BP_TurnBasedPawn.BP_TurnBasedPawn_C|GetPawnCamera (Utilities|MyPosessedPawn)))
  (LocalVariables|SetoriginalZoom (Transformation|GetActorLocation (Utilities|MyPosessedPawn)))
  (Transformation|AddActorWorldOffset (Utilities|MyPosessedPawn) (* (Math|Vector|GetForwardVector (LocalVariables|GetpawnCamera)) (* Input (Variables|Default|GetCameraZoomSpeed))))
  (Transformation|SetActorLocation (Utilities|MyPosessedPawn) (Math|Vector|MakeVector (.x __originalzoom) (.y __originalzoom) (Math|Float|Clamp(Float) (.Z (Math|Vector|BreakVector (Transformation|GetActorLocation))) (.x _maxzoom) (.y _maxzoom))) false false))

(fn RegisterCountryEvents)

(fn GetPlayerStateIndex
  (return (Utilities|Array|FindItem (Variables|/Script/Engine.GameStateBase|GetPlayerArray (Game|GetGameState)) (Variables|GetPlayerState))))

(fn GetSelectableActors
  (return (Default|RelevantCountries (Variables|/Game/Blueprints/Game/BP_TurnBasedGameState.BP_TurnBasedGameState_C|GetActive%20Card (CallFunction|TBGameState)))))

(fn IsActorSelectable
  (params (Actor%20Class :type Actor%20Object%20Reference))
  (Utilities|FlowControl|Sequence
    (:then_0
      (bind _returnvalue (Class|CommonBlueprintHelpers|GetParentClasses (Utilities|GetClass Actor%20Class)))
      (for _array_element 0
        (LocalVariables|Set_IsActorSelectable (or (Utilities|Array|ContainsItem _returnvalue _array_element) (LocalVariables|Get_IsActorSelectable)))))
    (:then_1
      (for _array_element_2 0
        (LocalVariables|Set_IsActorSelectable (or (Utilities|Array|ContainsItem (Variables|/Script/Engine.Actor|GetTags Actor%20Class) _array_element_2) (LocalVariables|Get_IsActorSelectable)))))
    (:then_2
      (LocalVariables|Set_IsActorSelectable (or (Utilities|Array|ContainsItem (Variables|Selection|GetSelectableActorObjects) Actor%20Class) (LocalVariables|Get_IsActorSelectable))))
    (:then_3
      (return (LocalVariables|Get_IsActorSelectable)))))

(fn SetUIDisplayRace
  (params (Playable%20Race :type PlayableRaceEnum%20Enum :default "NewEnumerator6"))
  (bind _output_get (Variables|Default|Set_UISelectedRace Playable%20Race))
  (Default|CallLocalRaceSelected _output_get (Default|GetRaceStructStructforRace (CallFunction|TBGameState) _output_get) (CallFunction|GetDeckManager _output_get)))

(fn GetUIDisplayRace
  (return (Variables|Default|Get_UISelectedRace)))

(fn AddSelectableActorObject
  (params (Selectable%20Actor :type Actor%20Object%20Reference))
  (Utilities|Array|Add (Variables|Selection|GetSelectableActorObjects) Selectable%20Actor)
  (return))

(fn AddSelectableActorObjects
  (params (Selectable%20Actors :type Array%20of%20Actor%20Object%20References))
  (for _array_element Selectable%20Actors
    (Utilities|Array|Add (Variables|Selection|GetSelectableActorObjects) _array_element))
  (return))

(fn RemoveSelectableActorObject
  (params (Selectable%20Actor :type Actor%20Object%20Reference))
  (Utilities|Array|RemoveItem (Variables|Selection|GetSelectableActorObjects) Selectable%20Actor)
  (return))

(fn RemoveAllSelectableActorObjects
  (Utilities|Array|Clear (Variables|Selection|GetSelectableActorObjects))
  (return))

(fn RemoveAllSelectables
  (Selection|RemoveAllSelectableActorObjects)
  (return))

(fn TBPlayerState
  (bind _asbp_turn_based_player_state (Utilities|Casting|CastToBP_TurnBasedPlayerState (Variables|GetPlayerState)))
  (return _asbp_turn_based_player_state))

(fn GetClientAnimationManager
  (return (.AsBP%20Client%20Animation%20Manager (Utilities|Casting|CastToBP_Client_Animation_Manager (Variables|/Script/Engine.ChildActorComponent|GetChildActor (Variables|Default|GetClient%20Animation%20Manager))))))

(fn GetGameplayAbilityManager
  (return (.AsBP%20Client%20GA%20Manager (Utilities|Casting|CastToBP_Client_GA_Manager (Variables|/Script/Engine.ChildActorComponent|GetChildActor (Variables|Default|GetClient%20Gameplay%20Ability%20Manager))))))

(fn GetDebugString
  (return (Default|DebugString (.AsBP%20Turn%20Based%20Player%20State (Utilities|Casting|CastToBP_TurnBasedPlayerState (Variables|GetPlayerState self))))))