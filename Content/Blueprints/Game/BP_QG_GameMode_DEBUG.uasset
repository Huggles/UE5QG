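; Debug game mode for a turn-based Axis versus Allies game that starts a match with preset players.
; Once players spawn locally, it sets up race structs, then names the first two player states and gives each three races.
; It then constructs a ComplexGameSetup_DEBUG object and passes it to the turn-based game state to set up the match.
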(event EventHandleStartingNewPlayer
  (params (NewPlayer :type Player%20Controller%20Object%20Reference))
  (|CallParentFunction NewPlayer))

(event EventHandlePlayersLocallySpawned
  (bind _tb_game_state (CallFunction|TBGameState))
  (CallFunction|SetupRaceStructs)
  (CallFunction|SetupDebugPlayers)
  (bind _returnvalue (Game|ConstructObjectfromClass "/Game/Blueprints/Game/GameSetups/ComplexGameSetup_DEBUG.ComplexGameSetup_DEBUG_C" _tb_game_state))
  (Default|SetupGameState _tb_game_state _returnvalue))

(fn ConstructionScript
  (|CallParentFunction))

(fn SetupDebugPlayer
  (params (Player%20Number :type Integer) (New%20Player%20State :type BP%20Turn%20Based%20Player%20State%20Object%20Reference))
  (LocalVariables|SetLocal%20Player%20State New%20Player%20State)
  (switch int Player%20Number
    (:0
      (Variables|/Game/Blueprints/Game/BP_TurnBasedPlayerState.BP_TurnBasedPlayerState_C|SetPlayer%20Name (LocalVariables|GetLocal%20Player%20State) "Player 1 (Axis)")
      (Utilities|Array|Add (Variables|/Game/Blueprints/Game/BP_TurnBasedPlayerState.BP_TurnBasedPlayerState_C|GetPlayer%20Races (LocalVariables|GetLocal%20Player%20State)) "NewEnumerator0")
      (Utilities|Array|Add (Variables|/Game/Blueprints/Game/BP_TurnBasedPlayerState.BP_TurnBasedPlayerState_C|GetPlayer%20Races (LocalVariables|GetLocal%20Player%20State)) "NewEnumerator2")
      (Utilities|Array|Add (Variables|/Game/Blueprints/Game/BP_TurnBasedPlayerState.BP_TurnBasedPlayerState_C|GetPlayer%20Races (LocalVariables|GetLocal%20Player%20State)) "NewEnumerator1"))
    (:1
      (Variables|/Game/Blueprints/Game/BP_TurnBasedPlayerState.BP_TurnBasedPlayerState_C|SetPlayer%20Name (LocalVariables|GetLocal%20Player%20State) "Player 2 (Allies)")
      (Utilities|Array|Add (Variables|/Game/Blueprints/Game/BP_TurnBasedPlayerState.BP_TurnBasedPlayerState_C|GetPlayer%20Races (LocalVariables|GetLocal%20Player%20State)) "NewEnumerator3")
      (Utilities|Array|Add (Variables|/Game/Blueprints/Game/BP_TurnBasedPlayerState.BP_TurnBasedPlayerState_C|GetPlayer%20Races (LocalVariables|GetLocal%20Player%20State)) "NewEnumerator4")
      (Utilities|Array|Add (Variables|/Game/Blueprints/Game/BP_TurnBasedPlayerState.BP_TurnBasedPlayerState_C|GetPlayer%20Races (LocalVariables|GetLocal%20Player%20State)) "NewEnumerator5")))
  (return (LocalVariables|GetLocal%20Player%20State)))

(fn SetupDebugPlayers
  (for (_array_element _array_index) (Variables|/Script/Engine.GameStateBase|GetPlayerArray (.TB%20Game%20State (CallFunction|TBGameState)))
    (bind _asbp_turn_based_player_state (Utilities|Casting|CastToBP_TurnBasedPlayerState _array_element))
    (CallFunction|SetupDebugPlayer _array_index _asbp_turn_based_player_state)))