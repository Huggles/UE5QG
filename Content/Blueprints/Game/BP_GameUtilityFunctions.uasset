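; BP_GameUtilityFunctions is a set of shared lookup helpers for a turn-based game with countries and cards.
; It casts to the turn-based game state to expose the active player controller, and resolves the client's controller and player state from player index 0.
; Card drop and display widgets are found by class search, returned only when exactly one exists; the drop lookup also prints the count.
; GetAdjacentCountries is an empty stub.
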(fn GetTurnBasedGameState
  (bind _asbp_turn_based_game_state (Utilities|Casting|CastToBP_TurnBasedGameState (Game|GetGameState (LocalVariables|Get__WorldContext))))
  (return _asbp_turn_based_game_state))

(fn GetActivePlayerController
  (bind _turn_based_game_state (GameState|GetTurnBasedGameState (LocalVariables|Get__WorldContext)))
  (bind _turn_based_player_controller (Default|GetActivePlayerController _turn_based_game_state))
  (return _turn_based_player_controller))

(fn GetPlayerController(Client)
  (return (.AsBP%20Turn%20Based%20Player%20Controller (Utilities|Casting|CastToBP_TurnBasedPlayerController (Game|GetPlayerController (LocalVariables|Get__WorldContext))))))

(fn GetPlayerState(Client)
  (return (Utilities|GetTBPlayerStateforController (.AsBP%20Turn%20Based%20Player%20Controller (Utilities|Casting|CastToBP_TurnBasedPlayerController (Game|GetPlayerController (LocalVariables|Get__WorldContext)))))))

(fn GetAdjacentCountries
  (params (Country :type BP%20Country%20Object%20Reference) (TB%20Player%20State :type Player%20State%20Object%20Reference)))

(fn GetCardsDrop(Client)
  (params (__WorldContext :type Object%20Object%20Reference))
  (bind _foundwidgets (Widget|GetAllWidgetsOfClass __WorldContext "/Game/Blueprints/UI/UIB_CardDrop.UIB_CardDrop_C" false))
  (Development|PrintString __WorldContext (Utilities|String|ToString(Integer) (Utilities|Array|Length _foundwidgets)))
  (if (== (Utilities|Array|Length _foundwidgets) 1)
    (return (Utilities|Array|Get(acopy) _foundwidgets))))

(fn GetCardsDisplay(Client)
  (bind _foundwidgets (Widget|GetAllWidgetsOfClass (LocalVariables|Get__WorldContext) "/Game/Blueprints/UI/UIB_CardsDisplay.UIB_CardsDisplay_C" false))
  (if (== (Utilities|Array|Length _foundwidgets) 1)
    (return (Utilities|Array|Get(acopy) _foundwidgets))))