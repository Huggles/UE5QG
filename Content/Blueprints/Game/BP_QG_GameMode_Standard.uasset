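; Standard game mode for a turn-based game, which prepares the match once players are spawned locally.
; HandlePlayersLocallySpawned sets up race structs and players, then constructs a DefaultGameSetup object and passes it to the turn-based game state's SetupGameState.
; SetupPlayers is a stub that only casts each PlayerArray entry to BP_TurnBasedPlayerState.
; New-player handling defers to the parent, and the construction script prints a debug string.
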(event Custom|Setup%20Players
  (for _array_element (Variables|/Script/Engine.GameStateBase|GetPlayerArray (CallFunction|TBGameState))
    (Utilities|Casting|CastToBP_TurnBasedPlayerState _array_element)))

(event EventHandlePlayersLocallySpawned
  (bind _tb_game_state (CallFunction|TBGameState))
  (CallFunction|SetupRaceStructs)
  (CallFunction|SetupPlayers)
  (bind _returnvalue (Game|ConstructObjectfromClass "/Game/Blueprints/Game/GameSetups/DefaultGameSetup.DefaultGameSetup_C" _tb_game_state))
  (Default|SetupGameState _tb_game_state _returnvalue))

(event EventHandleStartingNewPlayer
  (params (NewPlayer :type Player%20Controller%20Object%20Reference))
  (|CallParentFunction NewPlayer))

(fn ConstructionScript
  (|CallParentFunction)
  (Development|PrintString "Game Mode Standard Constructed"))