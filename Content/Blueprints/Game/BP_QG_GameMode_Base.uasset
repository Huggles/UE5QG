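; Base game mode for a turn-based multiplayer game that holds back match start and tracks when every player has the framework actors spawned locally.
; Binds to each joining controller's local-spawn events, counting controllers, player states, game states and worlds.
; When all counts match for two or more players, it fires an empty HandlePlayersLocallySpawned hook.
; Also builds faction structs from data assets into the game state and signals game start at InProgress.
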(event Custom|Controller%20Spawned%20Locally_Event
  (params (Controller :type BP%20Turn%20Based%20Player%20Controller%20Object%20Reference))
  (Development|PrintString (Utilities|GetDisplayName Controller))
  (Utilities|Array|AddUnique (Variables|Default|GetLocally%20Initialized%20Controllers%20) Controller)
  (if (CallFunction|AreFrameworkActorsLocallyLoaded)
    (CallFunction|HandlePlayersLocallySpawned)))

(event Custom|Player%20State%20Spawned%20Locally_Event
  (params (Controller :type BP%20Turn%20Based%20Player%20Controller%20Object%20Reference) (PlayerState :type BP%20Turn%20Based%20Player%20State%20Object%20Reference))
  (bind _locally_initialized_player_states (Variables|Default|GetLocally%20Initialized%20Player%20States))
  (Development|PrintString (Utilities|GetDisplayName PlayerState))
  (Utilities|Map|Add _locally_initialized_player_states Controller (+ (.Value (Utilities|Map|Find _locally_initialized_player_states Controller)) 1))
  (if (CallFunction|AreFrameworkActorsLocallyLoaded)
    (CallFunction|HandlePlayersLocallySpawned)))

(event Custom|Game%20State%20Spawned%20Locally_Event
  (params (GameState :type BP%20Turn%20Based%20Game%20State%20Object%20Reference) (Controller :type BP%20Turn%20Based%20Player%20Controller%20Object%20Reference))
  (Development|PrintString (Utilities|GetDisplayName GameState))
  (Variables|Default|SetLocally%20Initialized%20Game%20States (+ (Variables|Default|GetLocally%20Initialized%20Game%20States) 1))
  (if (CallFunction|AreFrameworkActorsLocallyLoaded)
    (CallFunction|HandlePlayersLocallySpawned)))

(event Custom|Handle%20Players%20Locally%20Spawned)

(event Custom|World%20Spawned%20Locally_Event_0
  (params (World :type BP%20World%20Object%20Reference) (Controller :type Controller%20Object%20Reference))
  (Variables|Default|SetLocally%20Initialized%20%20Worlds (+ (Variables|Default|GetLocally%20Initialized%20%20Worlds) 1))
  (if (CallFunction|AreFrameworkActorsLocallyLoaded)
    (CallFunction|HandlePlayersLocallySpawned)))

(event EventHandleStartingNewPlayer
  (params (NewPlayer :type Player%20Controller%20Object%20Reference))
  (bind _asbp_turn_based_player_controller (Utilities|Casting|CastToBP_TurnBasedPlayerController NewPlayer))
  (Utilities|Array|AddUnique (Variables|Default|GetControllers) _asbp_turn_based_player_controller)
  (Utilities|Map|Add (Variables|Default|GetLocally%20Initialized%20Player%20States) _asbp_turn_based_player_controller 0)
  (Utilities|FlowControl|Sequence
    (:then_0
      (EventDispatchers|AssignControllerSpawnedLocally _asbp_turn_based_player_controller (delegate Custom|Controller%20Spawned%20Locally_Event))
      (EventDispatchers|AssignPlayerStateSpawnedLocally _asbp_turn_based_player_controller (delegate Custom|Player%20State%20Spawned%20Locally_Event))
      (EventDispatchers|AssignGameStateSpawnedLocally _asbp_turn_based_player_controller (delegate Custom|Game%20State%20Spawned%20Locally_Event))
      (EventDispatchers|AssignWorldSpawnedLocally _asbp_turn_based_player_controller (delegate Custom|World%20Spawned%20Locally_Event_0)))
    (:then_1
      (bind _asbp_turn_based_player_state (Utilities|Casting|CastToBP_TurnBasedPlayerState (Variables|/Script/Engine.Controller|GetPlayerState _asbp_turn_based_player_controller)))
      (Default|AddPlayerState (.TB%20Game%20State (CallFunction|TBGameState)) _asbp_turn_based_player_state))))

(event EventOnSetMatchState
  (params (NewState :type Name :default "None"))
  (switch name NewState
    (:InProgress
      (Default|CallGameStarted))))

(fn ConstructionScript)

(fn ReadytoStartMatch
  (return false))

(fn ValidatePlayersJoined
  (bind _tb_game_state (CallFunction|TBGameState))
  (bind _playerarray (Variables|/Script/Engine.GameStateBase|GetPlayerArray _tb_game_state))
  (if (>= (Utilities|Array|Length _playerarray) 0)
    (for _array_element _playerarray
      (Utilities|Casting|CastToBP_TurnBasedPlayerState _array_element
        (:CastFailed
          (return false))))
    (return true)))

(fn SetupRaceStructs
  (bind _enumvalue (|ForEachFactionEnum)
    (:LoopBody
      (bind _returnvalue (Actor|GetActorOfClass (Variables|/Game/DataAssets/PDA_Faction.PDA_Faction_C|GetHomeSpace (.Value (Utilities|Map|Find (Variables|Default|GetDataAssets) _enumvalue)))))
      (Utilities|Array|Add (Variables|/Game/Blueprints/Game/BP_TurnBasedGameState.BP_TurnBasedGameState_C|GetPlayableRaceStructs (.TB%20Game%20State (CallFunction|TBGameState))) (Utilities|Struct|MakeFactionStruct (Default|GetRaceName (.Value (Utilities|Map|Find (Variables|Default|GetDataAssets) _enumvalue))) (Variables|/Game/DataAssets/PDA_Faction.PDA_Faction_C|GetRace (.Value (Utilities|Map|Find (Variables|Default|GetDataAssets) _enumvalue))) (Variables|/Game/DataAssets/PDA_Faction.PDA_Faction_C|GetTeam (.Value (Utilities|Map|Find (Variables|Default|GetDataAssets) _enumvalue))) (Variables|/Game/DataAssets/PDA_Faction.PDA_Faction_C|GetColor (.Value (Utilities|Map|Find (Variables|Default|GetDataAssets) _enumvalue))) (Variables|/Game/DataAssets/PDA_Faction.PDA_Faction_C|GetText%20Color%20Light (.Value (Utilities|Map|Find (Variables|Default|GetDataAssets) _enumvalue))) (Variables|/Game/DataAssets/PDA_Faction.PDA_Faction_C|GetText%20Color%20Dark (.Value (Utilities|Map|Find (Variables|Default|GetDataAssets) _enumvalue))) _returnvalue 0 0 (Variables|/Game/DataAssets/PDA_Faction.PDA_Faction_C|GetFlag (.Value (Utilities|Map|Find (Variables|Default|GetDataAssets) _enumvalue))))))
    (:then
      (return))))

(fn AreFrameworkActorsLocallyLoaded
  (bind _controllers (Variables|Default|GetControllers))
  (bind _returnvalue (Utilities|Array|Length _controllers))
  (return (Math|Boolean|ANDBoolean (CallFunction|ArePlayerStateActorsLocallyLoaded) (== (Utilities|Array|Length (Variables|Default|GetLocally%20Initialized%20Controllers%20)) _returnvalue) (== _returnvalue (Variables|Default|GetLocally%20Initialized%20Game%20States)) (> _returnvalue 1) (== _returnvalue (Variables|Default|GetLocally%20Initialized%20%20Worlds)))))

(fn ArePlayerStateActorsLocallyLoaded
  (bind _locally_initialized_player_states (Variables|Default|GetLocally%20Initialized%20Player%20States))
  (bind _keys (Utilities|Map|Keys _locally_initialized_player_states))
  (for _array_element _keys
    (LocalVariables|SetAll%20Loaded (and (LocalVariables|GetAll%20Loaded) (== (.Value (Utilities|Map|Find _locally_initialized_player_states _array_element)) (Utilities|Array|Length (Variables|Default|GetControllers))))))
  (return (LocalVariables|GetAll%20Loaded)))