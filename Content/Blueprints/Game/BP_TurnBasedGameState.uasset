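; Game state for a turn-based, six-nation WWII card-and-unit game, handling match setup, turn flow and victory points.
; Setup spawns unit pools and decks, waits for replication to all clients, then deals hands, places units (including debug extras) and starts turn zero.
; TurnCounter modulo six selects the active race; each turn end scores its units on supply spaces.
; Helpers map races to player states and controllers, and commands go to the CommandManager.
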(event Custom|Progress%20Turn
  (CallFunction|EndTurn (Variables|Default|GetTurnCounter))
  (bind _output_get (Variables|Default|SetTurnCounter (+ (Variables|Default|GetTurnCounter) 1)))
  (CallFunction|StartTurn _output_get))

(event Custom|DEBUG%20Add%20Units
  (bind _bp_world (CallFunction|BPWorld))
  (bind _ability_factory (CallFunction|AbilityFactory))
  (bind _countrymap (Variables|/Game/Blueprints/Countries/BP_World.BP_World_C|GetCountryMap _bp_world))
  (Default|BuildUnit(Ability) _ability_factory 0 (.Value (Utilities|Map|Find _countrymap "/Game/Blueprints/Countries/BP_EasternEurope.BP_EasternEurope_C")) "NewEnumerator0" "NewEnumerator0" false false false)
  (Default|BuildUnit(Ability) _ability_factory 0 (.Value (Utilities|Map|Find _countrymap "/Game/Blueprints/Countries/BP_Ukraine.BP_Ukraine_C")) "NewEnumerator4" "NewEnumerator0" false false false)
  (Default|BuildUnit(Ability) _ability_factory 0 (.Value (Utilities|Map|Find _countrymap "/Game/Blueprints/Countries/BP_Russia.BP_Russia_C")) "NewEnumerator4" "NewEnumerator0" false false false)
  (Default|BuildUnit(Ability) _ability_factory 0 (.Value (Utilities|Map|Find _countrymap "/Game/Blueprints/Countries/BP_WesternEurope.BP_WesternEurope_C")) "NewEnumerator4" "NewEnumerator0" false false false))

(event Custom|DEBUG%20Add%20debug%20cards
  (params (Deck%20Manager :type BP%20Player%20Deck%20Manager%20Object%20Reference))
  (bind _deck (Variables|/Game/Blueprints/Cards/BP_PlayerDeckManager.BP_PlayerDeckManager_C|GetDeck Deck%20Manager))
  (switch Utilities|FlowControl|Switch|SwitchonPlayableRaceEnum (Variables|/Game/Blueprints/Cards/BP_PlayerDeckManager.BP_PlayerDeckManager_C|GetPlayable%20Race Deck%20Manager)
    (:NewEnumerator0
      (bind _bp_card (Default|GetCardbyClass Deck%20Manager "/Game/Blueprints/Cards/Germany/BP_Status_Blitzkrieg.BP_Status_Blitzkrieg_C"))
      (Utilities|Array|Add (Variables|/Game/Blueprints/Cards/BP_PlayerDeckManager.BP_PlayerDeckManager_C|GetStatusCards Deck%20Manager) _bp_card)
      (Utilities|Array|RemoveItem _deck _bp_card))
    (:NewEnumerator3
      (bind _bp_card_2 (Default|GetCardbyClass Deck%20Manager "/Game/Blueprints/Cards/UnitedKingdom/BP_Response_BreakingTheEnigmaCode.BP_Response_BreakingTheEnigmaCode_C"))
      (Utilities|Array|Add (Variables|/Game/Blueprints/Cards/BP_PlayerDeckManager.BP_PlayerDeckManager_C|GetResponseCards Deck%20Manager) _bp_card_2)
      (Utilities|Array|RemoveItem _deck _bp_card_2))))

(event Custom|Place%20Starting%20Units
  (for _array_element (Variables|Default|GetPlayableRaceStructs)
    (Default|SetHomeSpaceforPlayer (.homespace _array_element) (.race _array_element))
    (Default|BuildUnit(Ability) (CallFunction|AbilityFactory) 0 (.homespace _array_element) (.race _array_element) "NewEnumerator0" false false false))
  (CallFunction|DEBUGAddUnits))

(event Custom|Execute%20Scoring%20Phase
  (bind _active_race (Game|GetActiveRace))
  (bind _score_for_race (CallFunction|CalculateTurnPointsforRace _active_race))
  (CallFunction|AddScoretoRace _active_race _score_for_race "Scoring Phase"))

(event Custom|Start%20Turn
  (params (Turn :type Integer))
  (Variables|/Game/Blueprints/Game/BP_TurnBasedPlayerState.BP_TurnBasedPlayerState_C|SetTurn%20State (PlayerState|GetActivePlayerState) "NewEnumerator1")
  (CallFunction|SendPositiveGameNotificationtoAll (Utilities|Text|ToText(String) (Utilities|String|Append (Variables|/Game/Blueprints/Game/BP_TurnBasedPlayerState.BP_TurnBasedPlayerState_C|GetPlayer%20Name (PlayerState|GetActivePlayerState)) "'s turn ( " (Utilities|String|EnumtoString (Game|GetActiveRace)) " )")) true)
  (Default|EvPlayerTurnStarted (PlayerState|GetActivePlayerController(Server)) "NewEnumerator1" (Game|GetActiveRace)))

(event Custom|Setup%20Game
  (CallFunction|InitStartingUnits)
  (CallFunction|InitDecks))

(event Custom|Init%20Decks
  (bind _outactors (Actor|GetAllActorsOfClass "/Game/Blueprints/Cards/BP_PlayerDeckManager.BP_PlayerDeckManager_C"))
  (bind _output_get (Variables|Default|SetCard%20Decks _outactors))
  (for _array_element _output_get
    (Default|InstantiateDeck _array_element (PlayerState|GetPlayerControllerforRace(Server) (Variables|/Game/Blueprints/Cards/BP_PlayerDeckManager.BP_PlayerDeckManager_C|GetPlayable%20Race _array_element)))))

(event Custom|Setup%20Player%20Game%20Parts
  (CallFunction|DrawStartingHandCards)
  (CallFunction|PlaceStartingUnits))

(event Custom|Draw%20Starting%20Hand%20Cards
  (for _array_element (CallFunction|GetAllDeckManagers)
    (CallFunction|DEBUGAddDebugCards _array_element)
    (Default|DrawCards(Server) _array_element 5)))

(event Custom|Unit%20Pool%20Spawned%20For%20All%20Clients
  (params (Unit%20Pool :type BP%20Unit%20Pool%20Object%20Reference))
  (if (and (CallFunction|AreAllUnitPoolsCompletelySpawned) (CallFunction|AreAllCardDecksCompletelySpawned))
    (CallFunction|SetupPlayerGameParts)
    (Class|GameMode|StartMatch (Utilities|TBGameMode))
    (Default|CallMatchStarted)
    (for _array_element (CallFunction|GetAllTBPlayerControllers)
      (Default|SetupBaseUI _array_element))
    (Utilities|FlowControl|Delay 5.0)
    (CallFunction|StartTurn)))

(event Custom|Card%20Deck%20Spawned%20For%20All%20Clients
  (params (Deck%20Manager :type BP%20Player%20Deck%20Manager%20Object%20Reference))
  (if (and (CallFunction|AreAllUnitPoolsCompletelySpawned) (CallFunction|AreAllCardDecksCompletelySpawned))
    (CallFunction|SetupPlayerGameParts)
    (Class|GameMode|StartMatch (Utilities|TBGameMode))
    (Default|CallMatchStarted)
    (for _array_element (CallFunction|GetAllTBPlayerControllers)
      (Default|SetupBaseUI _array_element))
    (Utilities|FlowControl|Delay 5.0)
    (CallFunction|StartTurn)))

(event Custom|Add%20Score%20To%20Race
  (params (Race :type PlayableRaceEnum%20Enum :default "NewEnumerator0") (Points :type Integer) (Reason :type String))
  (bind _index (CallFunction|RaceStructforRace Race))
  (bind _playableracestructs (Variables|Default|GetPlayableRaceStructs))
  (bind _output (Utilities|Array|Get(acopy) _playableracestructs _index))
  (Utilities|Struct|SetmembersinPlayableRaceStruct _output (+ (.VictoryPoints (Utilities|Struct|BreakPlayableRaceStruct _output)) Points))
  (CallFunction|SendPositiveGameNotificationtoAll (Utilities|Text|ToText(String) (Utilities|String|Append (Utilities|String|EnumtoString (Game|GetActiveRace)) " gained " (Utilities|String|ToString(Integer) Points) " points for " Reason)) true))

(event Custom|Init%20Starting%20Units
  (bind _outactors (Actor|GetAllActorsOfClass "/Game/Blueprints/Units/BP_UnitPool.BP_UnitPool_C"))
  (bind _output_get (Variables|Default|SetUnit%20Pools _outactors))
  (for _array_element _output_get
    (Default|InstantiateUnits _array_element)))

(event Custom|End%20Turn
  (params (Turn :type Integer))
  (CallFunction|ExecuteScoringPhase)
  (Variables|/Game/Blueprints/Game/BP_TurnBasedPlayerState.BP_TurnBasedPlayerState_C|SetTurn%20State (PlayerState|GetActivePlayerState) "NewEnumerator0"))

(event Custom|Cancel%20All%20Request%20Effective%20Card%20%28Server%29
  (for _array_element (CallFunction|GetAllTBPlayerControllers)
    (Default|CancelRequestEffectiveCard(Client) _array_element)))

(event Custom|Execute%20Commands%20%28Server%29
  (params (Commands :type Array%20of%20BP%20Command%20Object%20References))
  (Default|AddCommands (CallFunction|CommandManager) Commands))

(event Custom|Execute%20Command
  (params (Command :type BP%20Command%20Object%20Reference))
  (CallFunction|ExecuteCommands(Server) (Utilities|Array|MakeArray Command)))

(event Custom|Show%20Cards
  (params (Race :type PlayableRaceEnum%20Enum :default "NewEnumerator6") (Card%20Type :type CardTypeEnum%20Enum :default "NewEnumerator0")))

(event Custom|Player%20Skips%20Ability
  (params (Controller :type BP%20Turn%20Based%20Player%20Controller%20Object%20Reference) (Ability :type BP%20Ability%20Object%20Reference)))

(fn ConstructionScript)

(fn OnRepTurnBasedPlayerStates
  (Default|CallPlayerStatesChanged))

(fn GetPlayerStateforRace
  (params (Player%20Race :type PlayableRaceEnum%20Enum :default "NewEnumerator6"))
  (for _array_element (Variables|GameplayInstanceReferences|GetTurn%20Based%20Player%20States)
    (if (Utilities|Array|ContainsItem (Variables|/Game/Blueprints/Game/BP_TurnBasedPlayerState.BP_TurnBasedPlayerState_C|GetPlayer%20Races _array_element) Player%20Race)
      (return _array_element))))

(fn GetPlayerControllerforRace(Server)
  (params (Player%20Race :type PlayableRaceEnum%20Enum :default "NewEnumerator6"))
  (return (.AsBP%20Turn%20Based%20Player%20Controller (Utilities|Casting|CastToBP_TurnBasedPlayerController (Game|GetPlayerController (PlayerState|GetPlayerStateforRace Player%20Race))))))

(fn GetActivePlayerState
  (return (PlayerState|GetPlayerStateforRace (Game|GetActiveRace))))

(fn GetActivePlayerController(Server)
  (return (PlayerState|GetPlayerControllerforRace(Server) (Game|GetActiveRace))))

(fn AddPlayerState
  (params (Player%20State :type BP%20Turn%20Based%20Player%20State%20Object%20Reference))
  (Utilities|Array|Add (Variables|GameplayInstanceReferences|GetTurn%20Based%20Player%20States) Player%20State)
  (Variables|GameplayInstanceReferences|SetTurn%20Based%20Player%20States (Variables|GameplayInstanceReferences|GetTurn%20Based%20Player%20States)))

(fn GetRaceStructStructforRace
  (params (Playable%20Race :type PlayableRaceEnum%20Enum :default "NewEnumerator6"))
  (for _array_element (Variables|Default|GetPlayableRaceStructs)
    (if (Utilities|Enum|Equal(Enum) (.Race (Utilities|Struct|BreakPlayableRaceStruct _array_element)) Playable%20Race)
      (return _array_element)))
  (return ""))

(fn RemovePlayerState
  (params (Player%20State :type BP%20Turn%20Based%20Player%20State%20Object%20Reference))
  (Utilities|Array|RemoveItem (Variables|GameplayInstanceReferences|GetTurn%20Based%20Player%20States) Player%20State)
  (Variables|GameplayInstanceReferences|SetTurn%20Based%20Player%20States (Variables|GameplayInstanceReferences|GetTurn%20Based%20Player%20States)))

(fn GetActiveRace
  (return (Utilities|Select :Index (Utilities|ActiveRaceCounter) :Option%200 "NewEnumerator0" :Option%201 "NewEnumerator3" :Option%202 "NewEnumerator2" :Option%203 "NewEnumerator4" :Option%204 "NewEnumerator1" :Option%205 "NewEnumerator5")))

(fn NumOfRemoteControllers
  (return (Utilities|Array|Length (Variables|GameplayInstanceReferences|GetRemote%20Controllers))))

(fn RaceStructforRace
  (params (Race :type PlayableRaceEnum%20Enum :default "NewEnumerator6"))
  (for (_array_element _array_index) (Variables|Default|GetPlayableRaceStructs)
    (if (Utilities|Enum|Equal(Enum) (.Race (Utilities|Struct|BreakPlayableRaceStruct _array_element)) Race)
      (return _array_element _array_index)))
  (return "" 0))

(fn GetTeamScoreforTeam
  (params (Team :type TeamEnum%20Enum :default "NewEnumerator0"))
  (LocalVariables|SetTeamScoreLocal 0)
  (for _array_element (CallFunction|GetRacesinTeam Team)
    (LocalVariables|SetTeamScoreLocal (+ (LocalVariables|GetTeamScoreLocal) (.victorypoints (PlayerState|GetRaceStructStructforRace _array_element)))))
  (return (LocalVariables|GetTeamScoreLocal)))

(fn CalculateTurnPointsforRace
  (params (Playable%20Race :type PlayableRaceEnum%20Enum :default "NewEnumerator6"))
  (if (>= (Variables|Default|GetTurnCounter) 0)
    (for _array_element (Default|GetAllPlacedUnitsforRace (CallFunction|BPWorld) Playable%20Race)
      (if (Variables|/Game/Blueprints/Countries/BP_Country.BP_Country_C|GetIsSupply (Variables|/Game/Blueprints/Units/BP_Unit.BP_Unit_C|GetCountry _array_element))
        (LocalVariables|SetScoreDelta (+ (LocalVariables|GetScoreDelta) (Math|Integer|Max(Integer) (- 3 (Utilities|Array|Length (Default|GetUnitsinCountry (Variables|/Game/Blueprints/Units/BP_Unit.BP_Unit_C|GetCountry _array_element)))) 1)))))
    (return (LocalVariables|GetScoreDelta))))

(fn GetGameRoundandTurnNumber
  (bind _turncounter (Variables|Default|GetTurnCounter))
  (return (Math|Float|Ceil (/ (Math|Conversions|ToFloat(Integer) (+ _turncounter 1)) 6.0)) _turncounter))

(fn AreAllUnitPoolsCompletelySpawned
  (for _array_element (Variables|Default|GetUnit%20Pools)
    (bind _output_get (LocalVariables|SetComplete (and (LocalVariables|GetComplete) (Default|AllUnitsSpawnedonAllClients _array_element)))))
  (return (LocalVariables|GetComplete)))

(fn AreAllCardDecksCompletelySpawned
  (for _array_element (Variables|Default|GetCard%20Decks)
    (LocalVariables|SetComplete (and (LocalVariables|GetComplete) (Default|AllCardsSpawnedonAllClients _array_element))))
  (return (LocalVariables|GetComplete)))

(fn SetPlayerTurnStateforRace
  (params (Race :type PlayableRaceEnum%20Enum :default "NewEnumerator0") (Turn%20State :type PlayerTurnStateEnum%20Enum :default "NewEnumerator5"))
  (bind _controller (CallFunction|GetControllerforRace(ServerOnly) Race))
  (if (Utilities|IsValid _controller)
    (Variables|/Game/Blueprints/Game/BP_TurnBasedPlayerState.BP_TurnBasedPlayerState_C|SetTurn%20State (Default|TBPlayerState _controller) Turn%20State)))

(fn SetPlayerTurnStateforAlliesOfRace
  (params (Race :type PlayableRaceEnum%20Enum :default "NewEnumerator0") (Turn%20State :type PlayerTurnStateEnum%20Enum :default "NewEnumerator5"))
  (for _array_element (CallFunction|GetAlliesforRace Race)
    (Variables|/Game/Blueprints/Game/BP_TurnBasedPlayerState.BP_TurnBasedPlayerState_C|SetTurn%20State (Default|TBPlayerState (CallFunction|GetControllerforRace(ServerOnly) _array_element)) Turn%20State)))

(fn SetEnemiesPlayerTurnState
  (params (Playable%20Race :type PlayableRaceEnum%20Enum :default "NewEnumerator0") (Turn%20State :type PlayerTurnStateEnum%20Enum :default "NewEnumerator5"))
  (for _array_element (CallFunction|GetRacesinTeam (CallFunction|GetEnemyTeamforRace Playable%20Race))
    (Variables|/Game/Blueprints/Game/BP_TurnBasedPlayerState.BP_TurnBasedPlayerState_C|SetTurn%20State (Default|TBPlayerState (CallFunction|GetControllerforRace(ServerOnly) _array_element)) Turn%20State)))