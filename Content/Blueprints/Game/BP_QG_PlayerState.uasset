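; BP_QG_PlayerState is a player state Blueprint that adds debug output for identifying players across network roles.
; Debug String builds a label from an authority or remote tag and the player name, and Debug Player State prints it.
; BeginPlay and the construction script are empty, and the TB Game State graph holds only an unused cast to BP_TurnBasedGameState.
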(event EventBeginPlay)

(fn ConstructionScript)

(fn DebugPlayerState
  (Development|PrintString (CallFunction|DebugString)))

(fn DebugString
  (return (Utilities|String|Append (Utilities|String|SelectString "(Authority)" "(Remote)" (Ability|HasAuthority)) "Player State:" (Variables|Default|GetPlayer%20Name))))