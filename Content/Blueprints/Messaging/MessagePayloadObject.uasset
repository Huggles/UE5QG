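; MessagePayloadObject is a messaging payload that formats a message as display text from its DateTime, Sender and Text values.
; MessageWithSender joins the timestamp, the bracketed sender name, a colon and the message body.
; MessageWithoutSender joins only the timestamp, a colon and the body.
; HasSender reports whether the Sender string is non-empty.
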(fn MessagewithSender
  (return (Utilities|Text|ToText(String) (Utilities|String|Append (Utilities|String|ToString(Text) (Class|KismetTextLibrary|AsTimeDateTime (Variables|Default|GetDateTime))) " " (Utilities|String|Append "[" (Variables|Default|GetSender) "]") ": " (Utilities|String|ToString(Text) (Variables|Default|GetText))))))

(fn MessageWithoutSender
  (return (Utilities|Text|ToText(String) (Utilities|String|Append (Utilities|String|ToString(Text) (Class|KismetTextLibrary|AsTimeDateTime (Variables|Default|GetDateTime))) ": " (Utilities|String|ToString(Text) (Variables|Default|GetText))))))

(fn HasSender
  (return (not (Utilities|Array|IsEmpty (Variables|Default|GetSender)))))