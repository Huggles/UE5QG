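; BP_CardUtilities is a utility Blueprint that supplies card artwork for the six WWII factions in a card game.
; CardFrontTexture switches on faction, then selects a texture by card type, while CardBackTexture selects one back per faction.
; Some combinations return Unknown_Card, and Italy and US economic warfare cards reuse their Status textures.
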(fn CardFrontTexture
  (params (Faction :type PlayableRaceEnum%20Enum :default "NewEnumerator0") (Card%20Type :type CardTypeEnum%20Enum :default "NewEnumerator0"))
  (LocalVariables|SetType Card%20Type)
  (switch Utilities|FlowControl|Switch|SwitchonPlayableRaceEnum Faction
    (:NewEnumerator0
      (return (Utilities|Select :Index (LocalVariables|GetType) :NewEnumerator0 "/Game/Sprites/Textures/Cards/Germany/Germany_BuildArmy.Germany_BuildArmy" :NewEnumerator6 "/Game/Sprites/Textures/Cards/Germany/Germany_BuildNavy.Germany_BuildNavy" :NewEnumerator1 "/Game/Sprites/Textures/Cards/Germany/Germany_LandBattle.Germany_LandBattle" :NewEnumerator7 "/Game/Sprites/Textures/Cards/Germany/Germany_SeaBattle.Germany_SeaBattle" :NewEnumerator2 "/Game/Sprites/Textures/Cards/Germany/Germany_Event.Germany_Event" :NewEnumerator3 "/Game/Sprites/Textures/Cards/Germany/Germany_Status.Germany_Status" :NewEnumerator4 "/Game/Sprites/Textures/Cards/Unknown_Card.Unknown_Card" :NewEnumerator5 "/Game/Sprites/Textures/Cards/Germany/Germany_EconomicWarfare.Germany_EconomicWarfare")))
    (:NewEnumerator3
      (return (Utilities|Select :Index (LocalVariables|GetType) :NewEnumerator0 "/Game/Sprites/Textures/Cards/UnitedKingdom/UKBuildArmy.UKBuildArmy" :NewEnumerator6 "/Game/Sprites/Textures/Cards/UnitedKingdom/UKBuildNavy.UKBuildNavy" :NewEnumerator1 "/Game/Sprites/Textures/Cards/UnitedKingdom/UKLandBattle.UKLandBattle" :NewEnumerator7 "/Game/Sprites/Textures/Cards/UnitedKingdom/UKSeaBattle.UKSeaBattle" :NewEnumerator2 "/Game/Sprites/Textures/Cards/UnitedKingdom/UKEvent.UKEvent" :NewEnumerator3 "/Game/Sprites/Textures/Cards/UnitedKingdom/UKStatus.UKStatus" :NewEnumerator4 "/Game/Sprites/Textures/Cards/UnitedKingdom/UKResponse.UKResponse" :NewEnumerator5 "/Game/Sprites/Textures/Cards/UnitedKingdom/UKEconomicWarfare.UKEconomicWarfare")))
    (:NewEnumerator2
      (return (Utilities|Select :Index (LocalVariables|GetType) :NewEnumerator0 "/Game/Sprites/Textures/Cards/Japan/Japan_BuildArmy.Japan_BuildArmy" :NewEnumerator6 "/Game/Sprites/Textures/Cards/Japan/Japan_BuildNavy.Japan_BuildNavy" :NewEnumerator1 "/Game/Sprites/Textures/Cards/Japan/Japan_LandBattle.Japan_LandBattle" :NewEnumerator7 "/Game/Sprites/Textures/Cards/Japan/Japan_SeaBattle.Japan_SeaBattle" :NewEnumerator2 "/Game/Sprites/Textures/Cards/Unknown_Card.Unknown_Card" :NewEnumerator3 "/Game/Sprites/Textures/Cards/Japan/Japan_Status.Japan_Status" :NewEnumerator4 "/Game/Sprites/Textures/Cards/Japan/Japan_Response.Japan_Response" :NewEnumerator5 "/Game/Sprites/Textures/Cards/Japan/Japan_EconomicWarfare.Japan_EconomicWarfare")))
    (:NewEnumerator4
      (return (Utilities|Select :Index (LocalVariables|GetType) :NewEnumerator0 "/Game/Sprites/Textures/Cards/Soviet/Soviet_BuildArmy.Soviet_BuildArmy" :NewEnumerator6 "/Game/Sprites/Textures/Cards/Soviet/Soviet_BuildNavy.Soviet_BuildNavy" :NewEnumerator1 "/Game/Sprites/Textures/Cards/Soviet/Soviet_LandBattle.Soviet_LandBattle" :NewEnumerator7 "/Game/Sprites/Textures/Cards/Soviet/Soviet_SeaBattle.Soviet_SeaBattle" :NewEnumerator2 "/Game/Sprites/Textures/Cards/Soviet/Soviet_Event.Soviet_Event" :NewEnumerator3 "/Game/Sprites/Textures/Cards/Soviet/Soviet_Status.Soviet_Status" :NewEnumerator4 "/Game/Sprites/Textures/Cards/Soviet/Soviet_Response.Soviet_Response" :NewEnumerator5 "/Game/Sprites/Textures/Cards/Unknown_Card.Unknown_Card")))
    (:NewEnumerator1
      (return (Utilities|Select :Index (LocalVariables|GetType) :NewEnumerator0 "/Game/Sprites/Textures/Cards/Italy/Italy_BuildArmy.Italy_BuildArmy" :NewEnumerator6 "/Game/Sprites/Textures/Cards/Italy/Italy_BuildNavy.Italy_BuildNavy" :NewEnumerator1 "/Game/Sprites/Textures/Cards/Italy/Italy_LandBattle.Italy_LandBattle" :NewEnumerator7 "/Game/Sprites/Textures/Cards/Italy/Italy_SeaBattle.Italy_SeaBattle" :NewEnumerator2 "/Game/Sprites/Textures/Cards/Italy/Italy_Event.Italy_Event" :NewEnumerator3 "/Game/Sprites/Textures/Cards/Italy/Italy_Status.Italy_Status" :NewEnumerator4 "/Game/Sprites/Textures/Cards/Italy/Italy_Response.Italy_Response" :NewEnumerator5 "/Game/Sprites/Textures/Cards/Italy/Italy_Status.Italy_Status")))
    (:NewEnumerator5
      (return (Utilities|Select :Index (LocalVariables|GetType) :NewEnumerator0 "/Game/Sprites/Textures/Cards/UnitedStates/US_BuildArmy.US_BuildArmy" :NewEnumerator6 "/Game/Sprites/Textures/Cards/UnitedStates/US_BuildNavy.US_BuildNavy" :NewEnumerator1 "/Game/Sprites/Textures/Cards/UnitedStates/US_LandBattle.US_LandBattle" :NewEnumerator7 "/Game/Sprites/Textures/Cards/UnitedStates/US_SeaBattle.US_SeaBattle" :NewEnumerator2 "/Game/Sprites/Textures/Cards/UnitedStates/US_Event.US_Event" :NewEnumerator3 "/Game/Sprites/Textures/Cards/UnitedStates/US_Status.US_Status" :NewEnumerator4 "/Game/Sprites/Textures/Cards/Unknown_Card.Unknown_Card" :NewEnumerator5 "/Game/Sprites/Textures/Cards/UnitedStates/US_Status.US_Status")))))

(fn CardBackTexture
  (params (Faction :type PlayableRaceEnum%20Enum :default "NewEnumerator0"))
  (return (Utilities|Select :Index Faction :NewEnumerator0 "/Game/Sprites/Textures/Cards/Germany/Germany_CardBack.Germany_CardBack" :NewEnumerator3 "/Game/Sprites/Textures/Cards/UnitedKingdom/UK_CardBack.UK_CardBack" :NewEnumerator2 "/Game/Sprites/Textures/Cards/Japan/Japan_CardBack.Japan_CardBack" :NewEnumerator4 "/Game/Sprites/Textures/Cards/Soviet/Soviet_CardBack.Soviet_CardBack" :NewEnumerator1 "/Game/Sprites/Textures/Cards/Italy/Italy_CardBack.Italy_CardBack" :NewEnumerator5 "/Game/Sprites/Textures/Cards/UnitedStates/US_CardBack.US_CardBack")))