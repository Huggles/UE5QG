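; Blueprint utility functions for looking up turn-based and menu player controllers from a world context.
; The get-all functions loop over player controller indices and collect those that cast to BP_TurnBasedPlayerController or BP_MenuPlayerController.
; The first-local getters reuse those lists and return the first local controller, while a turn-based variant returns every controller except the one passed in.
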(fn GetAllTBPlayerControllers
  (for _index (range 0 (- (Class|GameplayStatics|GetNumPlayerControllers (LocalVariables|Get__WorldContext)) 1))
    (bind _asbp_turn_based_player_controller (Utilities|Casting|CastToBP_TurnBasedPlayerController (Game|GetPlayerController (LocalVariables|Get__WorldContext) _index)))
    (Utilities|Array|Add (LocalVariables|Get_localControllers) _asbp_turn_based_player_controller))
  (return (LocalVariables|Get_localControllers)))

(fn GetFirstLocalTBPlayerController
  (for _array_element (TBControllers|GetAllTBPlayerControllers (LocalVariables|Get__WorldContext))
    (if (Pawn|IsLocalPlayerController _array_element)
      (return _array_element))))

(fn GetAllOtherTBPlayerControllers
  (params (My%20Player%20Controller :type BP%20Turn%20Based%20Player%20Controller%20Object%20Reference))
  (for _index (range 0 (- (Class|GameplayStatics|GetNumPlayerControllers (LocalVariables|Get__WorldContext)) 1))
    (bind _asbp_turn_based_player_controller (Utilities|Casting|CastToBP_TurnBasedPlayerController (Game|GetPlayerController (LocalVariables|Get__WorldContext) _index)))
    (if (!= _asbp_turn_based_player_controller My%20Player%20Controller)
      (Utilities|Array|Add (LocalVariables|Get_localControllers) _asbp_turn_based_player_controller)))
  (return (LocalVariables|Get_localControllers)))

(fn GetFirstLocalMenuPlayerController
  (for _array_element (MenuControllers|GetAllMenuPlayerControllers (LocalVariables|Get__WorldContext))
    (if (Pawn|IsLocalPlayerController _array_element)
      (return _array_element))))

(fn GetAllMenuPlayerControllers
  (for _index (range 0 (- (Class|GameplayStatics|GetNumPlayerControllers (LocalVariables|Get__WorldContext)) 1))
    (bind _asbp_menu_player_controller (Utilities|Casting|CastToBP_MenuPlayerController (Game|GetPlayerController (LocalVariables|Get__WorldContext) _index)))
    (Utilities|Array|Add (LocalVariables|Get_localControllers) _asbp_menu_player_controller))
  (return (LocalVariables|Get_localControllers)))