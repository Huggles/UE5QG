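; Utility Blueprint with a single Arrays Equal function that tests whether two arrays hold equal elements in the same order.
; It rejects differing lengths first, then compares elements index by index, returning false at the first mismatch.
; The result accumulates in an AreEqual variable that the function never sets before the loop, so the outcome depends on that variable's initial value.
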(fn ArraysEqual
  (params (Array%201 :type Array%20of%20Object%20Object%20References) (Array%202 :type Array%20of%20Object%20Object%20References))
  (if (== (Utilities|Array|Length Array%201) (Utilities|Array|Length Array%202))
    (for (_array_element _array_index) Array%201
      (bind _output_get (LocalVariables|SetAre%20Equal (and (LocalVariables|GetAre%20Equal) (== _array_element (Utilities|Array|Get(acopy) Array%202 _array_index)))))
      (if (not _output_get)
        (return false)))
    (return (LocalVariables|GetAre%20Equal))
    (else
      (return false))))