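; BP_AbilityFactory creates the card-driven ability and command actors that build, eliminate and attack units, attack countries and force card discards.
; Each ability function spawns its ability actor with the origin card, target data and trigger settings, then executes it immediately.
; The Build Unit command instead pops an available unit from the faction's game-state pool, spawns a command actor and optionally queues it on the server command manager.
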(fn ConstructionScript)

(fn BuildUnit(Ability)
  (params (Origin%20Card :type BP%20Card%20Object%20Reference) (Country :type BP%20Country%20Object%20Reference) (Race :type FactionEnum%20Enum :default "NewEnumerator0") (Type :type UnitTypeEnum%20Enum :default "NewEnumerator0") (TriggerResponse :type Boolean) (TriggerStatus :type Boolean) (Focus :type Boolean))
  (bind _returnvalue (Game|SpawnActorfromClass "/Game/Blueprints/Abilities/BP_Ability_BuildUnit.BP_Ability_BuildUnit_C" (Variables|Default|GetSpawn%20Transform) "Undefined" "MultiplyWithRoot" 0 Race Type Country Focus Origin%20Card TriggerResponse TriggerStatus 0))
  (Default|ExecuteAbility _returnvalue)
  (return _returnvalue))

(fn EliminateUnit(Ability)
  (params (Origin%20Card :type BP%20Card%20Object%20Reference) (Unit :type BP%20Unit%20Object%20Reference) (TriggerResponse :type Boolean) (TriggerStatus :type Boolean))
  (bind _returnvalue (Game|SpawnActorfromClass "/Game/Blueprints/Abilities/BP_Ability_EliminateUnit.BP_Ability_EliminateUnit_C" (Variables|Default|GetSpawn%20Transform) "Undefined" "MultiplyWithRoot" 0 Unit Origin%20Card TriggerResponse TriggerStatus 0))
  (Default|ExecuteAbility _returnvalue)
  (return _returnvalue))

(fn ForceCardDiscard(Ability)
  (params (Origin%20Card :type BP%20Card%20Object%20Reference) (Target%20Card :type BP%20Card%20Object%20Reference) (TriggerResponse :type Boolean) (TriggerStatus :type Boolean))
  (bind _returnvalue (Game|SpawnActorfromClass "/Game/Blueprints/Abilities/BP_Ability_ForceStatusCardDiscard.BP_Ability_ForceStatusCardDiscard_C" (Variables|Default|GetSpawn%20Transform) "Undefined" "MultiplyWithRoot" 0 Target%20Card Origin%20Card TriggerResponse TriggerStatus 0))
  (Default|ExecuteAbility _returnvalue)
  (return _returnvalue))

(fn AttackCountry(Ability)
  (params (Origin%20Card :type BP%20Card%20Object%20Reference) (Country :type BP%20Country%20Object%20Reference) (TriggerResponse :type Boolean) (TriggerStatus :type Boolean))
  (bind _returnvalue (Game|SpawnActorfromClass "/Game/Blueprints/Abilities/BP_Ability_AttackCountry.BP_Ability_AttackCountry_C" (Variables|Default|GetSpawn%20Transform) "Undefined" "MultiplyWithRoot" 0 Country Origin%20Card TriggerResponse TriggerStatus 0))
  (Default|ExecuteAbility _returnvalue))

(fn AttackUnit(Ability)
  (params (Origin%20Card :type BP%20Card%20Object%20Reference) (Unit :type BP%20Unit%20Object%20Reference) (TriggerResponse :type Boolean) (TriggerStatus :type Boolean))
  (bind _returnvalue (Game|SpawnActorfromClass "/Game/Blueprints/Abilities/BP_Ability_AttackUnit.BP_Ability_AttackUnit_C" (Variables|Default|GetSpawn%20Transform) "Undefined" "MultiplyWithRoot" 0 Unit Origin%20Card TriggerResponse TriggerStatus 0))
  (Default|ExecuteAbility _returnvalue)
  (return _returnvalue))

(fn BuildUnit(Command)
  (params (Faction :type FactionEnum%20Enum :default "NewEnumerator0") (Type :type UnitTypeEnum%20Enum :default "NewEnumerator0") (Country :type BP%20Country%20Object%20Reference) (Blocking :type Boolean) (Add%20To%20Queue :type Boolean))
  (bind _unit (Default|PopAvailableUnit (.Value (Utilities|Map|Find (Variables|/Game/Blueprints/Game/BP_TurnBasedGameState.BP_TurnBasedGameState_C|GetUnit%20Pool%20By%20Faction (.TB%20Game%20State (CallFunction|TBGameState))) Faction)) Type))
  (bind _returnvalue (Game|SpawnActorfromClass "/Game/Blueprints/Commands/ServerCommands/BuildUnitCommand.BuildUnitCommand_C" (Variables|Default|GetSpawn%20Transform) "Undefined" "MultiplyWithRoot" 0 _unit Country 0 Blocking 0))
  (if Add%20To%20Queue
    (Default|AddCommand (CallFunction|ServerCommandManager) _returnvalue))
  (return _returnvalue))