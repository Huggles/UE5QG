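; Per-faction pool of army and navy pieces for a turn-based board game, limiting how many units a faction can field.
; InstantiateUnits pre-spawns hidden, attached units and counts their spawned-on-all callbacks, notifying game setup once every client has them.
; Pop hands out a unit not in play and removes it from the pool.
; On the authority, the game event manager's remove-unit event returns units, clearing their country and reattaching them.
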(event Custom|Instantiate%20Units
  (params (Army :type Integer) (Navy :type Integer))
  (bind _faction (Variables|Default|GetFaction))
  (bind _spawn_transform (Variables|Default|GetSpawn%20Transform))
  (Variables|Default|SetArmyNum Army)
  (Variables|Default|SetNavyNum Navy)
  (Utilities|FlowControl|Sequence
    (:then_0
      (for _index (range 0 (- (Variables|Default|GetArmyNum) 1))
        (bind _returnvalue (Game|SpawnActorfromClass "/Game/Blueprints/Units/BP_Army.BP_Army_C" _spawn_transform "Undefined" "MultiplyWithRoot" 0 _faction 0))
        (Transformation|AttachActorToActor _returnvalue self "None" "KeepRelative" "KeepRelative" "KeepRelative" true)
        (Rendering|SetVisibility (Variables|/Game/Blueprints/Base/BP_SpawnableActor.BP_SpawnableActor_C|GetDefaultSceneRoot _returnvalue) false true)
        (Utilities|Array|Add (Variables|Default|GetUnits) _returnvalue)
        (EventDispatchers|AssignActorSpawnedonAll _returnvalue (delegate Custom|Army%20Spawned%20On%20All%20Event))))
    (:then_1
      (for _index_2 (range 0 (- (Variables|Default|GetNavyNum) 1))
        (bind _returnvalue_2 (Game|SpawnActorfromClass "/Game/Blueprints/Units/BP_Navy.BP_Navy_C" _spawn_transform "Undefined" "MultiplyWithRoot" 0 _faction 0))
        (Transformation|AttachActorToActor _returnvalue_2 self "None" "KeepRelative" "KeepRelative" "KeepRelative" true)
        (Rendering|SetVisibility (Variables|/Game/Blueprints/Base/BP_SpawnableActor.BP_SpawnableActor_C|GetDefaultSceneRoot _returnvalue_2) false true)
        (Utilities|Array|Add (Variables|Default|GetUnits) _returnvalue_2)
        (EventDispatchers|AssignActorSpawnedonAll _returnvalue_2 (delegate Custom|Navy%20Spawned%20On%20All%20Event))))))

(event Custom|Army%20Spawned%20On%20All%20Event
  (params (Actor :type BP%20Spawnable%20Actor%20Object%20Reference))
  (Variables|Default|SetArmies%20Spawned%20On%20Clients (+ (Variables|Default|GetArmies%20Spawned%20On%20Clients) 1))
  (if (CallFunction|AllUnitsSpawnedonAllClients)
    (Default|UnitPoolSpawnedforAllClients (Variables|/Game/Blueprints/Game/BP_TurnBasedGameState.BP_TurnBasedGameState_C|GetGame%20Setup (.TB%20Game%20State (CallFunction|TBGameState))) self)))

(event Custom|Navy%20Spawned%20On%20All%20Event
  (params (Actor :type BP%20Spawnable%20Actor%20Object%20Reference))
  (Variables|Default|SetNavies%20Spawned%20On%20Clients (+ (Variables|Default|GetNavies%20Spawned%20On%20Clients) 1))
  (if (CallFunction|AllUnitsSpawnedonAllClients)
    (Default|UnitPoolSpawnedforAllClients (Variables|/Game/Blueprints/Game/BP_TurnBasedGameState.BP_TurnBasedGameState_C|GetGame%20Setup (.TB%20Game%20State (CallFunction|TBGameState))) self)))

(event Custom|Remove%20Unit%20From%20Country_Event
  (params (Unit :type BP%20Unit%20Object%20Reference) (Country :type BP%20Country%20Object%20Reference))
  (CallFunction|ReturnUnit Unit))

(event EventBeginPlay
  (Networking|SwitchHasAuthority
    (:Authority
      (EventDispatchers|AssignRemoveUnitfromCountry (CallFunction|GameEventManager) (delegate Custom|Remove%20Unit%20From%20Country_Event)))))

(fn ConstructionScript)

(fn GetAvailableUnit
  (params (Type :type UnitTypeEnum%20Enum :default "NewEnumerator0"))
  (for _array_element (CallFunction|GetUnitsOfType Type)
    (if (not (Default|IsinPlay _array_element))
      (return _array_element))))

(fn PopAvailableUnit
  (params (Type :type UnitTypeEnum%20Enum :default "NewEnumerator0"))
  (bind _unit (CallFunction|GetAvailableUnit Type))
  (if (Utilities|IsValid _unit)
    (Utilities|Array|RemoveItem (Variables|Default|GetUnits) _unit)
    (return _unit true)
    (else
      (Development|PrintString (Utilities|String|Append "Faction is out of pieces" (Utilities|String|EnumtoString (Variables|Default|GetFaction))))
      (return 0 false))))

(fn GetUnitsOfType
  (params (Type :type UnitTypeEnum%20Enum :default "NewEnumerator0"))
  (for _array_element (Variables|Default|GetUnits)
    (if (== (Utilities|GetClass _array_element) (Utilities|Select :Index Type :NewEnumerator0 "/Game/Blueprints/Units/BP_Army.BP_Army_C" :NewEnumerator1 "/Game/Blueprints/Units/BP_Navy.BP_Navy_C" :NewEnumerator2 0))
      (Utilities|Array|Add (LocalVariables|GetlocalUnits) _array_element)))
  (return (LocalVariables|GetlocalUnits)))

(fn NumAvailableUnits
  (params (Type :type UnitTypeEnum%20Enum :default "NewEnumerator0"))
  (for _array_element (CallFunction|GetUnitsOfType Type)
    (LocalVariables|SetCounter (+ (LocalVariables|GetCounter) (Math|Integer|SelectInt 0 1 (Default|IsinPlay _array_element)))))
  (return (LocalVariables|GetCounter)))

(fn AllUnitsSpawnedonAllClients
  (return (and (== (Variables|Default|GetArmyNum) (Variables|Default|GetArmies%20Spawned%20On%20Clients)) (== (Variables|Default|GetNavyNum) (Variables|Default|GetNavies%20Spawned%20On%20Clients)))))

(fn ReturnUnit
  (params (Unit :type BP%20Unit%20Object%20Reference))
  (Utilities|Array|AddUnique (Variables|Default|GetUnits) Unit)
  (Variables|/Game/Blueprints/Units/BP_Unit.BP_Unit_C|SetCountry Unit 0)
  (Transformation|AttachActorToActor Unit self "None" "KeepRelative" "KeepRelative" "KeepRelative" true)
  (Transformation|SetActorLocationAndRotation Unit "0, 0, 0")
  (Default|ToggleSupplyVisibility Unit true))