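; BP_Unit is a faction-owned unit in a turn-based game that sits on countries and tracks whether it is supplied.
; On authority, it sets up faction-colored dynamic materials and follows GameEventManager events to attach to country spawn points or its faction's pool.
; Capsule cursor events drive selection color and animated hover indicator, reporting clicks to GameEventManager.
; Supply checks pathfind to occupied supply countries, showing a rotating indicator when none is reachable.
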(event OnBeginCursorOver(Capsule)
  (params (TouchedComponent :type Primitive%20Component%20Object%20Reference))
  (Input|OnMousein))

(event OnEndCursorOver(Capsule)
  (params (TouchedComponent :type Primitive%20Component%20Object%20Reference))
  (Input|OnMouseOut))

(event OnClicked(Capsule)
  (params (TouchedComponent :type Primitive%20Component%20Object%20Reference) (ButtonPressed :type Key%20Structure))
  (Input|OnMouseClick))

(event Custom|Add%20Unit%20To%20Country_Event
  (params (Country :type BP%20Country%20Object%20Reference) (Unit :type BP%20Unit%20Object%20Reference))
  (if (== Unit self)
    (CallFunction|AddUnittoCountry Country)))

(event Custom|Stop%20SupplyBarrel%20Indicator
  (bind _rotation (Timeline|Timeline_0 Stop)
    (:Update
      (Transformation|SetRelativeRotation (Variables|Default|GetSupplyIndicator) (Math|Rotator|MakeRotator 9e+01 0.0 _rotation) false false))))

(event Custom|Start%20SupplyBarrel%20Indicator
  (bind _rotation (Timeline|Timeline_0 PlayFromStart)
    (:Update
      (Transformation|SetRelativeRotation (Variables|Default|GetSupplyIndicator) (Math|Rotator|MakeRotator 9e+01 0.0 _rotation) false false))))

(event Custom|Start%20Animate%20Hover%20Indicator
  (bind _hoverindicator (Variables|Default|GetHoverIndicator))
  (bind _relativelocation (Variables|/Script/Engine.SceneComponent|GetRelativeLocation _hoverindicator))
  (bind _hover_indicator_animation (Timeline|Timeline Play)
    (:Update
      (Transformation|SetRelativeLocation _hoverindicator (Math|Vector|MakeVector (.x _relativelocation) (.y _relativelocation) (+ (.z _relativelocation) (* _hover_indicator_animation (Variables|Default|GetHover%20Indicator%20Speed)))) false false))))

(event Custom|Stop%20Animate%20Hover%20Indicator
  (bind _hoverindicator (Variables|Default|GetHoverIndicator))
  (bind _relativelocation (Variables|/Script/Engine.SceneComponent|GetRelativeLocation _hoverindicator))
  (bind _hover_indicator_animation (Timeline|Timeline Stop)
    (:Update
      (Transformation|SetRelativeLocation _hoverindicator (Math|Vector|MakeVector (.x _relativelocation) (.y _relativelocation) (+ (.z _relativelocation) (* _hover_indicator_animation (Variables|Default|GetHover%20Indicator%20Speed)))) false false))))

(event Custom|Handle%20Materials
  ;[1 1 1] Set Materials
  (Utilities|FlowControl|Sequence
    (:then_0
      (bind _returnvalue (Rendering|Material|CreateDynamicMaterialInstance (Variables|Default|GetUnitMesh) 0 "/Game/Material/Units/M_Unit_Inst.M_Unit_Inst" "Unit_Inst_Dynamic" :!class /Script/Engine.PrimitiveComponent))
      (Variables|Materials|SetDynamic%20Unit%20Material _returnvalue)
      (Rendering|Material|SetMaterial (Variables|Default|GetUnitMesh) 0 (Variables|Materials|GetDynamic%20Unit%20Material)))
    (:then_1
      (bind _returnvalue_2 (Rendering|Material|CreateDynamicMaterialInstance (Variables|Default|GetSelectionRing) 1 "/Game/Material/Units/M_UnitSelectionPlane_Inst.M_UnitSelectionPlane_Inst" "Unit_Selected_Inst_Dynamic" :!class /Script/Engine.PrimitiveComponent))
      (Variables|Materials|SetDynamic%20Selection%20Circle%20Material _returnvalue_2)
      (Rendering|Material|SetMaterial (Variables|Default|GetSelectionRing) 1 (Variables|Materials|GetDynamic%20Selection%20Circle%20Material)))
    (:then_2
      (bind _returnvalue_3 (Rendering|Material|CreateDynamicMaterialInstance (Variables|Default|GetSupplyIndicator) 1 "/Game/Meshes/GameplayElements/SupplyBarrel/M_Simple_Color_Black.M_Simple_Color_Black" "FactionColor_Inst_Dynamic" :!class /Script/Engine.PrimitiveComponent))
      (Variables|Materials|SetFaction%20Color%20Material _returnvalue_3)
      (Rendering|Material|SetMaterial (Variables|Default|GetSupplyIndicator) 1 (Variables|Materials|GetFaction%20Color%20Material)))))

(event Custom|Add%20Unit%20To%20Country
  (params (Country :type BP%20Country%20Object%20Reference))
  (bind _output_get (Variables|Hierarchy|SetCountry Country))
  (bind _output_get_2 (Variables|Hierarchy|SetSpawn%20Point (Default|GetAvailableUnitPos _output_get)))
  (Transformation|AttachComponentToComponent _output_get_2 "None" "SnapToTarget" "KeepRelative" "KeepRelative" true))

(event Custom|Remove%20Unit%20From%20Country
  (Variables|Hierarchy|SetCountry 0)
  (Variables|Hierarchy|SetSpawn%20Point 0)
  (Transformation|AttachActorToActor (.Value (Utilities|Map|Find (Variables|/Game/Blueprints/Game/BP_TurnBasedGameState.BP_TurnBasedGameState_C|GetUnit%20Pool%20By%20Faction (.TB%20Game%20State (CallFunction|TBGameState))) (Variables|Default|GetFaction))) "None" "KeepRelative" "KeepRelative" "KeepRelative" true))

(event Custom|Set%20Clickable
  (params (Clickable :type Boolean))
  (bind _output_get (Variables|Default|SetClickable Clickable))
  (CallFunction|ToggleSelectionVisibility _output_get)
  (Input|OnMouseOut))

(event Custom|Hide%20Actor
  (CallFunction|ToggleHoverVisibility false)
  (CallFunction|ToggleSelectionVisibility false)
  (CallFunction|ToggleUnitVisibility false)
  (CallFunction|ToggleSupplyVisibility false))

(event Custom|Remove%20Unit%20From%20Country_Event
  (params (Unit :type BP%20Unit%20Object%20Reference) (Country :type BP%20Country%20Object%20Reference))
  (if (== Unit self)
    (CallFunction|RemoveUnitfromCountry)))

(event Custom|Set%20Local%20Properties
  (params (Faction%20Color :type Linear%20Color%20Structure))
  (CallFunction|HandleMaterials)
  (CallFunction|SetUnitFactionColor Faction%20Color)
  (Input|SetSelectionColor (Variables|Default|GetDefaultSelectionColor)))

(event EventBeginPlay
  (bind _game_event_manager (CallFunction|GameEventManager))
  (|CallParentFunction)
  (Networking|SwitchHasAuthority
    (:Authority
      (Utilities|FlowControl|Sequence
        (:then_0
          (CallFunction|HideActor)
          (CallFunction|SetLocalProperties (Math|Conversions|ToLinearColor(Color) (.color (Default|GetRaceStructStructforRace (.TB%20Game%20State (CallFunction|TBGameState)) (Variables|Default|GetFaction))))))
        (:then_1
          (EventDispatchers|AssignAddUnittoCountry _game_event_manager (delegate Custom|Add%20Unit%20To%20Country_Event))
          (EventDispatchers|AssignRemoveUnitfromCountry _game_event_manager (delegate Custom|Remove%20Unit%20From%20Country_Event)))))))

(fn ConstructionScript)

(fn FnSetPlayer
  (params (Player :type Player%20Struct%20Structure)))

(fn DebugClick
  (Development|PrintString (Utilities|String|Append "Clicked on Unit" (Utilities|GetDisplayName self)) true true "(R=1.000000,G=0.918244,B=0.000000,A=1.000000)" 5.0))

(fn TBGameState
  (bind _asbp_turn_based_game_state (Utilities|Casting|CastToBP_TurnBasedGameState (Game|GetGameState)))
  (return _asbp_turn_based_game_state))

(fn IsSupplied
  (return (or (Variables|Supply|GetSupplied) (Variables|Supply|GetOverrideSupplied))))

(fn IsinPlay
  (return (and (Utilities|IsValid (Variables|Hierarchy|GetCountry)) (Utilities|IsValid (Variables|Hierarchy|GetSpawn%20Point)))))

(fn OnMouseClick
  (Default|CallUnitClicked (CallFunction|GameEventManager) (CallFunction|GetFirstLocalTBPlayerController) self (Variables|Default|GetClickable)))

(fn OnMousein
  (if (Variables|Default|GetClickable)
    (Input|SetSelectionColor (Variables|Default|GetHoverSelectionColor))
    (Rendering|SetVisibility (Variables|Default|GetHoverIndicator) true true)
    (CallFunction|StartAnimateHoverIndicator)))

(fn OnMouseOut
  (Input|SetSelectionColor (Variables|Default|GetDefaultSelectionColor))
  (Rendering|SetVisibility (Variables|Default|GetHoverIndicator) false true)
  (CallFunction|StopAnimateHoverIndicator))

(fn SetSelectionColor
  (params (Color :type Linear%20Color%20Structure))
  (Rendering|Material|SetVectorParameterValue (Variables|Materials|GetDynamic%20Selection%20Circle%20Material) "c" Color :!class /Script/Engine.MaterialInstanceDynamic))

(fn SetUnitFactionColor
  (params (Color :type Linear%20Color%20Structure))
  (Rendering|Material|SetVectorParameterValue (Variables|Materials|GetDynamic%20Unit%20Material) "c" Color :!class /Script/Engine.MaterialInstanceDynamic)
  (Rendering|Material|SetVectorParameterValue (Variables|Materials|GetFaction%20Color%20Material) "color" Color :!class /Script/Engine.MaterialInstanceDynamic))

(fn ToggleHoverVisibility
  (params (Visibility :type Boolean))
  (Rendering|SetVisibility (Variables|Default|GetHoverIndicator) Visibility true))

(fn ToggleSelectionVisibility
  (params (Visibility :type Boolean))
  (Rendering|SetVisibility (Variables|Default|GetSelectionRing) Visibility true))

(fn ToggleSupplyVisibility
  (params (Supplied :type Boolean))
  (bind _returnvalue (not Supplied))
  (Rendering|SetVisibility (Variables|Default|GetSupplyIndicator) _returnvalue true)
  (if _returnvalue
    (CallFunction|StartSupplyBarrelIndicator)
    (else
      (CallFunction|StopSupplyBarrelIndicator))))

(fn ToggleUnitVisibility
  (params (Visibility :type Boolean))
  (Rendering|SetVisibility (Variables|Default|GetUnitMesh) Visibility true))

(fn CalculateUnitSupplyLine
  (bind _country (Variables|Hierarchy|GetCountry))
  (bind _faction (Variables|Default|GetFaction))
  (for _array_element (.occupiedsupplycountries (Default|GetFactionState (.TB%20Game%20State (CallFunction|TBGameState)) (Variables|Default|GetFaction)))
    (bind _returnvalue (Game|ConstructObjectfromClass "/Game/Blueprints/Navigation/SupplyPathfindingManager.SupplyPathfindingManager_C" _faction (CallFunction|GetTeamforRace _faction)))
    (bind (_path_found _path) (Default|FindPath _returnvalue _country _array_element))
    (Utilities|FlowControl|Sequence
      (:then_0
        (Development|PrintString (Utilities|String|Append "Found Path From: " (Utilities|GetDisplayName _country) " to " (Utilities|GetDisplayName _array_element)))
        (for _array_element_2 _path
          (Development|PrintString (Utilities|GetDisplayName (Variables|/Game/Blueprints/Navigation/PathfindingNode.PathfindingNode_C|GetCountry _array_element_2)))))
      (:then_1
        (if _path_found
          (return true)))))
  (return false))

(fn CalculateIsUnitSupplied
  (bind _is_supplied (Supply|CalculateUnitSupplyLine))
  (bind _output_get (Variables|Supply|SetSupplied _is_supplied))
  (CallFunction|ToggleSupplyVisibility _output_get)
  (return _output_get))

(fn DebugUnitState
  (bind _self self)
  (Development|PrintString (Utilities|String|Append (Utilities|GetDisplayName (Variables|BP_Unit_C|GetCountry _self)) " - " (Utilities|String|EnumtoString (Variables|BP_Unit_C|GetFaction _self)) " - " (Utilities|String|ToString(Boolean) (CallFunction|IsSupplied _self)))))