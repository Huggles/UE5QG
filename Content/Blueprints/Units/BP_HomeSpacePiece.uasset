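; BP_HomeSpacePiece is a board piece marking a player's home space, tinted with that player's race color.
; SetPlayerRace stores the race, then builds a dynamic material instance on the mesh and sets its "Player Color" from the game state's race data.
; SetTowerVisibility shows or hides the mesh along with its children.
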(event Custom|Set%20Player%20Race
  (params (Race :type PlayableRaceEnum%20Enum :default "NewEnumerator6"))
  (Variables|Default|SetRace Race)
  (CallFunction|HandleMaterials))

(event Custom|Set%20Tower%20Visibility
  (params (Visible :type Boolean))
  (Rendering|SetVisibility (Variables|Default|GetHomeSpacePieceMesh) Visible true))

(event Custom|Handle%20Materials
  ;[1 1 1] Set Materials
  (bind _returnvalue (Rendering|Material|CreateDynamicMaterialInstance (Variables|Default|GetHomeSpacePieceMesh) 0 (Variables|Default|GetSource%20Material) "None" :!class /Script/Engine.PrimitiveComponent))
  (bind _output_get (Variables|Default|SetDynamic%20Material _returnvalue))
  (Rendering|Material|SetVectorParameterValue _output_get "Player Color" (Math|Conversions|ToLinearColor(Color) (.color (Default|GetRaceStructStructforRace (CallFunction|TBGameState) (Variables|Default|GetRace)))) :!class /Script/Engine.MaterialInstanceDynamic)
  (Rendering|Material|SetMaterial (Variables|Default|GetHomeSpacePieceMesh) 0 (Variables|Default|GetDynamic%20Material)))

(fn ConstructionScript)