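; Pathfinding manager that searches for a route between two countries, wrapping each in a PathfindingNode.
; FindPath runs an open/closed-list search using only distance from start, with no heuristic, re-parenting open neighbors when a shorter route appears.
; GetLowestCostNode's comparison actually selects the highest-distance node, despite its name.
; The path is rebuilt through parent links from target to start; the navigability check always passes.
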(fn FindPath
  (params (From :type BP%20Country%20Object%20Reference) (To :type BP%20Country%20Object%20Reference))
  (bind _open (Variables|Default|GetOpen))
  (bind _returnvalue (Game|ConstructObjectfromClass "/Game/Blueprints/Navigation/PathfindingNode.PathfindingNode_C" From))
  (bind _output_get (LocalVariables|SetFrom%20Node _returnvalue))
  (bind _returnvalue_2 (Game|ConstructObjectfromClass "/Game/Blueprints/Navigation/PathfindingNode.PathfindingNode_C" To))
  (LocalVariables|SetTarget%20Node _returnvalue_2)
  (Utilities|Array|Add _open _output_get)
  (while (Utilities|Array|IsNotEmpty _open)
    (bind _output_get_2 (LocalVariables|SetCurrent%20Node%20%28Q%29 (CallFunction|GetLowestCostNode _open)))
    (if (CallFunction|ConsiderNode _output_get_2)
      (Utilities|Array|RemoveItem _open _output_get_2)
      (Utilities|Array|Add (Variables|Default|GetClosed) (LocalVariables|GetCurrent%20Node%20%28Q%29))
      (if (CallFunction|NodesEqual (LocalVariables|GetCurrent%20Node%20%28Q%29) (LocalVariables|GetTarget%20Node))
        (return true (CallFunction|CalculatePathforEndNode (LocalVariables|GetCurrent%20Node%20%28Q%29)))
        (else
          (bind _neighboornodes (Default|Neighboors (LocalVariables|GetCurrent%20Node%20%28Q%29)))
          (LocalVariables|SetCurrent%20Node%20Neighboors _neighboornodes)
          (for _array_element (LocalVariables|GetCurrent%20Node%20Neighboors)
            (if (CallFunction|ConsiderNode _array_element)
              (Variables|/Game/Blueprints/Navigation/PathfindingNode.PathfindingNode_C|SetParentNode _array_element (LocalVariables|GetCurrent%20Node%20%28Q%29))
              (if (.Contains (CallFunction|ContainsCountryNode (Variables|Default|GetOpen) _array_element))
                (if (> (Default|DistancefromStart(G) (Utilities|Array|Get(acopy) (Variables|Default|GetOpen) (.Array%20Index (CallFunction|ContainsCountryNode (Variables|Default|GetOpen) _array_element)))) (Default|DistancefromStart(G) _array_element))
                  (Variables|/Game/Blueprints/Navigation/PathfindingNode.PathfindingNode_C|SetParentNode (Utilities|Array|Get(acopy) (Variables|Default|GetOpen) (.Array%20Index (CallFunction|ContainsCountryNode (Variables|Default|GetOpen) _array_element))) (LocalVariables|GetCurrent%20Node%20%28Q%29)))
                (else
                  (Utilities|Array|Add (Variables|Default|GetOpen) _array_element)))))))
      (else
        (return false 0))))
  (return false 0))

(fn GetLowestCostNode
  (params (Cost%20Map :type Array%20of%20Pathfinding%20Node%20Object%20References))
  (for _array_element Cost%20Map
    (if (not (Utilities|IsValid (LocalVariables|GetLowestCostNodeLocal)))
      (LocalVariables|SetLowestCostNodeLocal _array_element :!label _label)
      (elif (< (Default|DistancefromStart(G) (LocalVariables|GetLowestCostNodeLocal)) (Default|DistancefromStart(G) _array_element))
        (goto _label))))
  (return (LocalVariables|GetLowestCostNodeLocal)))

(fn ContainsCountryNode
  (params (Nodes :type Array%20of%20Pathfinding%20Node%20Object%20References) (node :type Pathfinding%20Node%20Object%20Reference))
  (for (_array_element _array_index) Nodes
    (if (== (Variables|/Game/Blueprints/Navigation/PathfindingNode.PathfindingNode_C|GetCountry _array_element) (Variables|/Game/Blueprints/Navigation/PathfindingNode.PathfindingNode_C|GetCountry node))
      (return true _array_index)))
  (return false 0))

(fn NodesEqual
  (params (Node%201 :type Pathfinding%20Node%20Object%20Reference) (Node%202 :type Pathfinding%20Node%20Object%20Reference))
  (return (== (Variables|/Game/Blueprints/Navigation/PathfindingNode.PathfindingNode_C|GetCountry Node%201) (Variables|/Game/Blueprints/Navigation/PathfindingNode.PathfindingNode_C|GetCountry Node%202))))

(fn IsNodeNavigatable
  (params (Node :type Pathfinding%20Node%20Object%20Reference))
  (return true))

(fn CalculatePathforEndNode
  (params (End%20Node :type Pathfinding%20Node%20Object%20Reference))
  (LocalVariables|SetCurrent%20Path%20Calculation%20Node End%20Node)
  (Utilities|Array|Add (LocalVariables|GetPath%20Local_0) (LocalVariables|GetCurrent%20Path%20Calculation%20Node))
  (while (Utilities|IsValid (Variables|/Game/Blueprints/Navigation/PathfindingNode.PathfindingNode_C|GetParentNode (LocalVariables|GetCurrent%20Path%20Calculation%20Node)))
    (Utilities|Array|Add (LocalVariables|GetPath%20Local_0) (Variables|/Game/Blueprints/Navigation/PathfindingNode.PathfindingNode_C|GetParentNode (LocalVariables|GetCurrent%20Path%20Calculation%20Node)))
    (LocalVariables|SetCurrent%20Path%20Calculation%20Node (Variables|/Game/Blueprints/Navigation/PathfindingNode.PathfindingNode_C|GetParentNode (LocalVariables|GetCurrent%20Path%20Calculation%20Node))))
  (return (LocalVariables|GetPath%20Local_0)))

(fn ConsiderNode
  (params (Node :type Pathfinding%20Node%20Object%20Reference))
  (return (and (not (.Contains (CallFunction|ContainsCountryNode (Variables|Default|GetClosed) Node))) (CallFunction|IsNodeNavigatable Node))))