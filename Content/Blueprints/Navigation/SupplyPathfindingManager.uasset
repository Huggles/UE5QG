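; Supply pathfinding manager Blueprint that decides which country nodes a faction's supply routes can pass through.
; IsNodeNavigatable accepts a node only when the faction has a unit in that country.
; Water countries additionally require the faction to have a port there, while land countries pass with the unit alone.
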(fn IsNodeNavigatable
  (params (Node :type Pathfinding%20Node%20Object%20Reference))
  (bind _country (Variables|/Game/Blueprints/Navigation/PathfindingNode.PathfindingNode_C|GetCountry Node))
  (bind _faction (Variables|Default|GetFaction))
  (if (.Player%20Has%20Unit (Default|HasPlayerUnit _country _faction))
    (if (Default|IsWater _country)
      (return (Default|FactionHasPort _country _faction))
      (else
        (return true)))
    (else
      (return false))))