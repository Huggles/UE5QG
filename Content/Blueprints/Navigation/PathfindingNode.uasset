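; PathfindingNode is an A*-style search node that wraps a Country for pathfinding across connected countries.
; Neighboors constructs a new node for each connected country without assigning its parent.
; G counts hops recursively through the ParentNode chain.
; H is a placeholder derived from a constant minus G rather than any target, and F returns constant zero instead of combining G and H.
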(fn Neighboors
  (for _array_element (Variables|/Game/Blueprints/Countries/BP_Country.BP_Country_C|GetConnectedCountries (Variables|Default|GetCountry))
    (bind _returnvalue (Game|ConstructObjectfromClass _array_element "PathfindingNode_C" _array_element))
    (Utilities|Array|Add (LocalVariables|GetNeighboorNodesLocal) _returnvalue))
  (return (LocalVariables|GetNeighboorNodesLocal)))

(fn TotalCost(F)
  (return (+ 0 0)))

(fn DistancefromStart(G)
  (bind _parentnode (Variables|Default|GetParentNode))
  (if (Utilities|IsValid _parentnode)
    (return (+ (CallFunction|DistancefromStart(G) _parentnode) 1))
    (else
      (return 0))))

(fn EstimatedDistancetoEnd(H)
  (return (- 10 (CallFunction|DistancefromStart(G)))))