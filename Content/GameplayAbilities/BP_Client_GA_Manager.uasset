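; Client-side manager actor for gameplay ability actors, holding pending and current ability lists and reporting whether it is working.
; On authority it takes its parent actor as owner at BeginPlay.
; Added abilities join the pending queue and attach to the first local TB player controller's ability manager.
; Execution is unfinished: ExecuteNextAbility only checks the queue, while preprocessing and completion-chaining logic sit disconnected and NotifyAnimationCompleted is empty.
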(event Custom|Notify%20Animation%20Completed)

(event Custom|Execute%20Next%20Ability
  (if (CallFunction|HasPendingAbility)
    _))

(event Custom|Add%20Gameplay%20Ability
  (params (Ability :type BP%20Gameplay%20Ability%20Object%20Reference%20%28by%20ref%29))
  (Utilities|Array|Add (Variables|Default|GetPendingGameplayAbilities) Ability)
  (Transformation|AttachActorToActor Ability (Default|GetGameplayAbilityManager (CallFunction|GetFirstLocalTBPlayerController)) "None" "KeepRelative" "KeepRelative" "KeepRelative" true)
  (CallFunction|ExecuteNextAbility))

(event EventBeginPlay
  (Networking|SwitchHasAuthority
    (:Authority
      (Actor|SetOwner (Actor|GetParentActor self))
      (Development|PrintString "Hello"))))

(fn ConstructionScript)

(fn NextAbility
  (return (Utilities|Array|Get(acopy) (Variables|Default|GetPendingGameplayAbilities))))

(fn IsExecutingAbility
  (return (> (Utilities|Array|Length (Variables|Default|GetCurrentGameplayAbilities)) 0)))

(fn HasPendingAbility
  (return (> (Utilities|Array|Length (Variables|Default|GetPendingGameplayAbilities)) 0)))

(fn IsWorking
  (return (or (CallFunction|IsExecutingAbility) (CallFunction|HasPendingAbility))))