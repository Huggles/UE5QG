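; BP_GA_BuildUnit is a turn-based gameplay ability that places a new unit of a given Race and Type in a Country.
; On task initialization it takes an available unit from the race's unit pool and adds it to the country.
; It then queues two ability tasks: a camera zoom on the local player's pawn to the unit's spawn point, optionally saving the original position, and a task that shows the unit.
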(event EventInitializeTasks
  (bind _unit_pool (CallFunction|GetUnitPool (Variables|Default|GetRace)))
  (bind _unit (Default|GetAvailableUnit _unit_pool (Variables|Default|GetType)))
  (Default|AddUnittoCountry _unit (Variables|Default|GetCountry))
  (bind _returnvalue (Game|ConstructObjectfromClass "/Game/GameplayAbilities/Tasks/BP_GAT_ZoomCamera.BP_GAT_ZoomCamera_C" (.AsBP%20Turn%20Based%20Pawn (Utilities|Casting|CastToBP_TurnBasedPawn (Pawn|GetControlledPawn (CallFunction|GetFirstLocalTBPlayerController)))) (Transformation|GetWorldLocation (Variables|/Game/Blueprints/Units/BP_Unit.BP_Unit_C|GetSpawn%20Point _unit)) (Math|Vector|MakeVector 0.0 5e+02 1e+03) (Variables|Default|GetSave%20Camera%20Position)))
  (bind _returnvalue_2 (Game|ConstructObjectfromClass "/Game/GameplayAbilities/Tasks/BP_GAT_ShowUnit.BP_GAT_ShowUnit_C" _unit))
  (Utilities|Array|AppendArray (Variables|Default|GetGA_Tasks) (Utilities|Array|MakeArray _returnvalue _returnvalue_2)))

(fn ConstructionScript
  (|CallParentFunction))