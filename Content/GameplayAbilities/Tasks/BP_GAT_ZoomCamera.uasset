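; Gameplay ability task that zooms the camera by moving its Pawn to a Target position offset by Distance.
; On execute it optionally saves the Pawn's current location to the Pawn's OriginalPosition.
; A fixed-duration sine ease-in-out vector tween then sets the Pawn location on each easing update, without sweep, and signals task finished on completion.
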(event EventExecuteTask
  (bind _pawn (Variables|Default|GetPawn))
  (bind _target (Variables|Default|GetTarget))
  (bind (_x _y _z) (Math|Vector|BreakVector _target))
  (bind _returnvalue (Transformation|GetActorLocation _pawn))
  (if (Variables|Default|GetSave%20Original%20Position)
    (Variables|/Game/Blueprints/Game/BP_TurnBasedPawn.BP_TurnBasedPawn_C|SetOriginalPosition _pawn _returnvalue))
  (bind _value (|TweenVector _returnvalue (+ (Math|Vector|MakeVector _x _y _z) (Variables|Default|GetDistance)) 1.5 "InOutSine")
    (:ApplyEasing
      (Transformation|SetActorLocation _pawn _value false false))
    (:OnComplete
      (Default|CallTaskFinished self))))