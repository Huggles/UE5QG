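; Gameplay ability task that plays out a unit's removal from its country during an attack.
; On execution it attaches a particle emitter to the unit's mesh and tweens the actor through a 90-degree rotation from its current orientation.
; When the tween completes, it hides the mesh and its children, zeroes the relative rotation, removes the unit from its country and signals that the task is finished.
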(event EventExecuteTask
  (bind _unit (Variables|Default|GetUnit))
  (bind _unit_2 (Variables|Default|GetUnit))
  (bind _returnvalue (Transformation|GetActorRotation _unit))
  (Effects|SpawnEmitterAttached 0 (Variables|/Game/Blueprints/Units/BP_Unit.BP_Unit_C|GetUnitMesh (Variables|Default|GetUnit)) "None")
  (bind _value (|TweenRotator _returnvalue (Math|Rotator|CombineRotators _returnvalue "90.000000,0.000000,0.000000") 1.0 "InOutQuad")
    (:ApplyEasing
      (Transformation|SetActorRelativeRotation (Variables|Default|GetUnit) _value))
    (:OnComplete
      (Rendering|SetVisibility (Variables|/Game/Blueprints/Units/BP_Unit.BP_Unit_C|GetUnitMesh (Variables|Default|GetUnit)) false true)
      (Transformation|SetActorRelativeRotation _unit_2)
      (Default|RemoveUnitfromCountry _unit_2)
      (Default|CallTaskFinished self))))