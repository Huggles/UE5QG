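; Gameplay ability task that presents a played card to the player as a zoomed view in the turn-based controller's UI.
; On execute it shows the card zoom with a subtitle from Card Presentation Title for a fixed duration, then binds to the hide animation's end to finish the task.
; The title function holds only an unconnected node that would join the card's race with "plays".
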(event Custom|On%20Played%20Card%20Shown
  (Default|CallTaskFinished self))

(event EventExecuteTask
  (bind _tb_controller (Variables|Default|GetTB%20Controller))
  (bind _userinterfacewidget (Variables|/Game/Blueprints/Game/BP_TurnBasedPlayerController.BP_TurnBasedPlayerController_C|GetUserInterfaceWidget _tb_controller))
  (Default|ShowPlayedCardZoom _userinterfacewidget (Variables|Default|GetCard) (Utilities|CardPresentationTitle) 3.0)
  (Class|UserWidget|BindtoAnimationFinished _userinterfacewidget (Variables|/Game/Blueprints/UI/UIB_GameInterface_Base.UIB_GameInterface_Base_C|GetHidePlayedCardZoomAnimation _userinterfacewidget) (delegate Custom|On%20Played%20Card%20Shown)))