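; Gameplay ability task that eliminates a unit with a short falling-over animation.
; A rotator tween turns the unit from its current rotation by a combined yaw and roll offset, applying it each easing step.
; On completion it hides the unit and its children, resets the rotation, removes the unit from its country and signals the task finished.
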(event EventExecuteTask
  (bind _unit (Variables|Default|GetUnit))
  (bind _unit_2 (Variables|Default|GetUnit))
  (bind _returnvalue (Transformation|GetActorRotation _unit))
  (bind _value (|TweenRotator _returnvalue (Math|Rotator|CombineRotators _returnvalue "90.000000,90.000000,0.000000") 1.0 "InOutQuad")
    (:ApplyEasing
      (Transformation|SetActorRelativeRotation (Variables|Default|GetUnit) _value))
    (:OnComplete
      (Rendering|SetVisibility (Variables|/Script/Engine.Actor|GetRootComponent _unit_2) false true)
      (Transformation|SetActorRelativeRotation _unit_2)
      (Default|RemoveUnitfromCountry _unit_2)
      (Default|CallTaskFinished self))))