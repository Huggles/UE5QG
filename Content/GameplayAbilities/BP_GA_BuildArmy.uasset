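; Gameplay ability that builds an army unit for a country.
; Preprocessing takes an available unit of the requested type from the race's unit pool and adds it to the country.
; It returns client animation payloads that play the build animation, wrapped in camera moves to the unit's spawn point and back when focus is enabled.
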(event EventPreprocessAbility
  (bind _unit_pool (CallFunction|GetUnitPool (Variables|Default|GetRace)))
  (bind _unit (Default|GetAvailableUnit _unit_pool (Variables|Default|GetType)))
  (bind _output_get (Variables|Default|SetUnit _unit))
  (Default|AddUnittoCountry _output_get (Variables|Default|GetCountry)))

(fn ConstructionScript
  (|CallParentFunction))

(fn AbilityAnimations
  (return (select (Variables|Default|GetFocus) (Utilities|Array|MakeArray (Utilities|Struct|MakeAnimation_Payload "/Game/ClientAnimations/BP_Client_Animation_MoveCamera.BP_Client_Animation_MoveCamera_C" 0 true 0 1.0 0 0 "0.000000,0.000000,0.000000" (Transformation|GetWorldLocation (Variables|/Game/Blueprints/Units/BP_Unit.BP_Unit_C|GetSpawn%20Point (Variables|Default|GetUnit))) "1.000000,1.000000,1.000000" "/Game/StarterContent/Particles/P_Explosion.P_Explosion" 0.0 0) (Utilities|Struct|MakeAnimation_Payload "/Game/ClientAnimations/BP_Client_Animation_BuildUnit.BP_Client_Animation_BuildUnit_C" 0 true 0 1.0 (Utilities|Array|MakeArray (Variables|Default|GetUnit)) 0 "0.000000,0.000000,0.000000" "0.000000,0.000000,0.000000" "1.000000,1.000000,1.000000" "/Game/StarterContent/Particles/P_Explosion.P_Explosion" 0.0 0) (Utilities|Struct|MakeAnimation_Payload "/Game/ClientAnimations/BP_Client_Animation_ReturnCamera.BP_Client_Animation_ReturnCamera_C" 0 true 0 1.0 0 0 "0.000000,0.000000,0.000000" "0.000000,0.000000,0.000000" "1.000000,1.000000,1.000000" "/Game/StarterContent/Particles/P_Explosion.P_Explosion" 0.0 0)) (Utilities|Array|MakeArray (Utilities|Struct|MakeAnimation_Payload "/Game/ClientAnimations/BP_Client_Animation_BuildUnit.BP_Client_Animation_BuildUnit_C" 0 false 0 1.0 (Utilities|Array|MakeArray (Variables|Default|GetUnit)) 0 "0.000000,0.000000,0.000000" "0.000000,0.000000,0.000000" "1.000000,1.000000,1.000000" "/Game/StarterContent/Particles/P_Explosion.P_Explosion" 0.0 0)))))