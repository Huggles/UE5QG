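; Client animation Blueprint that plays the destruction of a unit, using the first unit in its payload.
; It attaches the payload's particle effect to the unit mesh and tweens a quarter-turn yaw rotation over the payload duration.
; After a cooldown timer, it hides the mesh, resets the rotation, removes the unit from its country and reports the animation finished.
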(event Custom|On%20Timer%20Completed
  (bind _unit (Variables|Default|GetUnit))
  (Rendering|SetVisibility (Variables|/Game/Blueprints/Units/BP_Unit.BP_Unit_C|GetUnitMesh _unit) false true)
  (Transformation|SetActorRelativeRotation _unit)
  (Default|RemoveUnitfromCountry _unit)
  (Default|CallAnimationFinished self))

(event EventStartAnimation
  (bind _unit (Variables|Default|GetUnit))
  (bind _payload (Variables|Default|GetPayload))
  (bind _returnvalue (Transformation|GetActorRotation _unit))
  (Effects|SpawnEmitterAttached (.particlesystem _payload) (Variables|/Game/Blueprints/Units/BP_Unit.BP_Unit_C|GetUnitMesh (Variables|Default|GetUnit)) "None" "0, 0, 0" "0, 0, 0" (.scale _payload))
  (bind _value (|TweenRotator _returnvalue (Math|Rotator|CombineRotators _returnvalue "90.000000,0.000000,0.000000") (.duration _payload) "InOutQuad")
    (:ApplyEasing
      (Transformation|SetActorRelativeRotation (Variables|Default|GetUnit) _value))
    (:OnComplete
      (Utilities|Time|SetTimerbyEvent (delegate Custom|On%20Timer%20Completed) (+ (.cooldowntime _payload) 0.001)))))

(fn InitializeAnimationData
  (params (Local%20TB%20Player%20Controller :type BP%20Turn%20Based%20Player%20Controller%20Object%20Reference) (Payload :type CA%20Payload%20Structure))
  (bind (_animationclass _blocking _duration _units _countries _everyone _tbplayercontrollers _source _target _scale _particlesystem) (Utilities|Struct|BreakCA_Payload Payload))
  (|CallParentFunction Local%20TB%20Player%20Controller Payload)
  (Variables|Default|SetUnit (Utilities|Array|Get(acopy) _units))
  (Variables|Default|SetScale _scale)
  (Variables|Default|SetParticle%20System _particlesystem))