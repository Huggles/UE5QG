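; BP_Animation_ReturnCamera is a client animation that glides the player's turn-based pawn, presumably the camera, back to its original position.
; Initialization runs the parent setup, stores the payload target and caches the controller's pawn as BP_TurnBasedPawn.
; On start, an eased vector tween moves the pawn from its current location to OriginalPosition, then signals that the animation has finished.
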(event EventStartAnimation
  (bind _pawn (Variables|Default|GetPawn))
  (bind _value (|TweenVector (Transformation|GetActorLocation _pawn) (Variables|/Game/Blueprints/Game/BP_TurnBasedPawn.BP_TurnBasedPawn_C|GetOriginalPosition _pawn) 1.5 "InOutSine")
    (:then
      (Variables|/Game/Blueprints/Game/BP_TurnBasedPawn.BP_TurnBasedPawn_C|SetOriginalPosition (Variables|Default|GetPawn) (|Copy (Variables|/Game/Blueprints/Game/BP_TurnBasedPawn.BP_TurnBasedPawn_C|GetOriginalPosition _pawn))))
    (:ApplyEasing
      (Transformation|SetActorLocation _pawn _value false false))
    (:OnComplete
      (Default|CallAnimationFinished self))))

(fn InitializeAnimationData
  (params (Local%20TB%20Player%20Controller :type BP%20Turn%20Based%20Player%20Controller%20Object%20Reference) (Payload :type CA%20Payload%20Structure))
  (|CallParentFunction Local%20TB%20Player%20Controller Payload)
  (Variables|Default|SetTarget (.Target (Utilities|Struct|BreakCA_Payload Payload)))
  (Variables|Default|SetPawn (.AsBP%20Turn%20Based%20Pawn (Utilities|Casting|CastToBP_TurnBasedPawn (Pawn|GetControlledPawn Local%20TB%20Player%20Controller)))))