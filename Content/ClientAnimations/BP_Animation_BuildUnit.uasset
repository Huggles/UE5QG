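; Client animation for building a unit, which tweens the unit into place from a raised offset on the Z axis.
; Initialization calls the parent setup and caches the first unit from the payload.
; On start it resets the unit's relative rotation, shows its mesh and drives its relative location with an OutSine vector tween.
; When the tween completes, it signals that the animation has finished.
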(event EventStartAnimation
  (bind _unit (Variables|Default|GetUnit))
  (Transformation|SetActorRelativeRotation _unit)
  (Rendering|SetVisibility (Variables|/Game/Blueprints/Units/BP_Unit.BP_Unit_C|GetUnitMesh _unit) true false)
  (bind _value (|TweenVector "0.000000,0.000000,1500.000000" "0, 0, 0" 3.0 "OutSine")
    (:ApplyEasing
      (Transformation|SetActorRelativeLocation (Variables|Default|GetUnit) _value))
    (:OnComplete
      (Default|CallAnimationFinished self))))

(fn InitializeAnimationData
  (params (Local%20TB%20Player%20Controller :type BP%20Turn%20Based%20Player%20Controller%20Object%20Reference) (Payload :type CA%20Payload%20Structure))
  (|CallParentFunction Local%20TB%20Player%20Controller Payload)
  (Variables|Default|SetUnit (Utilities|Array|Get(acopy) (.Units (Utilities|Struct|BreakCA_Payload Payload)))))