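; Client animation manager that queues animation objects and starts them in order, holding the queue while any blocking animation plays.
; Adding animations triggers one attempt to start the head of the pending list, moving it to the current list and binding its finished event.
; A finished blocking animation starts the next pending one.
; With none pending, a finish fires AllAnimationsFinished only if other animations are still playing.
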(event Custom|Add%20Animations
  (params (Animations :type Array%20of%20BP%20Animation%20Object%20References))
  (Utilities|Array|AppendArray (Variables|Default|GetPendingAnimations) Animations)
  (CallFunction|RunNextAnimation))

(event Custom|Run%20Next%20Animation
  (bind _next_animation (CallFunction|NextAnimation))
  (if (and (CallFunction|HasPendingAnimation) (not (CallFunction|PlayingBlockingAnimation)))
    (EventDispatchers|AssignAnimationFinished _next_animation (delegate Custom|Animation%20Finished_Event))
    (Utilities|Array|Add (Variables|Default|GetCurrentAnimations) _next_animation)
    (Default|StartAnimation _next_animation)
    (Utilities|Array|RemoveItem (Variables|Default|GetPendingAnimations) _next_animation)))

(event Custom|Animation%20Finished_Event
  (params (Animation :type BP%20Animation%20Object%20Reference))
  (Utilities|Array|RemoveItem (Variables|Default|GetCurrentAnimations) Animation)
  (if (CallFunction|HasPendingAnimation)
    (if (Variables|/Game/ClientAnimations/BP_Animation.BP_Animation_C|GetBlocking Animation)
      (CallFunction|RunNextAnimation))
    (elif (CallFunction|IsPlayingAnimation)
      (Default|CallAllAnimationsFinished))))

(event Custom|Add%20Animation
  (params (Animation :type BP%20Animation%20Object%20Reference))
  (Utilities|Array|Add (Variables|Default|GetPendingAnimations) Animation)
  (CallFunction|RunNextAnimation))

(fn ConstructionScript)

(fn NextAnimation
  (return (Utilities|Array|Get(acopy) (Variables|Default|GetPendingAnimations))))

(fn PlayingBlockingAnimation
  (for _array_element (Variables|Default|GetCurrentAnimations)
    (if (Variables|/Game/ClientAnimations/BP_Animation.BP_Animation_C|GetBlocking _array_element)
      (return true)))
  (return false))

(fn IsPlayingAnimation
  (return (> (Utilities|Array|Length (Variables|Default|GetCurrentAnimations)) 0)))

(fn HasPendingAnimation
  (return (> (Utilities|Array|Length (Variables|Default|GetPendingAnimations)) 0)))