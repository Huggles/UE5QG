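; Server-side animation manager that relays animations to clients and signals when all have finished playing them.
; Payloads flagged for everyone are multicast to each local controller's client animation manager.
; Client finish reports trigger a check of every controller's manager; once none are working, a DoOnce, re-armed by each new animation, fires the all-finished call.
; Local queue helpers remain, but play and pause are empty.
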(event Custom|Add%20Gameplay%20Ability
  (params (Gameplay%20Ability :type BP%20Gameplay%20Ability%20Object%20Reference)))

(event Custom|Add%20Animation%20%28Multicast%29
  (params (Animation :type CA%20Payload%20Structure))
  (Default|AddAnimation (Default|GetClientAnimationManager (CallFunction|GetFirstLocalTBPlayerController)) Animation)
  (Utilities|FlowControl|DoOnce false) ; enters at Reset
)

(event Custom|Add%20Animation
  (params (Animation%20Payload :type CA%20Payload%20Structure))
  (if (.Everyone (Utilities|Struct|BreakCA_Payload Animation%20Payload))
    (CallFunction|AddAnimation(Multicast) Animation%20Payload)))

(event Custom|Add%20Animations
  (params (Animation%20Payloads :type Array%20of%20CA%20Payload%20Structures))
  (for _array_element Animation%20Payloads
    (if (.Everyone (Utilities|Struct|BreakCA_Payload _array_element))
      (CallFunction|AddAnimation(Multicast) _array_element))))

(event Custom|Animations%20Finished%20%28Server%29
  (params (TB%20Player%20Controller :type BP%20Turn%20Based%20Player%20Controller%20Object%20Reference))
  (if (not (CallFunction|AreClientsWorking(Server)))
    (Utilities|FlowControl|DoOnce false
      (:Completed
        (Default|CallAllAnimationsFinished)))))

(event EventBeginPlay)

(fn ConstructionScript)

(fn NextAnimation
  (return (Utilities|Array|Get(acopy) (Variables|Default|GetPendingAnimations))))

(fn PlayingBlockingAnimation
  (for _array_element (Variables|Default|GetCurrentAnimations)
    (if (Variables|/Game/ClientAnimations/BP_Animation.BP_Animation_C|GetBlocking _array_element)
      (return true)))
  (return false))

(fn IsPlayingAnimation
  (return (> (Utilities|Array|Length (Variables|Default|GetCurrentAnimations)) 0)))

(fn HasPendingAnimation
  (return (> (Utilities|Array|Length (Variables|Default|GetPendingAnimations)) 0)))

(fn OnRepPendingAnimations)

(fn BuildAnimation
  (switch Utilities|FlowControl|Switch|SwitchonClientAnimationType "NewEnumerator0"
    (:NewEnumerator0
      (for _array_element 0
        (bind _returnvalue (Game|ConstructObjectfromClass "/Game/ClientAnimations/BP_Animation_BuildUnit.BP_Animation_BuildUnit_C" _array_element))
        (Utilities|Array|Add (LocalVariables|Get_instantiatedAnimations) _returnvalue))
      (return (LocalVariables|Get_instantiatedAnimations)))))

(fn PauseAnimations)

(fn PlayAnimations)

(fn IsWorking
  (return (or (CallFunction|IsPlayingAnimation) (CallFunction|HasPendingAnimation))))

(fn AreClientsWorking(Server)
  (Networking|SwitchHasAuthority
    (:Authority
      (for _array_element (CallFunction|GetAllTBPlayerControllers)
        (LocalVariables|SetAreWorkingLocal (or (Default|IsWorking (Default|GetClientAnimationManager _array_element)) (LocalVariables|GetAreWorkingLocal))))
      (return (LocalVariables|GetAreWorkingLocal)))
    (:Remote
      (Development|PrintString "Checking Server Status on Client" true true "(R=1.000000,G=0.074492,B=0.000000,A=1.000000)" 5.0))))