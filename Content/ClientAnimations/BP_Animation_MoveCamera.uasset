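; Client animation that moves the local player's turn-based pawn, as the camera, to a target position from its payload.
; Initialization takes the target from the payload and caches the controlled BP_TurnBasedPawn.
; On start, it saves the pawn's original position on the pawn, then eases it to the target plus a Distance offset with a sine tween, signalling animation finished on completion.
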(event EventStartAnimation
  (bind _pawn (Variables|Default|GetPawn))
  (bind _target (Variables|Default|GetTarget))
  (bind (_x _y _z) (Math|Vector|BreakVector _target))
  (bind _output_get (Variables|/Game/Blueprints/Game/BP_TurnBasedPawn.BP_TurnBasedPawn_C|SetOriginalPosition _pawn (Transformation|GetActorLocation _pawn)))
  (bind _value (|TweenVector _output_get (+ (Math|Vector|MakeVector _x _y _z) (Variables|Default|GetDistance)) 1.5 "InOutSine")
    (:ApplyEasing
      (Transformation|SetActorLocation _pawn _value false false))
    (:OnComplete
      (Default|CallAnimationFinished self))))

(fn InitializeAnimationData
  (params (Local%20TB%20Player%20Controller :type BP%20Turn%20Based%20Player%20Controller%20Object%20Reference) (Payload :type CA%20Payload%20Structure))
  (|CallParentFunction Local%20TB%20Player%20Controller Payload)
  (Variables|Default|SetTarget (.Target (Utilities|Struct|BreakCA_Payload Payload)))
  (Variables|Default|SetPawn (.AsBP%20Turn%20Based%20Pawn (Utilities|Casting|CastToBP_TurnBasedPawn (Pawn|GetControlledPawn Local%20TB%20Player%20Controller)))))

(fn NewFunction)